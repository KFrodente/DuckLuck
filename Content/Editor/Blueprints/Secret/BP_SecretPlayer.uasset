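; BP_SecretPlayer is the player for a secret betting minigame where money is wagered on spawned balls.
; On BeginPlay it adds the IMC_Secret input context, shows the cursor and UW_Secret widget, and caches all TargetPoints as spawns.
; The selection input, if TotalMoney covers CurrentBet, spawns a BP_Ball worth that bet at a random point.
; A looping Payday timer and GainMoney handle income to TotalMoney.
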(event `self.ReceiveBeginPlay`
  (bind _asbp_player_controller (cast `/Game/Blueprints/Player/BP_PlayerController` (`GameplayStatics.GetPlayerController` 0)))
  (`EnhancedInputSubsystemInterface.AddMappingContext` (pcsubsystem `EnhancedInputLocalPlayerSubsystem` _asbp_player_controller) "/Game/Editor/Input/Secret/IMC_Secret.IMC_Secret" 0 (struct))
  (set `PlayerController.bShowMouseCursor` true (`GameplayStatics.GetPlayerController` 0))
  (bind _returnvalue (`|CreateWidget` "/Game/Editor/Blueprints/Secret/UW_Secret.UW_Secret_C"))
  (`UserWidget.AddToViewport` _returnvalue 0)
  (bind _outactors (`GameplayStatics.GetAllActorsOfClass` "/Script/Engine.TargetPoint"))
  (set `self.Spawns` _outactors)
  (`KismetSystemLibrary.K2_SetTimerDelegate` (delegate `Payday`) 20.0 true))

(event `Payday`
  (`/Game/BasicFunctions.+= (float)` 200.0 (`self.TotalMoney`)))

(event `EnhancedInput|/Game/Editor/Input/Secret/IA_SelectionToggle`
  (params (ActionValue :type Boolean) (ElapsedSeconds :type "Float (double-precision)") (TriggeredSeconds :type "Float (double-precision)") (InputAction :type "InputAction Object Reference" :default "/Game/Editor/Input/Secret/IA_SelectionToggle.IA_SelectionToggle"))
  (:`Triggered`
    (if (>= (- (`self.TotalMoney`) (`self.CurrentBet`)) 0.0)
      (`/Game/BasicFunctions.-= (float)` (`self.TotalMoney`) (`self.CurrentBet`))
      (`|SpawnActorFromClass` "/Game/Editor/Blueprints/Secret/BP_Ball.BP_Ball_C" (`self.GetTransform` (`KismetArrayLibrary.Array_Random` (`self.Spawns`))) "AlwaysSpawn" "MultiplyWithRoot" null (`self.CurrentBet`) null))))

(fn `GainMoney`
  (params (Amount :type "Float (double-precision)"))
  (`/Game/BasicFunctions.+= (float)` (`self.TotalMoney`) Amount))

(fn `UserConstructionScript`)