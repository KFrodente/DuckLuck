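; BP_Ball is a ball actor in the secret minigame that pays out money when it lands in a score box.
; On BeginPlay it gives its point light a random color.
; Overlapping a BP_ScoreBox awards the ball's Worth times that box's ScoreMult to the BP_SecretPlayer, found by class lookup, then destroys the ball.
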(event `self.ReceiveBeginPlay`
  (`LightComponent.SetLightColor` (`self.PointLight`) (make `LinearColor` (`KismetMathLibrary.RandomFloat`) (`KismetMathLibrary.RandomFloat`) (`KismetMathLibrary.RandomFloat`) 1.0) true))

(event `self.ReceiveActorBeginOverlap`
  (params (OtherActor :type "Actor Object Reference"))
  (bind _asbp_score_box (cast `/Game/Editor/Blueprints/Secret/BP_ScoreBox` OtherActor))
  (bind _returnvalue (`GameplayStatics.GetActorOfClass` "/Game/Editor/Blueprints/Secret/BP_SecretPlayer.BP_SecretPlayer_C"))
  (`/Game/Editor/Blueprints/Secret/BP_SecretPlayer.GainMoney` _returnvalue (* (`self.Worth`) (`/Game/Editor/Blueprints/Secret/BP_ScoreBox.ScoreMult` _asbp_score_box)))
  (`self.K2_DestroyActor`))

(fn `UserConstructionScript`)