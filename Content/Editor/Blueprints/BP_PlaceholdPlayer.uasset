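; Placeholder player pawn for an in-game editor, judging by its name and assets, that flies the view around with Enhanced Input.
; On BeginPlay it requires BP_PlayerController, adds the IMC_Editor mapping context, shows the mouse cursor and opens the UW_EditorActorSelect widget.
; FloatingPawnMovement receives movement input on the world XZ plane and zoom input as movement along world Y.
; The select input is bound but does nothing.
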(event `self.ReceiveBeginPlay`
  (bind _asbp_player_controller (cast `/Game/Blueprints/Player/BP_PlayerController` (`GameplayStatics.GetPlayerController` 0)))
  (`EnhancedInputSubsystemInterface.AddMappingContext` (pcsubsystem `EnhancedInputLocalPlayerSubsystem` _asbp_player_controller) "/Game/Editor/Input/IMC_Editor.IMC_Editor" 0 (struct))
  (set `PlayerController.bShowMouseCursor` true (`GameplayStatics.GetPlayerController` 0))
  (bind _returnvalue (`|CreateWidget` "/Game/Editor/UI/UW_EditorActorSelect.UW_EditorActorSelect_C"))
  (`UserWidget.AddToViewport` _returnvalue 0))

(event `EnhancedInput|/Game/Editor/Input/IA_EMovement`
  (params (ActionValue :type "Vector2D Structure") (ElapsedSeconds :type "Float (double-precision)") (TriggeredSeconds :type "Float (double-precision)") (InputAction :type "InputAction Object Reference" :default "/Game/Editor/Input/IA_EMovement.IA_EMovement"))
  (bind (_x _y) (`KismetMathLibrary.BreakVector2D` ActionValue))
  (:`Triggered`
    (`PawnMovementComponent.AddInputVector` (`self.FloatingPawnMovement`) (`KismetMathLibrary.MakeVector` (* _x 100.0) 0.0 (* _y 100.0)) false)))

(event `EnhancedInput|/Game/Editor/Input/IA_EZoom`
  (params (ActionValue :type "Float (double-precision)") (ElapsedSeconds :type "Float (double-precision)") (TriggeredSeconds :type "Float (double-precision)") (InputAction :type "InputAction Object Reference" :default "/Game/Editor/Input/IA_EZoom.IA_EZoom"))
  (:`Triggered`
    (`PawnMovementComponent.AddInputVector` (`self.FloatingPawnMovement`) (`KismetMathLibrary.MakeVector` 0.0 (* ActionValue 100.0)) false)))

(event `EnhancedInput|/Game/Editor/Input/IA_ESelect`
  (params (ActionValue :type Boolean) (ElapsedSeconds :type "Float (double-precision)") (TriggeredSeconds :type "Float (double-precision)") (InputAction :type "InputAction Object Reference" :default "/Game/Editor/Input/IA_ESelect.IA_ESelect")))

(fn `UserConstructionScript`)