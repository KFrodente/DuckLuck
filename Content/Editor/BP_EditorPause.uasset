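; BP_EditorPause is the editor's pause menu actor, offering Resume, Wake Up (main menu) and Exit Game buttons.
; On BeginPlay it spawns each menu-item actor at its placeholder component's transform, then links them into a wrapping adjacency loop.
; GetNextBox moves the selection along that adjacency from the sign of a direction's X and Y, and ResetSelection returns it to Resume.
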(event `self.ReceiveBeginPlay`
  (`|ExecutionSequence`
    (:`then_0`
      (bind _returnvalue (`|SpawnActorFromClass` "/Game/Blueprints/Inventory/Boxes/MenuPieces/BP_MenuItem_ResumeGame_Editor.BP_MenuItem_ResumeGame_Editor_C" (`SceneComponent.K2_GetComponentToWorld` (`self.Resume`)) "Undefined" "MultiplyWithRoot" null (struct) null))
      (set `self.ResumeButton` _returnvalue)
      (bind _returnvalue_2 (`|SpawnActorFromClass` "/Game/Blueprints/Inventory/Boxes/MenuPieces/BP_MenuItem_MainMenu.BP_MenuItem_MainMenu_C" (`SceneComponent.K2_GetComponentToWorld` (`self.WakeUp`)) "Undefined" "MultiplyWithRoot" null (struct) null))
      (set `self.WakeUpButton` _returnvalue_2)
      (bind _returnvalue_3 (`|SpawnActorFromClass` "/Game/Blueprints/Inventory/Boxes/MenuPieces/BP_MenuItem_ExitGame.BP_MenuItem_ExitGame_C" (`SceneComponent.K2_GetComponentToWorld` (`self.ExitGame`)) "Undefined" "MultiplyWithRoot" null (struct) null))
      (set `self.ExitGameButton` _returnvalue_3))
    (:`then_1`
      (set `/Game/Blueprints/Inventory/Boxes/BP_MenuItem_Base.AdjacentButtons` (make `/Game/Blueprints/Inventory/S_SurroundingButtons` (`self.ExitGameButton`) (`self.WakeUpButton`) null null) (`self.ResumeButton`))
      (set `/Game/Blueprints/Inventory/Boxes/BP_MenuItem_Base.AdjacentButtons` (make `/Game/Blueprints/Inventory/S_SurroundingButtons` (`self.ResumeButton`) (`self.ExitGameButton`) null null) (`self.WakeUpButton`))
      (set `/Game/Blueprints/Inventory/Boxes/BP_MenuItem_Base.AdjacentButtons` (make `/Game/Blueprints/Inventory/S_SurroundingButtons` (`self.WakeUpButton`) (`self.ResumeButton`) null null) (`self.ExitGameButton`)))))

(fn `GetNextBox`
  (params (Dir :type "Vector Structure") (Dir_X :type "Float (double-precision)" :default 0.0) (Dir_Y :type "Float (double-precision)" :default 0.0) (Dir_Z :type "Float (double-precision)" :default 0.0))
  (bind (_adjacentbuttons_up _adjacentbuttons_down) (break `/Game/Blueprints/Inventory/S_SurroundingButtons` (`/Game/Blueprints/Inventory/Boxes/BP_MenuItem_Base.AdjacentButtons` (`self.CurrentSelection`))))
  (bind (_adjacentbuttons_up_2 _adjacentbuttons_down_2 _adjacentbuttons_left _adjacentbuttons_right) (break `/Game/Blueprints/Inventory/S_SurroundingButtons` (`/Game/Blueprints/Inventory/Boxes/BP_MenuItem_Base.AdjacentButtons` (`self.CurrentSelection`))))
  (bind _returnvalue (select `int` (+ (`KismetMathLibrary.Round` (`KismetMathLibrary.SignOfFloat` Dir_Y)) 1) :`0` _adjacentbuttons_down :`1` null :`2` _adjacentbuttons_up))
  (bind _returnvalue_2 (select `int` (+ (`KismetMathLibrary.Round` (`KismetMathLibrary.SignOfFloat` Dir_X)) 1) :`0` _adjacentbuttons_left :`1` null :`2` _adjacentbuttons_right))
  (`/Engine/EditorBlueprintResources/StandardMacros.IsValid` _returnvalue_2
    (:`Is Valid`
      (`/Game/Blueprints/Inventory/Boxes/BP_MenuItem_Base.SetSelected` _returnvalue_2 true)
      (`/Game/Blueprints/Inventory/Boxes/BP_MenuItem_Base.SetSelected` (`self.CurrentSelection`) false)
      (set `self.CurrentSelection` _returnvalue_2))
    (:`Is Not Valid`
      _))
  (`/Engine/EditorBlueprintResources/StandardMacros.IsValid` _returnvalue
    (:`Is Valid`
      (`/Game/Blueprints/Inventory/Boxes/BP_MenuItem_Base.SetSelected` _returnvalue true)
      (`/Game/Blueprints/Inventory/Boxes/BP_MenuItem_Base.SetSelected` (`self.CurrentSelection`) false)
      (set `self.CurrentSelection` _returnvalue))))

(fn `ResetSelection`
  (bind _resumebutton (`self.ResumeButton`))
  (`/Game/Blueprints/Inventory/Boxes/BP_MenuItem_Base.SetSelected` _resumebutton true)
  (set `self.CurrentSelection` _resumebutton)
  (`/Game/Blueprints/Inventory/Boxes/BP_MenuItem_Base.SetSelected` (`self.WakeUpButton`) false)
  (`/Game/Blueprints/Inventory/Boxes/BP_MenuItem_Base.SetSelected` (`self.ExitGameButton`) false))

(fn `UserConstructionScript`)