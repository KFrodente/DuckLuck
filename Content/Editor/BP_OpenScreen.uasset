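; BP_OpenScreen is an actor that plays an expanding radial opening effect on a plane through material parameters.
; Construction passes the arrow's location to the material as "PL".
; Open enables tick, which eases "OuterRadius" toward a large target, then hides the plane and stops ticking past a threshold.
; Reset zeroes the material radius and shows the plane, but leaves the stored radius variable unchanged.
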(event `Open`
  (set `self.OpenScreen` true)
  (`self.SetActorTickEnabled` true))

(event `self.ReceiveTick`
  (params (DeltaSeconds :type "Float (single-precision)"))
  (if (`self.OpenScreen`)
    (bind _output_get (set `self.RadiusDefaultValue` (`KismetMathLibrary.FInterpTo` (`self.RadiusDefaultValue`) 15000.0 (`GameplayStatics.GetWorldDeltaSeconds`) 1.0)))
    (`MeshComponent.SetScalarParameterValueOnMaterials` (`self.Plane`) "OuterRadius" _output_get)
    (if (>= _output_get 13000.0)
      (`KismetSystemLibrary.K2_ClearAndInvalidateTimerHandle` (`self.WidenTimer`))
      (`SceneComponent.SetVisibility` (`self.Plane`) false false)
      (`self.SetActorTickEnabled` false))))

(fn `Reset`
  (set `self.OpenScreen` false)
  (`MeshComponent.SetScalarParameterValueOnMaterials` (`self.Plane`) "OuterRadius" 0.0)
  (`SceneComponent.SetVisibility` (`self.Plane`) true false))

(fn `UserConstructionScript`
  (`MeshComponent.SetVectorParameterValueOnMaterials` (`self.Plane`) "PL" (`SceneComponent.K2_GetComponentLocation` (`self.Arrow`))))