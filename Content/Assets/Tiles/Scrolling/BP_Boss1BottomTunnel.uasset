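; Boss 1 bottom tunnel actor that scrolls upward once activated and stops at a fixed height.
; Tick raises it by a fixed step per frame, not scaled by delta time, then snaps it into place at the threshold.
; On arrival it disables its tick, shakes the global camera, retargets it to the player and destroys BlackWall-tagged actors.
; Logic to position and activate the Boss 1 interlude is present but never runs.
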(event `activate`
  (set `self.Activated` true))

(event `DeActivate`
  (set `self.Activated` false)
  (`self.SetActorTickEnabled` false))

(event `self.ReceiveTick`
  (params (DeltaSeconds :type "Float (single-precision)"))
  (bind (_returnvalue_x _returnvalue_y _returnvalue_z) (`KismetMathLibrary.BreakVector` (`self.K2_GetActorLocation`)))
  (if (`self.Activated`)
    (`self.K2_SetActorLocation` (+ (`self.K2_GetActorLocation`) (0.0 0.0 100.0)))
    (if (>= _returnvalue_z -76224.0)
      (`self.K2_SetActorLocation` (`KismetMathLibrary.MakeVector` _returnvalue_x 0.0 -76320.0) false true)
      (`/Engine/EditorBlueprintResources/StandardMacros.DoOnce` false
        (:`Completed`
          (`self.DeActivate`)
          (bind _returnvalue (`GameplayStatics.GetActorOfClass` "/Game/Blueprints/World/BP_GlobalCamera.BP_GlobalCamera_C"))
          (`/Game/Blueprints/World/BP_GlobalCamera.ScreenShake` _returnvalue 500.0 500.0 0.02 0.2)
          (bind _returnvalue_2 (`GameplayStatics.GetActorOfClass` "/Game/Blueprints/Player/BP_PlayerWithHat.BP_PlayerWithHat_C"))
          (set `/Game/Blueprints/World/BP_GlobalCamera.CurrentFollowTarget` _returnvalue_2 _returnvalue)
          (set `/Game/Blueprints/World/BP_GlobalCamera.CurrentFollowDistance` (0.0 1000.0 0.0) _returnvalue)
          (bind _outactors (`GameplayStatics.GetAllActorsWithTag` "BlackWall"))
          (`self.K2_DestroyActor` _outactors)
          (`self.DeActivate`))))))

(fn `UserConstructionScript`)