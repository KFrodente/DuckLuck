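; BP_Boss1Interlude is a scrolling actor, apparently the interlude segment for the first boss.
; While activated, it moves up the Z axis by a fixed step each tick, without delta-time scaling.
; On reaching a hard-coded height, it teleports to a slightly lower fixed Z, then a DoOnce deactivates it and disables its tick.
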(event `activate`
  (set `self.Activated` true))

(event `DeActivate`
  (set `self.Activated` false)
  (`self.SetActorTickEnabled` false))

(event `self.ReceiveTick`
  (params (DeltaSeconds :type "Float (single-precision)"))
  (bind (_returnvalue_x _returnvalue_y _returnvalue_z) (`KismetMathLibrary.BreakVector` (`self.K2_GetActorLocation`)))
  (if (`self.Activated`)
    (`self.K2_SetActorLocation` (+ (`self.K2_GetActorLocation`) (0.0 0.0 100.0)))
    (if (>= _returnvalue_z -76224.0)
      (`self.K2_SetActorLocation` (`KismetMathLibrary.MakeVector` _returnvalue_x 0.0 -76320.0) false true)
      (`/Engine/EditorBlueprintResources/StandardMacros.DoOnce` false
        (:`Completed`
          (`self.DeActivate`))))))

(fn `UserConstructionScript`)