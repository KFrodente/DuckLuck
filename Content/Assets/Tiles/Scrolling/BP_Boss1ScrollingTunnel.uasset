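; BP_Boss1ScrollingTunnel is a tunnel chunk for the first boss that scrolls upward to form a self-extending tunnel.
; Activate registers the chunk as BP_Boss's LowestTunnelChunk and starts a timer that destroys it.
; While active, it moves up a fixed step each Tick, unscaled by delta time.
; If SpawnsAnother is set, the player's first Box overlap spawns and activates the next chunk at the Arrow transform.
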(event `activate`
  (`KismetSystemLibrary.K2_SetTimerDelegate` (delegate `die`) 5.0 true (`self.Initial Start Delay`))
  (set `self.Activated` true)
  (bind _returnvalue (`GameplayStatics.GetActorOfClass` "/Game/Blueprints/Enemies/Boss/BP_Boss.BP_Boss_C"))
  (set `/Game/Blueprints/Enemies/Boss/BP_Boss.LowestTunnelChunk` self _returnvalue))

(event `die`
  (`self.K2_DestroyActor`))

(event `self.ReceiveTick`
  (params (DeltaSeconds :type "Float (single-precision)"))
  (if (`self.Activated`)
    (`self.K2_SetActorLocation` (+ (`self.K2_GetActorLocation`) (0.0 0.0 100.0)))))

(event `self.Box.OnComponentBeginOverlap`
  (params (OverlappedComponent :type "PrimitiveComponent Object Reference") (OtherActor :type "Actor Object Reference") (OtherComp :type "PrimitiveComponent Object Reference") (OtherBodyIndex :type Integer) (bFromSweep :type Boolean) (SweepResult :type "HitResult Structure (by ref)"))
  (if (`self.SpawnsAnother`)
    (cast `/Game/Blueprints/Player/BP_PlayerWithHat` OtherActor)
    (`/Engine/EditorBlueprintResources/StandardMacros.DoOnce` false
      (:`Completed`
        (bind _returnvalue (`|SpawnActorFromClass` "BP_Boss1ScrollingTunnel_C" (`SceneComponent.K2_GetComponentToWorld` (`self.Arrow`)) "Undefined" "MultiplyWithRoot" null true null))
        (`self.activate` _returnvalue)))))

(fn `UserConstructionScript`)