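; Basic trigger component for the player's gun, firing bullets with sound and camera shake while the hat is powered.
; Fire input passes a DoOnce and Gate into the gun's BulletManager, using BP_Gun's stats and a spawn transform.
; Timers drive follow-up burst shots, held-fire rate and automatic reload on empty ammo.
; A fresh press clears the fire-rate timer, so tapping can outpace holding, but active bursts block new shots.
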(event `self.ReceiveBeginPlay`
  (bind _returnvalue (`GameplayStatics.GetActorOfClass` "/Game/Blueprints/Weapons/Gun/BP_Gun.BP_Gun_C"))
  (`/Engine/EditorBlueprintResources/StandardMacros.IsValid` _returnvalue
    (:`Is Valid`
      (set `self.GunReference` _returnvalue)
      (bind _asbp_player_with_hat (cast `/Game/Blueprints/Player/BP_PlayerWithHat` (`self.GetOwner`)))
      (set `self.PlayerReference` _asbp_player_with_hat)
      (`self.Reload`))
    (:`Is Not Valid`
      (`KismetSystemLibrary.PrintString` "Something went wrong finding basic trigger in Basic trigger component"))))

(event `ShootAgain`
  (bind _playerreference (`self.PlayerReference`))
  (bind _gunreference (`self.GunReference`))
  (bind _gunreference_2 (`self.GunReference`))
  (bind _aimdir (`/Game/Blueprints/Player/BP_PlayerWithHat.AimDir` _playerreference))
  (bind _bulletsperspread (`Gun.bulletsPerSpread` _gunreference_2))
  (bind _fireagain (`/Game/Blueprints/Bullets/BP_BulletManager.SpawnBullet` (`/Game/Blueprints/Weapons/Gun/BP_Gun.BulletManager` _gunreference_2) (`KismetMathLibrary.MakeTransform` (+ (`Actor.K2_GetActorLocation` _playerreference) (* (select `bool` (== _aimdir (0.0 0.0 0.0)) :`false` _aimdir :`true` (select `bool` (`/Game/Blueprints/Player/BP_PlayerWithHat.FacingRight` _playerreference) :`false` (-1.0 0.0 0.0) :`true` (1.0 0.0 0.0) :!type "Vector Structure")) 60.0)) (`SceneComponent.K2_GetComponentRotation` (`/Game/Blueprints/Player/BP_PlayerWithHat.GunSection` _playerreference))) (`Gun.bulletVelocity` _gunreference_2) (`Gun.bulletDamage` _gunreference_2) (`Gun.burstAmount` _gunreference_2) _bulletsperspread (select `int` (- _bulletsperspread 1) :`0` 0.0 :`1` 7.0 :`2` 4.8 :`3` 1.5 :`4` 1.5 :`5` 0.0 :`6` 0.0 :`7` -1.0) (`Gun.spreadAngle` _gunreference_2) (`Gun.additionalBulletSize` _gunreference_2) (`Gun.damagePerCharge` _gunreference_2) (`Gun.velocityModPerCharge` _gunreference_2) 0 false 0 (`self.PlayerReference`) "/Game/Blueprints/Bullets/BP_Bullet_Base.BP_Bullet_Base_C" null 0.0 0.0 0.0 0.0 0.0 0.0 0.0 :!label _label))
  (`GameplayStatics.PlaySound2D` "/Game/Assets/Audio/Weapons/Basic/DLSE_BasicGun_Cue.DLSE_BasicGun_Cue" 1.0 (`KismetMathLibrary.RandomFloatInRange` 1.2 1.5) 0.0 null null)
  (`/Game/Blueprints/World/BP_GlobalCamera.ScreenShake` (`/Game/Blueprints/Player/BP_PlayerWithHat.GlobalCameraRef` (`self.PlayerReference`)) 5.0 5.0 0.02 0.06)
  (if _fireagain
    (bind _returnvalue (`KismetSystemLibrary.K2_SetTimerDelegate` (delegate `ShootAgain`) (`Gun.timeBetweenBursts` (`self.GunReference`))))
    (set `self.BurstTimer` _returnvalue)
    (elif (<= (`self.Ammo`) 0)
      (bind _returnvalue_2 (`KismetSystemLibrary.K2_SetTimerDelegate` (`|CreateDelegate` :!event `Reload`) (`Gun.reloadSpeed` _gunreference)))
      (set `self.ReloadTimer` _returnvalue_2)
      (goto _label_4 :!via `Close`)
      (else
        (bind _returnvalue_3 (`KismetSystemLibrary.K2_SetTimerDelegate` (`|CreateDelegate` :!event `Firerate`) (`Gun.fireRate` _gunreference)))
        (set `self.FirerateTimer` _returnvalue_3)))))

(event `Reload`
  (set `self.Ammo` (`Gun.bulletsPerReload` (`self.GunReference`)))
  (`|ExecutionSequence`
    (:`then_0`
      (goto _label_4 :!via `Open`))
    (:`then_1`
      (goto _label_3 :!via `Reset`))))

(event `EnhancedInput|/Game/Blueprints/Input/Player/IA_FireGun`
  (params (ActionValue :type Boolean) (ElapsedSeconds :type "Float (double-precision)") (TriggeredSeconds :type "Float (double-precision)") (InputAction :type "InputAction Object Reference" :default "/Game/Blueprints/Input/Player/IA_FireGun.IA_FireGun"))
  (:`Triggered`
    (if (and (`self.Active`) (`/Game/Blueprints/Player/BP_PlayerWithHat.HatPowered` (`self.PlayerReference`)) (not (`KismetSystemLibrary.K2_IsTimerActiveHandle` (`self.BurstTimer`)))) :!label _label_2
      (`/Engine/EditorBlueprintResources/StandardMacros.DoOnce` false :!label _label_3
        (:`Completed`
          (`/Engine/EditorBlueprintResources/StandardMacros.Gate` false :!label _label_4
            (:`Exit`
              (if ActionValue
                (`/Game/BasicFunctions.-= (int)` (`self.Ammo`) 1)
                (goto _label))))))))
  (:`Started`
    (`|ExecutionSequence`
      (:`then_0`
        (goto _label_3 :!via `Reset`))
      (:`then_1`
        (`KismetSystemLibrary.K2_ClearAndInvalidateTimerHandle` (`self.FirerateTimer`))
        (goto _label_2)))))

(event `Firerate`
  (goto _label_3 :!via `Reset`))

(fn `ActivateTrigger`
  (bind _asbp_player_controller (cast `/Game/Blueprints/Player/BP_PlayerController` (`GameplayStatics.GetPlayerController` 0)))
  (bind _returnvalue (pcsubsystem `EnhancedInputLocalPlayerSubsystem` _asbp_player_controller))
  (`EnhancedInputSubsystemInterface.RemoveMappingContext` _returnvalue "/Game/Blueprints/Input/Player/IMC_Gun.IMC_Gun" (struct))
  (`EnhancedInputSubsystemInterface.AddMappingContext` _returnvalue "/Game/Blueprints/Input/Player/IMC_Gun.IMC_Gun" 1 (struct)))