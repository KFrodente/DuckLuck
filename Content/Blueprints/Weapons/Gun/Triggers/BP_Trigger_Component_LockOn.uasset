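; Lock-on gun trigger component for the hat player that marks enemies while fire is held and shoots homing bullets at them on release.
; Holding fire runs a looping timer that grows a pulsing overlap sphere, collecting enemies up to MaxTargets and showing debug circles.
; On release, if the hat is powered, the gun's BulletManager fires tracking bullets at each target in turn.
; Timers space bursts and apply the fire-rate cooldown.
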(event `DoSearch`
  (bind _gunreference (`self.GunReference`))
  (bind _foundenemies (`self.FoundEnemies`))
  (bind _returnvalue (`Actor.K2_GetActorLocation` (`self.PlayerReference`)))
  (bind _returnvalue_2 (`KismetMathLibrary.FInterpTo` (`self.CurrentCircleRadius`) (`Gun.searchSize` _gunreference) (`GameplayStatics.GetWorldDeltaSeconds`) (`Gun.searchSpeed` _gunreference)))
  (if (and (`self.Active`) (`self.Search`))
    (bind _outactors (`KismetSystemLibrary.SphereOverlapActors` _returnvalue _returnvalue_2 (`self.EnemySearch`)))
    (`KismetSystemLibrary.DrawDebugCircle` _returnvalue _returnvalue_2 12 (struct :`R` 0.432794 :`G` 0.930176 :`B` 1.0 :`A` 1.0) 0.2 3.0 (0.0 0.0 1.0) (1.0 0.0 0.0))
    (bind _output_get (set `self.CurrentCircleRadius` _returnvalue_2))
    (if (<= (`KismetMathLibrary.Abs` (- (`Gun.searchSize` (`self.GunReference`)) _output_get)) 5.0)
      (set `self.CurrentCircleRadius` 0.0))
    (for _array_element _outactors
      (if (< (`KismetArrayLibrary.Array_Length` _foundenemies) (`Gun.maxTargets` (`self.GunReference`)))
        (bind _asbp_enemy_base (cast `/Game/Blueprints/Enemies/BP_Enemy_Base` _array_element))
        (`KismetArrayLibrary.Array_AddUnique` _foundenemies _asbp_enemy_base)))
    (for _array_element_2 (`self.FoundEnemies`)
      ;[1 1 1] Highlight found enemies
      (`KismetSystemLibrary.DrawDebugCircle` (`Actor.K2_GetActorLocation` _array_element_2) 35.0 12 (struct :`R` 1.0 :`G` 0.277561 :`B` 0.34731 :`A` 1.0) 0.1 2.0 (0.0 0.0 1.0) (1.0 0.0 0.0)))))

(event `Firerate`
  (goto _label :!via `Reset`))

(event `EnhancedInput|/Game/Blueprints/Input/Player/IA_FireGun`
  (params (ActionValue :type Boolean) (ElapsedSeconds :type "Float (double-precision)") (TriggeredSeconds :type "Float (double-precision)") (InputAction :type "InputAction Object Reference" :default "/Game/Blueprints/Input/Player/IA_FireGun.IA_FireGun"))
  (bind _playerreference (`self.PlayerReference`))
  (bind _gunreference (`self.GunReference`))
  (bind _returnvalue (`Actor.K2_GetActorLocation` _playerreference))
  (:`Triggered`
    (if (`self.Active`)
      (`/Engine/EditorBlueprintResources/StandardMacros.DoOnce` false :!label _label
        (:`Completed`
          (set `self.Search` true)
          (bind _returnvalue_2 (`KismetSystemLibrary.K2_SetTimerDelegate` (`|CreateDelegate` :!event `DoSearch`) 0.025 true))
          (set `self.SearchTimer` _returnvalue_2)))))
  (:`Canceled`
    (if (and (`self.Active`) (`/Game/Blueprints/Player/BP_PlayerWithHat.HatPowered` (`self.PlayerReference`))) :!label _label_2
      (set `self.Search` false)
      (`KismetSystemLibrary.K2_ClearAndInvalidateTimerHandle` (`self.SearchTimer`))
      (set `self.CurrentCircleRadius` 0.0)
      (if (> (`KismetArrayLibrary.Array_Length` (`self.FoundEnemies`)) 0)
        (bind _fireagain (`/Game/Blueprints/Bullets/BP_BulletManager.SpawnBullet` (`/Game/Blueprints/Weapons/Gun/BP_Gun.BulletManager` (`self.GunReference`)) (`KismetMathLibrary.MakeTransform` (+ _returnvalue (* (`/Game/Blueprints/Player/BP_PlayerWithHat.AimDir` _playerreference) 25.0)) (`KismetMathLibrary.FindLookAtRotation` _returnvalue (`Actor.K2_GetActorLocation` (`|GetArrayItem` (`self.FoundEnemies`) (`self.CurrentFiringIndex`))))) (+ (`Gun.bulletVelocity` _gunreference) (* (`Gun.velocityModPerCharge` _gunreference) (`KismetArrayLibrary.Array_Length` (`self.FoundEnemies`)))) (+ (`Gun.bulletDamage` _gunreference) (* (`Gun.damagePerCharge` _gunreference) (`KismetArrayLibrary.Array_Length` (`self.FoundEnemies`)))) (`Gun.burstAmount` _gunreference) (`Gun.bulletsPerSpread` _gunreference) 0.0 (`Gun.spreadAngle` _gunreference) (* (`Gun.additionalBulletSize` _gunreference) (`KismetArrayLibrary.Array_Length` (`self.FoundEnemies`))) 0.0 0.0 0 false 0 (`self.PlayerReference`) "/Game/Blueprints/Bullets/BP_Bullet_Tracking.BP_Bullet_Tracking_C" (`|GetArrayItem` (`self.FoundEnemies`) (`self.CurrentFiringIndex`)) :!label _label_3))
        ;[0.07878 0.1719 0.09399 0.435] If it goes through output node that means it is firing at the next enemy
        (if _fireagain
          (`KismetSystemLibrary.K2_SetTimerDelegate` (`|CreateDelegate` :!event `ShootAgain`) (`Gun.timeBetweenBursts` (`self.GunReference`)))
          (elif (== (`self.CurrentFiringIndex`) (- (`KismetArrayLibrary.Array_Length` (`self.FoundEnemies`)) 1))
            (`KismetSystemLibrary.K2_SetTimerDelegate` (`|CreateDelegate` :!event `Firerate`) (`Gun.fireRate` (`self.GunReference`)))
            (`KismetArrayLibrary.Array_Clear` (`self.FoundEnemies`))
            (set `self.CurrentFiringIndex` 0)
            (else
              (`/Engine/EditorBlueprintResources/StandardMacros.IncrementInt` (`self.CurrentFiringIndex`)
                (:`  `
                  (goto _label_3))))))
        (else
          (goto _label :!via `Reset`)))))
  (:`Completed`
    (goto _label_2)))

(event `ShootAgain`
  (goto _label_3))

(event `self.ReceiveBeginPlay`
  (`parent.ReceiveBeginPlay`)
  (bind _returnvalue (`GameplayStatics.GetActorOfClass` "/Game/Blueprints/Weapons/Gun/BP_Gun.BP_Gun_C"))
  (`/Engine/EditorBlueprintResources/StandardMacros.IsValid` _returnvalue
    (:`Is Valid`
      (set `self.GunReference` _returnvalue)
      (bind _asbp_player_with_hat (cast `/Game/Blueprints/Player/BP_PlayerWithHat` (`self.GetOwner`)))
      (bind _output_get (set `self.PlayerReference` _asbp_player_with_hat))
      (`KismetArrayLibrary.Array_Add` (`self.Actors to Ignore`) _output_get))))