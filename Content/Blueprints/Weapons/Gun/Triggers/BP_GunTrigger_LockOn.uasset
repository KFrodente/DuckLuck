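; Gun trigger variant that gathers lock-on targets around the player while triggered and fires at them when not triggered.
; DoFireSequence stores the results of a fixed-radius sphere overlap on the player pawn and draws a debug circle, holding fire until the untriggered call passes those targets out at a constant charge level.
; Becoming the active trigger also activates the lock-on trigger component on BP_PlayerWithHat.
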(fn `DoFireSequence`
  (params (Triggered :type Boolean))
  (returns (ChargeLevel :type Integer) (FireGun :type Boolean) (Targets :type "Array of Actor Object Reference"))
  (bind _returnvalue (`self.K2_GetActorLocation` (`GameplayStatics.GetPlayerPawn` 0)))
  (if Triggered
    (bind _outactors (`KismetSystemLibrary.SphereOverlapActors` _returnvalue 500.0 (`self.Object Types`)))
    (`KismetSystemLibrary.DrawDebugCircle` _returnvalue 500.0 12 (struct :`R` 1.0 :`G` 0.745305 :`B` 0.382669 :`A` 1.0) 0.1 2.0 (0.0 0.0 1.0) (1.0 0.0 0.0))
    (set `self.lockedOnTargets` _outactors)
    (return 1 false)
    (else
      (return 1 true (`self.lockedOnTargets`)))))

(fn `SetAsActiveTrigger`
  (`parent.SetAsActiveTrigger`)
  (bind _returnvalue (`GameplayStatics.GetActorOfClass` "/Game/Blueprints/Player/BP_PlayerWithHat.BP_PlayerWithHat_C"))
  (`/Engine/EditorBlueprintResources/StandardMacros.IsValid` _returnvalue
    (:`Is Valid`
      (bind _bp_trigger_component_lockon (`/Game/Blueprints/Player/BP_PlayerWithHat.BP_Trigger_Component_LockOn` _returnvalue))
      (set `/Game/Blueprints/Weapons/Gun/Triggers/BP_Trigger_Component_Base.Active` true _bp_trigger_component_lockon)
      (`/Game/Blueprints/Weapons/Gun/Triggers/BP_Trigger_Component_Base.ActivateTrigger` _bp_trigger_component_lockon))))

(fn `UserConstructionScript`
  (`parent.UserConstructionScript`))