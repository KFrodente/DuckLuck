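; Sword trigger component for the player's gun: holding fire builds charge, releasing it spawns slash projectiles, active only while the hat is powered.
; A looping-by-event timer adds charge levels up to the gun's maximum, with sound and shrinking intervals.
; Release spawns BP_Bullet_Slash through the gun's BulletManager using gun stats, with size scaled by charge.
; Chained timers handle bursts, repeat slashes per charge level, then apply the fire-rate cooldown.
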(event `Fire Rate`
  (bind _gunreference (`self.GunReference`))
  (goto _label_2 :!via `Reset`))

(event `AddCharge`
  (bind _gunreference (`self.GunReference`))
  (bind _result (`/Engine/EditorBlueprintResources/StandardMacros.IncrementInt` (`self.ChargeLevel`))
    (:`  `
      (`GameplayStatics.PlaySound2D` (`|GetArrayItem` (`self.SoundList`) _result) 1.0 1.0 0.0 null null false)
      (if (< (`self.ChargeLevel`) (`Gun.maxCharges` _gunreference)) :!label _label
        (bind _returnvalue (`KismetSystemLibrary.K2_SetTimerDelegate` (`|CreateDelegate` :!event `AddCharge`) (* (`Gun.chargeTime` _gunreference) (/ (`Gun.chargeTimeMod` _gunreference) (+ (`self.ChargeLevel`) 1)))))
        (set `self.ChargeTimer` _returnvalue)))))

(event `EnhancedInput|/Game/Blueprints/Input/Player/IA_FireGun`
  (params (ActionValue :type Boolean) (ElapsedSeconds :type "Float (double-precision)") (TriggeredSeconds :type "Float (double-precision)") (InputAction :type "InputAction Object Reference" :default "/Game/Blueprints/Input/Player/IA_FireGun.IA_FireGun"))
  (bind _playerreference (`self.PlayerReference`))
  (bind _gunreference (`self.GunReference`))
  (bind _gunreference_2 (`self.GunReference`))
  (bind _gunreference_3 (`self.GunReference`))
  (bind _gunreference_4 (`self.GunReference`))
  (bind _returnvalue (and (`self.Active`) (`/Game/Blueprints/Player/BP_PlayerWithHat.HatPowered` (`self.PlayerReference`))))
  (:`Triggered`
    (if _returnvalue
      (`/Engine/EditorBlueprintResources/StandardMacros.DoOnce` false :!label _label_2
        (:`Completed`
          (`/Engine/EditorBlueprintResources/StandardMacros.IncrementInt` (`self.ChargeLevel`)
            (:`  `
              (goto _label)))))))
  (:`Canceled`
    (if _returnvalue :!label _label_3
      (`KismetSystemLibrary.K2_ClearAndInvalidateTimerHandle` (`self.ChargeTimer`))
      (if (!= (`self.ChargeLevel`) 0)
        (bind _fireagain (`/Game/Blueprints/Bullets/BP_BulletManager.SpawnBullet` (`/Game/Blueprints/Weapons/Gun/BP_Gun.BulletManager` _gunreference_4) (`KismetMathLibrary.MakeTransform` (+ (`Actor.K2_GetActorLocation` _playerreference) (* (`/Game/Blueprints/Player/BP_PlayerWithHat.AimDir` _playerreference) 25.0)) (`SceneComponent.K2_GetComponentRotation` (`/Game/Blueprints/Player/BP_PlayerWithHat.GunSection` _playerreference))) (* (+ (`Gun.bulletVelocity` _gunreference_4) (* (`Gun.velocityModPerCharge` _gunreference_4) (`self.ChargeLevel`))) 0.25) (+ (`Gun.bulletDamage` _gunreference_3) (* (`Gun.damagePerCharge` _gunreference_3) (`self.ChargeLevel`))) (`Gun.burstAmount` _gunreference_2) (`Gun.bulletsPerSpread` _gunreference_2) 0.0 (`Gun.spreadAngle` _gunreference_2) (* (`Gun.additionalBulletSize` _gunreference_3) (`self.ChargeLevel`)) 1.0 1.0 0 false 0 (`self.PlayerReference`) "/Game/Blueprints/Bullets/BP_Bullet_Slash.BP_Bullet_Slash_C" null 0.0 0.0 0.0 0.0 0.0 0.0 0.0 :!label _label_4))
        (if _fireagain
          (`KismetSystemLibrary.K2_SetTimerDelegate` (`|CreateDelegate` :!event `Fire Again`) (`Gun.timeBetweenBursts` _gunreference))
          (elif (< (`self.TimesFired`) (- (`self.ChargeLevel`) 1))
            (`/Engine/EditorBlueprintResources/StandardMacros.IncrementInt` (`self.TimesFired`)
              (:`  `
                (`KismetSystemLibrary.K2_SetTimerDelegate` (`|CreateDelegate` :!event `Fire Again`) (* (`Gun.timeBetweenBursts` _gunreference) 0.5))))
            (else
              (`KismetSystemLibrary.K2_SetTimerDelegate` (`|CreateDelegate` :!event `Fire Rate`) (`Gun.fireRate` _gunreference))
              (set `self.ChargeLevel` 0)
              (set `self.TimesFired` 0))))
        (else
          (goto _label_2 :!via `Reset`)))))
  (:`Completed`
    (goto _label_3)))

(event `Fire Again`
  (goto _label_4))

(event `self.ReceiveBeginPlay`
  (bind _returnvalue (`GameplayStatics.GetActorOfClass` "/Game/Blueprints/Weapons/Gun/BP_Gun.BP_Gun_C"))
  (`/Engine/EditorBlueprintResources/StandardMacros.IsValid` _returnvalue
    (:`Is Valid`
      (set `self.GunReference` _returnvalue)
      (bind _asbp_player_with_hat (cast `/Game/Blueprints/Player/BP_PlayerWithHat` (`self.GetOwner`)))
      (set `self.PlayerReference` _asbp_player_with_hat))))