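; Gun trigger component for the hat-wearing player that charges a shot while fire is held and releases it when input ends, if the hat is powered.
; A re-armed timer raises ChargeLevel up to the gun's maximum with a sound per level, its interval varying with the level.
; Release spawns bullets through the gun's BulletManager, scaling additional size by charge, then timers handle bursts or fire-rate cooldown.
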(event `self.ReceiveBeginPlay`
  (`parent.ReceiveBeginPlay`)
  (bind _returnvalue (`GameplayStatics.GetActorOfClass` "/Game/Blueprints/Weapons/Gun/BP_Gun.BP_Gun_C"))
  (`/Engine/EditorBlueprintResources/StandardMacros.IsValid` _returnvalue
    (:`Is Valid`
      (set `self.GunReference` _returnvalue)
      (bind _asbp_player_with_hat (cast `/Game/Blueprints/Player/BP_PlayerWithHat` (`self.GetOwner`)))
      (set `self.PlayerReference` _asbp_player_with_hat))
    (:`Is Not Valid`
      (`KismetSystemLibrary.PrintString` "Something went wrong finding basic trigger in Basic trigger component"))))

(event `Firerate`
  (bind _gunreference (`self.GunReference`))
  (goto _label_3 :!via `Reset`))

(event `AddCharge`
  (bind _gunreference (`self.GunReference`))
  (bind _result (`/Engine/EditorBlueprintResources/StandardMacros.IncrementInt` (`self.ChargeLevel`))
    (:`  `
      (`GameplayStatics.PlaySound2D` (`|GetArrayItem` (`self.SoundList`) _result) 1.0 1.0 0.0 null null false)
      (if (< (`self.ChargeLevel`) (`Gun.maxCharges` _gunreference)) :!label _label
        (bind _returnvalue (`KismetSystemLibrary.K2_SetTimerDelegate` (`|CreateDelegate` :!event `AddCharge`) (* (`Gun.chargeTime` _gunreference) (/ (`Gun.chargeTimeMod` _gunreference) (+ (`self.ChargeLevel`) 1)))))
        (set `self.ChargeTimer` _returnvalue)))))

(event `ShootAgain`
  (bind _playerreference (`self.PlayerReference`))
  (bind _gunreference (`self.GunReference`))
  (bind _gunreference_2 (`self.GunReference`))
  (bind _gunreference_3 (`self.GunReference`))
  (bind _gunreference_4 (`self.GunReference`))
  (bind _bulletsperspread (`Gun.bulletsPerSpread` _gunreference_2))
  (bind _fireagain (`/Game/Blueprints/Bullets/BP_BulletManager.SpawnBullet` (`/Game/Blueprints/Weapons/Gun/BP_Gun.BulletManager` _gunreference_4) (`KismetMathLibrary.MakeTransform` (+ (`Actor.K2_GetActorLocation` _playerreference) (* (`/Game/Blueprints/Player/BP_PlayerWithHat.AimDir` _playerreference) 25.0)) (`SceneComponent.K2_GetComponentRotation` (`/Game/Blueprints/Player/BP_PlayerWithHat.GunSection` _playerreference))) (+ (`Gun.bulletVelocity` _gunreference_4) (* (`Gun.velocityModPerCharge` _gunreference_4) (`self.ChargeLevel`))) (+ (`Gun.bulletDamage` _gunreference_3) (* (`Gun.damagePerCharge` _gunreference_3) (`self.ChargeLevel`))) (`Gun.burstAmount` _gunreference_2) _bulletsperspread (select `int` (- _bulletsperspread 1) :`0` 0.0 :`1` 7.0 :`2` 4.5 :`3` 1.5 :`4` 1.5 :`5` 0.0 :`6` 0.0 :`7` -1.0) (`Gun.spreadAngle` _gunreference_2) (* (`Gun.additionalBulletSize` _gunreference_3) (`self.ChargeLevel`)) 1.0 1.0 0 false 0 (`self.PlayerReference`) "/Game/Blueprints/Bullets/BP_Bullet_Base.BP_Bullet_Base_C" null :!label _label_2))
  (if _fireagain
    (`KismetSystemLibrary.K2_SetTimerDelegate` (`|CreateDelegate` :!event `ShootAgain`) (`Gun.timeBetweenBursts` _gunreference))
    (else
      (`KismetSystemLibrary.K2_SetTimerDelegate` (`|CreateDelegate` :!event `Firerate`) (`Gun.fireRate` _gunreference))
      (set `self.ChargeLevel` 0))))

(event `EnhancedInput|/Game/Blueprints/Input/Player/IA_FireGun`
  (params (ActionValue :type Boolean) (ElapsedSeconds :type "Float (double-precision)") (TriggeredSeconds :type "Float (double-precision)") (InputAction :type "InputAction Object Reference" :default "/Game/Blueprints/Input/Player/IA_FireGun.IA_FireGun"))
  (:`Triggered`
    (if (`self.Active`)
      (`/Engine/EditorBlueprintResources/StandardMacros.DoOnce` false :!label _label_3
        (:`Completed`
          (goto _label)))))
  (:`Canceled`
    (if (and (`self.Active`) (`/Game/Blueprints/Player/BP_PlayerWithHat.HatPowered` (`self.PlayerReference`))) :!label _label_4
      (`KismetSystemLibrary.K2_ClearAndInvalidateTimerHandle` (`self.ChargeTimer`))
      (if (!= (`self.ChargeLevel`) 0)
        (goto _label_2)
        (else
          (goto _label_3 :!via `Reset`)))))
  (:`Completed`
    (goto _label_4)))

(fn `ActivateTrigger`
  (bind _asbp_player_controller (cast `/Game/Blueprints/Player/BP_PlayerController` (`Pawn.GetController` (`self.PlayerReference`))))
  (bind _returnvalue (pcsubsystem `EnhancedInputLocalPlayerSubsystem` _asbp_player_controller))
  (`EnhancedInputSubsystemInterface.RemoveMappingContext` _returnvalue "/Game/Blueprints/Input/Player/IMC_Gun.IMC_Gun" (struct))
  (`EnhancedInputSubsystemInterface.AddMappingContext` _returnvalue "/Game/Blueprints/Input/Player/IMC_Gun.IMC_Gun" 1 (struct)))