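; Base Blueprint for gun trigger parts, holding each part's unlock state and level.
; On BeginPlay it finds its matching ID in the game instance's GunParts data and loads that state through UseSaveData.
; GetSaveData returns the unlock state and level, but reports the ID as 0.
; DoFireSequence and SetAsActiveTrigger are stubs, with the fire sequence returning no charge and no shot.
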(event `self.ReceiveBeginPlay`
  (bind _savegamedata (message `/Game/Blueprints/SaveGame/BPI_SaveGame.GetGameData` (`GameplayStatics.GetGameInstance`)))
  (for _array_element (`/Game/Blueprints/SaveGame/BP_SaveGame.GunParts` _savegamedata)
    (if (== (`.ID_7_9F2B82FE416DDFE2686AA59F4BB58875` (break `/Game/Blueprints/SaveGame/S_GunPartData` _array_element)) (`self.ID`))
      (`self.UseSaveData` _array_element)
      (break))))

(fn `DoFireSequence`
  (params (Triggered :type Boolean))
  (returns (ChargeLevel :type Integer) (FireGun :type Boolean) (Targets :type "Array of Actor Object Reference"))
  (return 0 false))

(fn `GetSaveData`
  (returns (Data :type "/Game/Blueprints/SaveGame/S_GunPartData Structure"))
  (return (make `/Game/Blueprints/SaveGame/S_GunPartData` (`self.unlocked`) (`self.level`))))

(fn `SetAsActiveTrigger`)

(fn `UserConstructionScript`)

(fn `UseSaveData`
  (params (Data :type "/Game/Blueprints/SaveGame/S_GunPartData Structure"))
  (set `self.unlocked` Data_Unlocked_1_DBD524F14CEA6449E2FA35B2962A3AC7)
  (set `self.level` Data_Level_4_DCB0DF144A5180DCE07746986B70953C))