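; BP_GunTrigger_Charge is a charge-up gun trigger that builds charge while held and fires on release.
; DoFireSequence starts charging on press, then on release returns the held charge level with a fire signal.
; Tick raises the level using the parent Gun's charge settings, with the time threshold divided by the current level, and resets when not charging.
; A charge sound call is present but unconnected.
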(event `self.ReceiveTick`
  (params (DeltaSeconds :type "Float (single-precision)"))
  (if (`self.Charging`)
    (bind _asgun (cast `Gun` (`self.GetParentActor`)))
    (if (<= (`self.ChargeLevel`) (`Gun.maxCharges` _asgun))
      (bind _output_get (set `self.ChargeTime` (+ (`self.ChargeTime`) DeltaSeconds)))
      (if (>= _output_get (/ (`Gun.chargeTime` _asgun) (* (`Gun.chargeTimeMod` _asgun) (`self.ChargeLevel`))))
        (bind _result (`/Engine/EditorBlueprintResources/StandardMacros.IncrementInt` (`self.ChargeLevel`))
          (:`  `
            (set `self.ChargeTime` 0.0)))))
    (else
      (set `self.ChargeTime` 0.0)
      (set `self.ChargeLevel` 0))))

(fn `DoFireSequence`
  (params (Triggered :type Boolean))
  (returns (ChargeLevel :type Integer) (FireGun :type Boolean))
  (if Triggered
    (set `self.Charging` true)
    (return 0 false)
    (else
      (bind _output_get (set `self.HeldChargeLevel` (`self.ChargeLevel`)))
      (set `self.Charging` false)
      (return _output_get true))))

(fn `UserConstructionScript`
  (`parent.UserConstructionScript`))