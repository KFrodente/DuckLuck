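; Gun Blueprint that fires bullets with fire-rate cooldown, bursts, spread and charge scaling.
; FireGun asks a swappable Trigger whether to fire and at what charge level, then has BulletManager spawn bullets with charge-boosted velocity and damage and charge-scaled extra size.
; Charge is held across a burst, with FireAgain and a delay returned so the caller drives follow-up shots.
; Tick counts down the shared cooldown timer.
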(event `self.ReceiveTick`
  (params (DeltaSeconds :type "Float (single-precision)"))
  (if (> (`self.FirerateTimer`) 0.0)
    (bind _returnvalue (`StaticFunctionLibrary.MinusTimer` (`self.FirerateTimer`) DeltaSeconds))
    (set `self.FirerateTimer` _returnvalue)))

(fn `ChangeTrigger`
  (params (Trigger :type "/Game/Blueprints/Weapons/Gun/Triggers/BP_GunTrigger_Base Object Reference"))
  (set `self.Trigger` Trigger))

(fn `FireGun`
  (params (BulletTransform :type "Transform Structure") (Triggered :type Boolean))
  (returns (FireAgain :type Boolean) (Delay :type "Float (double-precision)"))
  (bind _timebetweenbursts (`self.timeBetweenBursts`))
  (bind _heldchargelevel (`self.HeldChargeLevel`))
  (if (<= (`self.FirerateTimer`) 0.0)
    (bind (_chargelevel _firegun) (`/Game/Blueprints/Weapons/Gun/Triggers/BP_GunTrigger_Base.DoFireSequence` (`self.Trigger`) Triggered))
    (if (== (`self.HeldChargeLevel`) 0)
      (set `self.HeldChargeLevel` _chargelevel))
    (if _firegun
      (bind _result (`/Engine/EditorBlueprintResources/StandardMacros.IncrementInt` (`self.TimesBurstFired`))
        (:`  `
          (`/Game/Blueprints/Bullets/BP_BulletManager.SpawnBullet` (`self.BulletManager`) BulletTransform (+ (`self.bulletVelocity`) (* (`self.velocityModPerCharge`) _heldchargelevel)) (+ (`self.bulletDamage`) (* (`self.damagePerCharge`) _heldchargelevel)) (`self.burstAmount`) (`self.bulletsPerSpread`) (`self.spreadAngle`) (* (`self.additionalBulletSize`) _heldchargelevel) 0.0 0.0 0 false 0)
          (if (< _result (`self.burstAmount`))
            (set `self.FirerateTimer` _timebetweenbursts)
            (return true _timebetweenbursts)
            (else
              (set `self.TimesBurstFired` 0)
              (set `self.HeldChargeLevel` 0)
              (set `self.FirerateTimer` (`self.fireRate`))
              (return false 0.0))))))))

(fn `UserConstructionScript`)