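; Weapon combo component that resolves a main and sub weapon number pair into a combo actor.
; On BeginPlay it spawns shared procedural pistol, shotgun and charge actors, plus one reusable base combo.
; CheckForProCombo copies weapon stats into those actors, returns any matching SpecificCombo, or else fills the shared combo's main and sub fire slots.
; AddNewPistolCombo spawns extra combos into PistolCombos, which the lookup never reads.
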(event `self.ReceiveBeginPlay`
  (`self.CreateProceduralBlueprints`))

(fn `AddNewPistolCombo`
  (params (ComboToAdd :type "/Game/Blueprints/Weapons/Combos/BP_WeaponCombo_Base Class Reference"))
  (bind _returnvalue (`|SpawnActorFromClass` ComboToAdd (`KismetMathLibrary.MakeTransform` (0.0 2500.0 0.0)) "Undefined" "MultiplyWithRoot" null null))
  (`KismetArrayLibrary.Array_Add` (`self.PistolCombos`) _returnvalue))

(fn `CheckForProCombo`
  (params (MainWeaponNum :type Integer) (SubWeaponNum :type Integer) (WeaponStats :type "WeaponStatsComponent Object Reference"))
  (returns (WasComboFound :type Boolean) (Combo :type "/Game/Blueprints/Weapons/Combos/BP_ProceduralWeaponCombo_Base Object Reference"))
  (bind _returncombo (`self.returnCombo`))
  (bind _returncombo_2 (`self.returnCombo`))
  (set `/Game/Blueprints/Weapons/Combos/BP_ProceduralWeaponCombo_Base.WeaponStats` WeaponStats (`self.ProceduralPistol`))
  (set `/Game/Blueprints/Weapons/Combos/BP_ProceduralWeaponCombo_Base.WeaponStats` WeaponStats (`self.ProceduralShotgun`))
  (set `/Game/Blueprints/Weapons/Combos/BP_ProceduralWeaponCombo_Base.WeaponStats` WeaponStats (`self.ProceduralCharge`))
  (for _array_element (`self.SpecificCombo`)
    (if (and (== (`WeaponCombo.mainWeaponNum` _array_element) MainWeaponNum) (== (`WeaponCombo.subWeaponNum` _array_element) SubWeaponNum))
      (return true _array_element)))
  (switch `int` MainWeaponNum
    (:`1`
      (set `/Game/Blueprints/Weapons/Combos/BP_ProceduralWeaponCombo_Base.MainEComboFire` (`self.ProceduralPistol`) _returncombo))
    (:`2`
      (set `/Game/Blueprints/Weapons/Combos/BP_ProceduralWeaponCombo_Base.MainEComboFire` (`self.ProceduralShotgun`) _returncombo))
    (:`3`
      (set `/Game/Blueprints/Weapons/Combos/BP_ProceduralWeaponCombo_Base.MainEComboFire` (`self.ProceduralCharge`) _returncombo)))
  (switch `int` SubWeaponNum
    (:`1`
      (set `/Game/Blueprints/Weapons/Combos/BP_ProceduralWeaponCombo_Base.SubEComboFire` (`self.ProceduralPistol`) _returncombo_2))
    (:`2`
      (set `/Game/Blueprints/Weapons/Combos/BP_ProceduralWeaponCombo_Base.SubEComboFire` (`self.ProceduralShotgun`) _returncombo_2))
    (:`3`
      (set `/Game/Blueprints/Weapons/Combos/BP_ProceduralWeaponCombo_Base.SubEComboFire` (`self.ProceduralCharge`) _returncombo_2)))
  (return true (`self.returnCombo`)))

(fn `CreateProceduralBlueprints`
  (bind _returnvalue (`|SpawnActorFromClass` "/Game/Blueprints/Weapons/Combos/BP_ProceduralPistol.BP_ProceduralPistol_C" (`KismetMathLibrary.MakeTransform` (0.0 2500.0 0.0)) "Undefined" "MultiplyWithRoot" null null))
  (set `self.ProceduralPistol` _returnvalue)
  (bind _returnvalue_2 (`|SpawnActorFromClass` "/Game/Blueprints/Weapons/Combos/BP_ProceduralCharge.BP_ProceduralCharge_C" (`KismetMathLibrary.MakeTransform` (0.0 2500.0 0.0)) "Undefined" "MultiplyWithRoot" null null))
  (set `self.ProceduralCharge` _returnvalue_2)
  (bind _returnvalue_3 (`|SpawnActorFromClass` "/Game/Blueprints/Weapons/Combos/BP_ProceduralShotgun.BP_ProceduralShotgun_C" (`KismetMathLibrary.MakeTransform` (0.0 2500.0 0.0)) "Undefined" "MultiplyWithRoot" null null))
  (set `self.ProceduralShotgun` _returnvalue_3)
  (bind _returnvalue_4 (`|SpawnActorFromClass` "/Game/Blueprints/Weapons/Combos/BP_ProceduralWeaponCombo_Base.BP_ProceduralWeaponCombo_Base_C" (`KismetMathLibrary.MakeTransform` (0.0 2500.0 0.0)) "Undefined" "MultiplyWithRoot" null null))
  (set `self.returnCombo` _returnvalue_4))