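; BP_PSCombo is a weapon combo that merges pistol and shotgun behavior, firing bursts of bullet spreads.
; FireCombo loops to spawn BP_Bullet_Base actors evenly across the spread angle by offsetting pitch, setting each projectile's velocity along its direction.
; An iteration counter tracks the burst, returning FireAgain and a delay to the caller until the pistol burst amount is reached.
; A delay modifier other than one rescales that delay by modifier over iteration.
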(fn `FireCombo`
  (params (ShootingTransform :type "Transform Structure") (BulletVelocity :type "Float (double-precision)"))
  (returns (FireAgain :type Boolean) (Delay :type "Float (double-precision)"))
  (bind _roll (.roll ShootingTransform_Rotation))
  (bind _yaw (.yaw ShootingTransform_Rotation))
  (bind _pistolvariables (`self.PistolVariables`))
  (bind _shotgunvariables (`self.ShotgunVariables`))
  (bind _returnvalue (+ (`self.Iterations`) 1))
  (bind _returnvalue_2 (+ (- (.pitch ShootingTransform_Rotation) (* (`ShotgunVariables.spreadAngle` (`self.ShotgunVariables`)) 0.5)) (* (`self.DegreePerBullet`) (`self.ShotgunIteration`))))
  (set `self.DegreePerBullet` (/ (`ShotgunVariables.spreadAngle` _shotgunvariables) (`ShotgunVariables.bulletsPerSpread` _shotgunvariables)))
  (bind _returnvalue_3 (`|SpawnActorFromClass` "/Game/Blueprints/Bullets/BP_Bullet_Base.BP_Bullet_Base_C" (`KismetMathLibrary.MakeTransform` ShootingTransform_Location (`KismetMathLibrary.MakeRotator` _roll _returnvalue_2 _yaw) ShootingTransform_Scale) "Undefined" "MultiplyWithRoot" (`self.GetParentActor`) null :!label _label))
  (set `MovementComponent.Velocity` (* (`KismetMathLibrary.Conv_RotatorToVector` (`KismetMathLibrary.MakeRotator` _roll _returnvalue_2 _yaw)) BulletVelocity) (`/Game/Blueprints/Bullets/BP_Bullet_Base.ProjectileMovement` _returnvalue_3))
  (bind _output_get (set `self.ShotgunIteration` (+ (`self.ShotgunIteration`) 1)))
  (if (<= _output_get (`ShotgunVariables.bulletsPerSpread` (`self.ShotgunVariables`)))
    (goto _label)
    (else
      (set `self.Iterations` _returnvalue)
      (set `self.ShotgunIteration` 0)
      (if (<= _returnvalue (`PistolVariables.burstAmount` _pistolvariables))
        (if (== (`PistolVariables.burstDelayMod` (`self.PistolVariables`)) 1)
          (return true (`PistolVariables.burstDelay` (`self.PistolVariables`)))
          (else
            (return true (* (`PistolVariables.burstDelay` _pistolvariables) (/ (`PistolVariables.burstDelayMod` _pistolvariables) (`self.Iterations`))))))
        (else
          (set `self.Iterations` 0)
          (return false 0.0))))))

(fn `UserConstructionScript`
  (`parent.UserConstructionScript`))