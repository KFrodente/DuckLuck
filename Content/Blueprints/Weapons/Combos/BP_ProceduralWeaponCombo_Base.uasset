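; Base Blueprint for procedural weapon combos, defining the shared firing interface that child combos are expected to override.
; MainProCombo, FireCombo and DoFireSequence are stubs that print a debug message and return no refire with zero delay.
; SubProCombo forwards the shooting transform and bullet velocity to MainEComboFire's MainProCombo and passes back its refire and delay results, leaving DamageAddition unused.
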(fn `DoFireSequence`
  (params (SubProCombo :type "/Game/Blueprints/Weapons/Combos/BP_ProceduralWeaponCombo_Base Object Reference") (ShootingTransform :type "Transform Structure") (BulletVelocity :type "Float (double-precision)") (Triggered :type Boolean))
  (returns (FireAgain :type Boolean) (Delay :type "Float (double-precision)"))
  (`KismetSystemLibrary.PrintString` "DoFireSequence from Base class")
  (return false 0.0))

(fn `FireCombo`
  (params (ShootingTransform :type "Transform Structure") (BulletVelocity :type "Float (double-precision)") (SubProCombo :type "/Game/Blueprints/Weapons/Combos/BP_ProceduralWeaponCombo_Base Object Reference"))
  (returns (FireAgain :type Boolean) (Delay :type "Float (double-precision)"))
  (`KismetSystemLibrary.PrintString` "called \"FIRE COMBO\" From parent class")
  (return false 0.0))

(fn `MainProCombo`
  (params (ShootingTransform :type "Transform Structure") (BulletVelocity :type "Float (double-precision)") (SubProCombo :type "/Game/Blueprints/Weapons/Combos/BP_ProceduralWeaponCombo_Base Object Reference"))
  (returns (FireAgain :type Boolean) (Delay :type "Float (double-precision)"))
  (`KismetSystemLibrary.PrintString` "Fired MainECombo from Base class")
  (return false 0.0))

(fn `SubProCombo`
  (params (ShootingTransform :type "Transform Structure") (BulletVelocity :type "Float (double-precision)") (DamageAddition :type "Float (double-precision)"))
  (returns (FireAgain :type Boolean) (Delay :type "Float (double-precision)"))
  (bind (_fireagain _delay) (`self.MainProCombo` (`self.MainEComboFire`) ShootingTransform BulletVelocity null))
  (return _fireagain _delay))

(fn `UserConstructionScript`)