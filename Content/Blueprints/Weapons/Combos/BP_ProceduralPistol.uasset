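; Procedural pistol combo Blueprint that fires bullets in bursts, as either the main or sub part of a weapon combo.
; FireCombo calls MainProCombo, which triggers the passed sub-combo, then spawns a bullet along the shooting transform's forward vector at the given velocity.
; An iteration counter drives the burst, returning FireAgain and a delay that a modifier can scale per shot, then resets.
; Its own SubProCombo only defers to the parent class.
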(fn `FireCombo`
  (params (ShootingTransform :type "Transform Structure") (BulletVelocity :type "Float (double-precision)") (SubProCombo :type "/Game/Blueprints/Weapons/Combos/BP_ProceduralWeaponCombo_Base Object Reference"))
  (returns (FireAgain :type Boolean) (Delay :type "Float (double-precision)"))
  (bind (_fireagain _delay) (`self.MainProCombo` ShootingTransform BulletVelocity SubProCombo))
  (return _fireagain _delay))

(fn `MainProCombo`
  (params (ShootingTransform :type "Transform Structure") (BulletVelocity :type "Float (double-precision)") (SubProCombo :type "/Game/Blueprints/Weapons/Combos/BP_ProceduralWeaponCombo_Base Object Reference"))
  (returns (FireAgain :type Boolean) (Delay :type "Float (double-precision)"))
  (bind _pistolvariables (`self.PistolVariables`))
  (bind _returnvalue (+ (`self.Iterations`) 1))
  (`self.SubProCombo` SubProCombo (`KismetMathLibrary.MakeTransform` ShootingTransform_Location ShootingTransform_Rotation ShootingTransform_Scale) BulletVelocity)
  (bind _returnvalue_2 (`|SpawnActorFromClass` "/Game/Blueprints/Bullets/BP_Bullet_Base.BP_Bullet_Base_C" (`KismetMathLibrary.MakeTransform` ShootingTransform_Location ShootingTransform_Rotation ShootingTransform_Scale) "Undefined" "MultiplyWithRoot" (`self.GetParentActor`) null))
  (set `MovementComponent.Velocity` (* (`KismetMathLibrary.Conv_RotatorToVector` ShootingTransform_Rotation) BulletVelocity) (`/Game/Blueprints/Bullets/BP_Bullet_Base.ProjectileMovement` _returnvalue_2))
  (set `self.Iterations` _returnvalue)
  (if (<= _returnvalue (`PistolVariables.burstAmount` _pistolvariables))
    (if (== (`PistolVariables.burstDelayMod` (`self.PistolVariables`)) 1)
      (return true (`PistolVariables.burstDelay` (`self.PistolVariables`)))
      (else
        (return true (* (`PistolVariables.burstDelay` _pistolvariables) (/ (`PistolVariables.burstDelayMod` _pistolvariables) (`self.Iterations`))))))
    (else
      (set `self.Iterations` 0)
      (return false 0.0))))

(fn `SubProCombo`
  (params (ShootingTransform :type "Transform Structure") (BulletVelocity :type "Float (double-precision)"))
  (returns (FireAgain :type Boolean) (Delay :type "Float (double-precision)"))
  (bind (_fireagain _delay) (`parent.SubProCombo` ShootingTransform BulletVelocity))
  (return _fireagain _delay))

(fn `UserConstructionScript`
  (`parent.UserConstructionScript`))