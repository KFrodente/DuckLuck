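; BP_ProceduralShotgun is the shotgun piece of a procedural weapon combo system, defining its behavior as main or sub combo.
; MainProCombo defers entirely to the parent implementation.
; SubProCombo loops through BulletManager to spawn a full spread at once, stepping pitch evenly across the WeaponStats spread angle with a fixed offset and negated bullet velocity.
; It then resets its bullet counter and requests no refire; DamageAddition goes unused.
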(fn `MainProCombo`
  (params (ShootingTransform :type "Transform Structure") (BulletVelocity :type "Float (double-precision)") (SubProCombo :type "/Game/Blueprints/Weapons/Combos/BP_ProceduralWeaponCombo_Base Object Reference"))
  (returns (FireAgain :type Boolean) (Delay :type "Float (double-precision)"))
  (bind (_fireagain _delay) (`parent.MainProCombo` ShootingTransform BulletVelocity null))
  (return _fireagain _delay))

(fn `SubProCombo`
  (params (ShootingTransform :type "Transform Structure") (BulletVelocity :type "Float (double-precision)") (DamageAddition :type "Float (double-precision)"))
  (returns (FireAgain :type Boolean) (Delay :type "Float (double-precision)"))
  (bind _shotgunvariables (`WeaponStatsComponent.shotgunVariables` (`self.WeaponStats`)))
  (set `self.DegreePerBullet` (/ (`ShotgunVariables.subSpreadAngle` _shotgunvariables) (`ShotgunVariables.subBulletsPerSpread` _shotgunvariables)))
  (`/Game/Blueprints/Bullets/BP_BulletManager.SpawnBullet` (`self.BulletManager`) (`KismetMathLibrary.MakeTransform` ShootingTransform_Location (`KismetMathLibrary.MakeRotator` (.roll (`KismetMathLibrary.MakeRotator` (.roll (.rotation ShootingTransform)) (.pitch (.rotation ShootingTransform)) (.yaw (.rotation ShootingTransform)))) (+ (- (.pitch (`KismetMathLibrary.MakeRotator` (.roll (.rotation ShootingTransform)) (.pitch (.rotation ShootingTransform)) (.yaw (.rotation ShootingTransform)))) (* (`ShotgunVariables.subSpreadAngle` (`WeaponStatsComponent.shotgunVariables` (`self.WeaponStats`))) 0.5)) (* (`self.DegreePerBullet`) (`self.BulletsFired`)) 10.0) (.yaw (`KismetMathLibrary.MakeRotator` (.roll (.rotation ShootingTransform)) (.pitch (.rotation ShootingTransform)) (.yaw (.rotation ShootingTransform))))) ShootingTransform_Scale) (* BulletVelocity -1.0) 0.0 0 0 0.0 0.0 0.0 0.0 0.0 0 false 0 null null null 0.0 0.0 0.0 0.0 0.0 0.0 0.0 true :!label _label)
  (set `self.BulletsFired` (+ (`self.BulletsFired`) 1))
  (if (>= (`self.BulletsFired`) (`ShotgunVariables.subBulletsPerSpread` (`WeaponStatsComponent.shotgunVariables` (`self.WeaponStats`))))
    (set `self.BulletsFired` 0)
    (return false 0.0)
    (else
      (goto _label))))

(fn `UserConstructionScript`
  (`parent.UserConstructionScript`))