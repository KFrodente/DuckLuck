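; Procedural weapon combo that adds a charge-and-release fire mode, charging while the trigger is held and firing on release.
; Tick raises the charge level through timed steps whose threshold is divided by the current level, playing a per-level sound and printing the timer for debugging.
; On release, DoFireSequence calls MainProCombo, which passes level-scaled projectile size, velocity and bonus damage to the nested SubProCombo and relays its refire request.
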(event `self.ReceiveTick`
  (params (DeltaSeconds :type "Float (single-precision)"))
  (`KismetSystemLibrary.PrintString` (`KismetStringLibrary.Conv_DoubleToString` (`self.ChargeTime`)) true true (struct :`G` 0.66 :`B` 1.0 :`A` 1.0) 0.1)
  (if (`self.Charging`)
    (if (<= (`self.ChargeLevel`) (`ChargeVariables.maxCharges` (`self.ChargeVariables`)))
      (bind _output_get (set `self.ChargeTime` (+ (`self.ChargeTime`) DeltaSeconds)))
      (if (>= _output_get (/ (`ChargeVariables.chargeTime` (`self.ChargeVariables`)) (* (`ChargeVariables.chargeTimeMod` (`self.ChargeVariables`)) (`self.ChargeLevel`))))
        (bind _result (`/Engine/EditorBlueprintResources/StandardMacros.IncrementInt` (`self.ChargeLevel`))
          (:`  `
            (`GameplayStatics.PlaySound2D` (`|GetArrayItem` (`self.SoundList`) _result) 1.0 1.0 0.0 null null)
            (set `self.ChargeTime` 0.0)))))
    (else
      (set `self.ChargeTime` 0.0)
      (set `self.ChargeLevel` 0))))

(fn `DoFireSequence`
  (params (SubProCombo :type "/Game/Blueprints/Weapons/Combos/BP_ProceduralWeaponCombo_Base Object Reference") (ShootingTransform :type "Transform Structure") (BulletVelocity :type "Float (double-precision)") (Triggered :type Boolean))
  (returns (FireAgain :type Boolean) (Delay :type "Float (double-precision)"))
  (if Triggered
    (set `self.Charging` true)
    (else
      (bind (_fireagain _delay) (`self.MainProCombo` ShootingTransform (* BulletVelocity (* (`ChargeVariables.velocityModPerCharge` (`self.ChargeVariables`)) (`self.ChargeLevel`))) SubProCombo))
      (set `self.Charging` false)))
  (return _fireagain _delay))

(fn `FireCombo`
  (params (ShootingTransform :type "Transform Structure") (BulletVelocity :type "Float (double-precision)") (SubProCombo :type "/Game/Blueprints/Weapons/Combos/BP_ProceduralWeaponCombo_Base Object Reference"))
  (returns (FireAgain :type Boolean) (Delay :type "Float (double-precision)"))
  (`self.MainProCombo` (struct))
  (return false 0.0))

(fn `MainProCombo`
  (params (ShootingTransform :type "Transform Structure") (BulletVelocity :type "Float (double-precision)") (SubProCombo :type "/Game/Blueprints/Weapons/Combos/BP_ProceduralWeaponCombo_Base Object Reference"))
  (returns (FireAgain :type Boolean) (Delay :type "Float (double-precision)"))
  (bind (_fireagain _delay) (`self.SubProCombo` SubProCombo (`KismetMathLibrary.MakeTransform` ShootingTransform_Location ShootingTransform_Rotation (* ShootingTransform_Scale (* (`self.ChargeLevel`) 0.6))) BulletVelocity (* (`ChargeVariables.bulletDamagePerCharge` (`self.ChargeVariables`)) (`self.ChargeLevel`))))
  (if _fireagain
    (return true _delay)
    (else
      (set `self.ChargeLevel` 1)
      (set `self.Firing` false)
      (return false 0.0))))

(fn `UserConstructionScript`
  (`parent.UserConstructionScript`))