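; BP_Shotgun is a weapon Blueprint whose FireWeapon spawns a spread of BP_Bullet_Base projectiles in one call.
; A wired-back loop steps each bullet's pitch by an even share of the spread angle, starting half the spread below the shooting transform.
; Each bullet gets a lifespan and a velocity rescaled to the given speed.
; The counter then resets and the function returns no refire and zero delay.
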(fn `FireWeapon`
  (params (ShootingTransform :type "Transform Structure") (BulletVelocity :type "Float (double-precision)"))
  (returns (FireAgain :type Boolean) (Delay :type "Float (double-precision)"))
  (bind _shotgunvariables (`self.ShotgunVariables`))
  (set `self.DegreePerBullet` (/ (`ShotgunVariables.spreadAngle` _shotgunvariables) (`ShotgunVariables.bulletsPerSpread` _shotgunvariables)))
  (bind _returnvalue (`|SpawnActorFromClass` "/Game/Blueprints/Bullets/BP_Bullet_Base.BP_Bullet_Base_C" (`KismetMathLibrary.MakeTransform` ShootingTransform_Location (`KismetMathLibrary.MakeRotator` (.roll ShootingTransform_Rotation) (+ (- (.pitch ShootingTransform_Rotation) (* (`ShotgunVariables.spreadAngle` (`self.ShotgunVariables`)) 0.5)) (* (`self.DegreePerBullet`) (`self.BulletsFired`))) (.yaw ShootingTransform_Rotation)) ShootingTransform_Scale) "Undefined" "MultiplyWithRoot" (`self.GetParentActor`) null :!label _label))
  (`self.SetLifeSpan` _returnvalue (`ShotgunVariables.bulletLifespan` (`self.ShotgunVariables`)))
  (bind _projectilemovement (`/Game/Blueprints/Bullets/BP_Bullet_Base.ProjectileMovement` _returnvalue))
  (set `MovementComponent.Velocity` (* (`KismetMathLibrary.Normal` (`MovementComponent.Velocity` _projectilemovement)) BulletVelocity) _projectilemovement)
  (set `self.BulletsFired` (+ (`self.BulletsFired`) 1))
  (if (>= (`self.BulletsFired`) (`ShotgunVariables.bulletsPerSpread` (`self.ShotgunVariables`)))
    (set `self.BulletsFired` 0)
    (return false 0.0)
    (else
      (goto _label))))

(fn `UserConstructionScript`
  (`parent.UserConstructionScript`))