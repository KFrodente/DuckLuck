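; Pistol weapon Blueprint that fires bursts of bullets through BulletManager.
; When triggered, DoFireSequence calls FireWeapon, which spawns one bullet and counts the shot against the burst amount in WeaponStats.
; It returns a loop flag and delay rather than waiting itself, leaving timing to the caller.
; A burst delay modifier other than 1 scales each gap by the modifier divided by the shot count.
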(fn `DoFireSequence`
  (params (BulletTransform :type "Transform Structure") (Triggered :type Boolean) (BulletVelocity :type "Float (double-precision)"))
  (returns (NeedsToLoop :type Boolean) (NeededDelay :type "Float (double-precision)"))
  (if Triggered
    (bind (_fireagain _delay) (`self.FireWeapon` BulletTransform BulletVelocity))
    (return _fireagain _delay)))

(fn `FireWeapon`
  (params (ShootingTransform :type "Transform Structure") (BulletVelocity :type "Float (double-precision)"))
  (returns (FireAgain :type Boolean) (Delay :type "Float (double-precision)"))
  (bind _returnvalue (+ (`self.Iterations`) 1))
  (bind _pistolvariables (`WeaponStatsComponent.pistolVariables` (`self.WeaponStats`)))
  (`/Game/Blueprints/Bullets/BP_BulletManager.SpawnBullet` (`self.BulletManager`) ShootingTransform BulletVelocity 0.0 0 0 0.0 0.0 0.0 0.0 0)
  (set `self.Iterations` _returnvalue)
  (if (<= _returnvalue (`PistolVariables.burstAmount` _pistolvariables))
    (if (== (`PistolVariables.burstDelayMod` (`WeaponStatsComponent.pistolVariables` (`self.WeaponStats`))) 1)
      (set `self.Firing` true)
      (return true (`PistolVariables.burstDelay` (`WeaponStatsComponent.pistolVariables` (`self.WeaponStats`))))
      (else
        (set `self.Firing` true)
        (return true (* (`PistolVariables.burstDelay` _pistolvariables) (/ (`PistolVariables.burstDelayMod` _pistolvariables) (`self.Iterations`))))))
    (else
      (set `self.Iterations` 0)
      (set `self.Firing` false)
      (return false 0.0))))

(fn `UserConstructionScript`)