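; Shotgun weapon Blueprint that fires a fan of bullets per trigger.
; DoFireSequence calls FireWeapon when triggered and passes back its repeat flag and delay.
; FireWeapon loops to spawn the whole spread at once through BulletManager, stepping each bullet's pitch across the WeaponStats spread angle with a fixed offset.
; It then resets its counter and reports no repeat or delay.
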(fn `DoFireSequence`
  (params (BulletTransform :type "Transform Structure") (Triggered :type Boolean) (BulletVelocity :type "Float (double-precision)"))
  (returns (NeedsToLoop :type Boolean) (NeededDelay :type "Float (double-precision)"))
  (if Triggered
    (bind (_fireagain _delay) (`self.FireWeapon` BulletTransform BulletVelocity))
    (return _fireagain _delay)))

(fn `FireWeapon`
  (params (ShootingTransform :type "Transform Structure") (BulletVelocity :type "Float (double-precision)"))
  (returns (FireAgain :type Boolean) (Delay :type "Float (double-precision)"))
  (bind _shotgunvariables (`WeaponStatsComponent.shotgunVariables` (`self.WeaponStats`)))
  (set `self.Firing` true)
  (set `self.DegreePerBullet` (/ (`ShotgunVariables.spreadAngle` _shotgunvariables) (`ShotgunVariables.bulletsPerSpread` _shotgunvariables)))
  (`/Game/Blueprints/Bullets/BP_BulletManager.SpawnBullet` (`self.BulletManager`) (`KismetMathLibrary.MakeTransform` ShootingTransform_Location (`KismetMathLibrary.MakeRotator` (.roll ShootingTransform_Rotation) (+ (- (.pitch ShootingTransform_Rotation) (* (`ShotgunVariables.spreadAngle` (`WeaponStatsComponent.shotgunVariables` (`self.WeaponStats`))) 0.5)) (* (`self.DegreePerBullet`) (`self.BulletsFired`)) 3.5) (.yaw ShootingTransform_Rotation)) ShootingTransform_Scale) BulletVelocity 0.0 0 0 0.0 0.0 0.0 0.0 0 false 0 null :!label _label)
  (set `self.BulletsFired` (+ (`self.BulletsFired`) 1))
  (if (>= (`self.BulletsFired`) (`ShotgunVariables.bulletsPerSpread` (`WeaponStatsComponent.shotgunVariables` (`self.WeaponStats`))))
    (set `self.BulletsFired` 0)
    (set `self.Firing` false)
    (return false 0.0)
    (else
      (goto _label))))

(fn `UserConstructionScript`
  (`parent.UserConstructionScript`))