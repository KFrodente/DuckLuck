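; BP_Charge is a charge weapon that builds power while the trigger is held and fires on release.
; Tick raises ChargeLevel up to around MaxCharges, playing a per-level sound, with each step's required time scaled by the current level.
; DoFireSequence toggles charging and scales bullet velocity by level, then FireWeapon spawns a level-scaled bullet through BulletManager.
; Per-charge damage is computed in an unused node.
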(event `self.ReceiveTick`
  (params (DeltaSeconds :type "Float (single-precision)"))
  (bind _chargevariables (`WeaponStatsComponent.chargeVariables` (`self.WeaponStats`)))
  (if (`self.Charging`)
    (if (<= (`self.ChargeLevel`) (`ChargeVariables.maxCharges` (`WeaponStatsComponent.chargeVariables` (`self.WeaponStats`))))
      (bind _output_get (set `self.ChargeTime` (+ (`self.ChargeTime`) DeltaSeconds)))
      (if (>= _output_get (/ (`ChargeVariables.chargeTime` _chargevariables) (* (`ChargeVariables.chargeTimeMod` _chargevariables) (`self.ChargeLevel`))))
        (bind _result (`/Engine/EditorBlueprintResources/StandardMacros.IncrementInt` (`self.ChargeLevel`))
          (:`  `
            (`GameplayStatics.PlaySound2D` (`|GetArrayItem` (`self.SoundList`) _result) 1.0 1.0 0.0 null null false)
            (set `self.ChargeTime` 0.0)))))
    (else
      (set `self.ChargeTime` 0.0)
      (set `self.ChargeLevel` 0))))

(fn `DoFireSequence`
  (params (BulletTransform :type "Transform Structure") (Triggered :type Boolean) (BulletVelocity :type "Float (double-precision)"))
  (returns (NeedsToLoop :type Boolean) (NeededDelay :type "Float (double-precision)"))
  (if Triggered
    (set `self.Charging` true)
    (else
      (`self.FireWeapon` BulletTransform (* BulletVelocity (* (`ChargeVariables.velocityModPerCharge` (`WeaponStatsComponent.chargeVariables` (`self.WeaponStats`))) (`self.ChargeLevel`))))
      (set `self.Charging` false)))
  (return false 0.0))

(fn `FireWeapon`
  (params (ShootingTransform :type "Transform Structure") (BulletVelocity :type "Float (double-precision)"))
  (returns (FireAgain :type Boolean) (Delay :type "Float (double-precision)"))
  (set `self.Firing` true)
  (`/Game/Blueprints/Bullets/BP_BulletManager.SpawnBullet` (`self.BulletManager`) (`KismetMathLibrary.MakeTransform` ShootingTransform_Location ShootingTransform_Rotation (* ShootingTransform_Scale (* (`self.ChargeLevel`) 0.6))) BulletVelocity 0.0 0 0 0.0 0.0 0.0 0.0 0)
  (set `self.Firing` false)
  (return false 0.0))

(fn `UserConstructionScript`
  (`parent.UserConstructionScript`))