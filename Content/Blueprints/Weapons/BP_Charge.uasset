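; BP_Charge is a charge-up weapon that builds levels while the trigger is held and fires one projectile on release.
; Tick advances ChargeLevel up to the configured cap, with each step's time threshold divided by the current level, and prints the charge timer.
; DoFireSequence starts charging or calls FireWeapon, which spawns a BP_Bullet_Base with size, damage and velocity scaled by ChargeLevel.
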(event `self.ReceiveTick`
  (params (DeltaSeconds :type "Float (single-precision)"))
  (bind _chargevariables (`self.ChargeVariables`))
  (`KismetSystemLibrary.PrintString` (`KismetStringLibrary.Conv_DoubleToString` (`self.ChargeTime`)) true true (struct :`G` 0.66 :`B` 1.0 :`A` 1.0) 0.1)
  (if (`self.Charging`)
    (if (<= (`self.ChargeLevel`) (`ChargeVariables.maxCharges` (`self.ChargeVariables`)))
      (bind _output_get (set `self.ChargeTime` (+ (`self.ChargeTime`) DeltaSeconds)))
      (if (>= _output_get (/ (`ChargeVariables.chargeTime` _chargevariables) (* (`ChargeVariables.chargeTimeMod` _chargevariables) (`self.ChargeLevel`))))
        ;[1 0 0] This is where it will play the sound of the next charge as well
        (set `self.ChargeLevel` (+ (`self.ChargeLevel`) 1))
        (set `self.ChargeTime` 0.0)))
    (else
      (set `self.ChargeTime` 0.0)
      (set `self.ChargeLevel` 1))))

(fn `DoFireSequence`
  (params (BulletTransform :type "Transform Structure") (Triggered :type Boolean) (BulletVelocity :type "Float (double-precision)"))
  (returns (NeedsToLoop :type Boolean) (NeededDelay :type "Float (double-precision)"))
  (if Triggered
    (set `self.Charging` true)
    (else
      (`self.FireWeapon` BulletTransform (* BulletVelocity (* (`ChargeVariables.velocityModPerCharge` (`self.ChargeVariables`)) (`self.ChargeLevel`))))
      (set `self.Charging` false)))
  (return false 0.0))

(fn `FireWeapon`
  (params (ShootingTransform :type "Transform Structure") (BulletVelocity :type "Float (double-precision)"))
  (returns (FireAgain :type Boolean) (Delay :type "Float (double-precision)"))
  (set `self.Firing` true)
  (bind _returnvalue (`|SpawnActorFromClass` "/Game/Blueprints/Bullets/BP_Bullet_Base.BP_Bullet_Base_C" (`KismetMathLibrary.MakeTransform` ShootingTransform_Location ShootingTransform_Rotation (* ShootingTransform_Scale (* (`self.ChargeLevel`) 0.6))) "Undefined" "MultiplyWithRoot" (`self.GetParentActor`) null))
  (set `/Game/Blueprints/Bullets/BP_Bullet_Base.ProjectileDamage` (* (`/Game/Blueprints/Bullets/BP_Bullet_Base.ProjectileDamage` _returnvalue) (* (`ChargeVariables.bulletDamagePerCharge` (`self.ChargeVariables`)) (`self.ChargeLevel`))) _returnvalue)
  (set `MovementComponent.Velocity` (* (`KismetMathLibrary.Conv_RotatorToVector` ShootingTransform_Rotation) BulletVelocity) (`/Game/Blueprints/Bullets/BP_Bullet_Base.ProjectileMovement` _returnvalue))
  (set `self.Firing` false)
  (return false 0.0))

(fn `UserConstructionScript`
  (`parent.UserConstructionScript`))