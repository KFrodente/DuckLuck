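; BP_PlayerWithHat is the side-scrolling player character, with hold-length multi-jump, directional dashing, aimed gun fire and overlap-based interaction.
; Enhanced Input drives movement and aim, while BP_Inventory supplies the gun, fire points and unlocked powers on possession.
; Tick traces for ground to refresh jumps and dash, grants invincibility while dashing and applies water buoyancy.
; Jumping mid-horizontal dash triggers a timeline-eased power dash, and the bubble power replaces buoyancy with reduced gravity.
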(event `self.ReceiveTick`
  (params (DeltaSeconds :type "Float (single-precision)"))
  (bind (_returnvalue_x _returnvalue_y _returnvalue_z) (`KismetMathLibrary.BreakVector` (`self.K2_GetActorLocation`)))
  (bind _charactermovement (`self.CharacterMovement`))
  (bind _ogravityscale (`self.OGravityScale`))
  (bind _charactermovement_2 (`self.CharacterMovement`))
  (bind (_velocity_x _velocity_y _velocity_z) (`KismetMathLibrary.BreakVector` (`MovementComponent.Velocity` _charactermovement_2)))
  (set `self.FireRateTimer` (- (`self.FireRateTimer`) DeltaSeconds))
  (if (`self.IsJumping`)
    (set `self.JumpLength` (- (`self.JumpLength`) DeltaSeconds)))
  (`self.DashInvincibility`)
  (`self.CheckGrounded`)
  (if (`self.InBubble`)
    (if (`self.InWater`)
      (set `CharacterMovementComponent.GravityScale` (* _ogravityscale 0.7) _charactermovement)
      (else
        (set `CharacterMovementComponent.GravityScale` _ogravityscale _charactermovement)))
    (elif (`self.EnteredWater`)
      (if (`self.OnGround`)
        (`self.LaunchCharacter` (0.0 0.0 100.0) false true))
      (if (< _returnvalue_z (+ (`self.WaterHeight`) (`self.WaterOrigin`)))
        (set `MovementComponent.Velocity` (`KismetMathLibrary.MakeVector` _velocity_x 0.0 (+ _velocity_z (* 12000.0 (`GameplayStatics.GetWorldDeltaSeconds`)))) _charactermovement_2)))))

(event `self.ReceiveBeginPlay`
  (bind _asbp_player_controller (cast `/Game/Blueprints/Player/BP_PlayerController` (`self.GetController`) :!label _label))
  (set `CharacterMovementComponent.MaxWalkSpeed` (`self.OWalkSpeed`) (`self.CharacterMovement`))
  (bind _returnvalue (`GameplayStatics.GetActorOfClass` "/Game/Blueprints/Inventory/BP_Inventory.BP_Inventory_C"))
  (bind _output_get (set `self.Inventory` _returnvalue))
  (set `self.HasDashPower` (`/Game/Blueprints/Inventory/BP_Inventory.HasDashUnlocked` _output_get))
  (set `self.HasBubblePower` (`/Game/Blueprints/Inventory/BP_Inventory.HasBubbleUnlocked` _output_get))
  (set `self.MaxPlayerJumps` (`/Game/Blueprints/Inventory/BP_Inventory.TotalJumps` _output_get))
  (`EnhancedInputSubsystemInterface.AddMappingContext` (pcsubsystem `EnhancedInputLocalPlayerSubsystem` _asbp_player_controller) "/Game/Blueprints/Input/Player/IMC_Default.IMC_Default" (`/Game/Blueprints/Inventory/BP_Inventory.ControlPriority` _output_get) (struct)))

(event `WeaponSwapped_Event`)

(event `self.ReceivePossessed`
  (params (NewController :type "Controller Object Reference"))
  (goto _label))

(event `EnhancedInput|/Game/Blueprints/Input/Player/IA_Horizontal_Movement`
  (params (ActionValue :type "Float (double-precision)") (ElapsedSeconds :type "Float (double-precision)") (TriggeredSeconds :type "Float (double-precision)") (InputAction :type "InputAction Object Reference" :default "/Game/Blueprints/Input/Player/IA_Horizontal_Movement.IA_Horizontal_Movement"))
  (bind _sprite (`self.Sprite`))
  (bind _hat (`self.Hat`))
  (:`Triggered`
    (if (`self.PlayerHasInputControl`)
      (`self.AddMovementInput` (`self.GetActorForwardVector`) ActionValue)
      (if (> ActionValue 0.0)
        (`SceneComponent.K2_SetWorldRotation` _sprite (`KismetMathLibrary.MakeRotator` 0.0) false false)
        (`SceneComponent.K2_SetWorldRotation` _hat (`KismetMathLibrary.MakeRotator` 0.0 0.0 180.0) false false)
        (set `self.FacingRight` true)
        (else
          (`SceneComponent.K2_SetWorldRotation` _sprite (`KismetMathLibrary.MakeRotator` 0.0 0.0 180.0) false false)
          (`SceneComponent.K2_SetWorldRotation` _hat (`KismetMathLibrary.MakeRotator` 0.0) false false)
          (set `self.FacingRight` false))))))

(event `EnhancedInput|/Game/Blueprints/Input/Player/IA_Jump`
  (params (ActionValue :type Boolean) (ElapsedSeconds :type "Float (double-precision)") (TriggeredSeconds :type "Float (double-precision)") (InputAction :type "InputAction Object Reference" :default "/Game/Blueprints/Input/Player/IA_Jump.IA_Jump"))
  (bind (_dashdir_x _dashdir_y _dashdir_z) (`KismetMathLibrary.BreakVector` (`self.DashDir`)))
  (bind _charactermovement (`self.CharacterMovement`))
  (bind _x (.x (* (`MovementComponent.Velocity` _charactermovement) (`KismetMathLibrary.MakeVector` (`self.PowerDashMult`) 1.0 1.0))))
  (:`Triggered`
    (if (and (> (`self.JumpLength`) 0.0) (> (`self.JumpsAvailable`) 0)) :!label _label_2
      (set `self.IsJumping` true)
      (`self.LaunchCharacter` (`KismetMathLibrary.MakeVector` 0.0 0.0 (`CharacterMovementComponent.JumpZVelocity` (`self.CharacterMovement`))) false true)
      (if (not (`self.InWater`))
        (set `self.EnteredWater` false))))
  (:`Started`
    (if (`self.Dashing`)
      (if (and (and (!= _dashdir_x 0.0) (== _dashdir_z 0.0)) (`self.Dashing`) (`self.HasDashPower`) (> (`self.JumpsAvailable`) 0))
        (set `self.CanDash` true)
        (set `self.IsJumping` false)
        (`GameplayStatics.PlaySound2D` "/Game/Assets/Audio/Player/PowerDash_Cue.PowerDash_Cue" 1.0 1.0 0.0 null null)
        (set `MovementComponent.Velocity` (`KismetMathLibrary.MakeVector` _x 0.0 (.z (* (`MovementComponent.Velocity` _charactermovement) (`KismetMathLibrary.MakeVector` (`self.PowerDashMult`) 1.0 1.0)))) _charactermovement)
        (bind _output_get (set `CharacterMovementComponent.MaxWalkSpeed` (`KismetMathLibrary.Abs` _x) _charactermovement)) ; output should be sent in as the "A" value in the lerp function
        (bind (_direction _newtrack_0) (`Timeline|Timeline` :!via `PlayFromStart`)
          (:`Update`
            (set `CharacterMovementComponent.MaxWalkSpeed` (`KismetMathLibrary.Lerp` _output_get (`self.OWalkSpeed`) _newtrack_0) _charactermovement))))
      (else
        (goto _label_2))))
  (:`Canceled`
    (`self.StopJumping` :!label _label_3)
    (set `self.JumpsAvailable` (- (`self.JumpsAvailable`) 1))
    (set `self.JumpLength` (`self.MaxJumpLength`))
    (set `self.IsJumping` false))
  (:`Completed`
    (goto _label_3)))

(event `EnhancedInput|/Game/Blueprints/Input/Player/IA_Dash`
  (params (ActionValue :type Boolean) (ElapsedSeconds :type "Float (double-precision)") (TriggeredSeconds :type "Float (double-precision)") (InputAction :type "InputAction Object Reference" :default "/Game/Blueprints/Input/Player/IA_Dash.IA_Dash"))
  (bind _charactermovement (`self.CharacterMovement`))
  (bind (_velocity_x _velocity_y _velocity_z) (`KismetMathLibrary.BreakVector` (`MovementComponent.Velocity` _charactermovement)))
  (:`Triggered`
    (if (and (`self.CanDash`) (`self.HasDashPower`))
      (bind _output_get (set `self.DashDir` (`self.AimDir`)))
      (bind _x (.x _output_get))
      (bind _z (.z _output_get))
      (if (not (and (== _x 0.0) (== _z 0.0)))
        (if (and (!= _x 0.0) (!= _z 0.0))
          (set `self.NVerticalDashDiminish` (* (`self.OVerticalDashDiminish`) 0.8))
          (set `self.NHorizontalDashDiminish` (* (`self.OHorizontalDashDiminish`) 0.8)))
        (if (and (!= (.x _output_get) 0.0) (== (.z _output_get) 0.0))
          (if (not (`self.Dashing`))
            (set `self.Dashing` true)
            (set `self.CanDash` false)
            (set `CharacterMovementComponent.GravityScale` 0.0 (`self.CharacterMovement`))
            (`self.LaunchCharacter` (`KismetMathLibrary.MakeVector` (* (.x (* (`KismetMathLibrary.Normal` (`self.DashDir`)) (`self.DashSpeedMultiplier`))) (`self.DashHorizontalSpeedMult`))) true true)
            (`GameplayStatics.PlaySound2D` "/Game/Assets/Audio/Player/Dash_Cue.Dash_Cue" 1.0 1.0 0.0 null null false :!label _label_4)
            (`KismetSystemLibrary.Delay` (`self.DashLength`))
            (set `self.Dashing` false)
            (if (`self.InWater`)
              (`self.SetWaterVars` true (`self.WaterHeight`) (`self.WaterOrigin`))
              (else
                (set `CharacterMovementComponent.GravityScale` (`self.OGravityScale`) _charactermovement)
                (bind _output_get_2 (set `MovementComponent.Velocity` (`KismetMathLibrary.MakeVector` (* _velocity_x (`self.NHorizontalDashDiminish`)) 0.0 (* _velocity_z (`self.NVerticalDashDiminish`))) _charactermovement))
                (set `self.EnteredWater` false)
                (`self.LaunchCharacter` _output_get_2 true true)))
            (set `self.NHorizontalDashDiminish` (`self.OHorizontalDashDiminish`))
            (set `self.NVerticalDashDiminish` (`self.OVerticalDashDiminish`)))
          (elif (not (`self.Dashing`))
            (set `self.Dashing` true)
            (set `self.CanDash` false)
            (set `CharacterMovementComponent.GravityScale` 0.0 (`self.CharacterMovement`))
            (`self.LaunchCharacter` (`KismetMathLibrary.MakeVector` (* (.x (* (`KismetMathLibrary.Normal` (`self.DashDir`)) (`self.DashSpeedMultiplier`))) (`self.DashHorizontalSpeedMult`)) (.y (* (`KismetMathLibrary.Normal` (`self.DashDir`)) (`self.DashSpeedMultiplier`))) (.z (* (`KismetMathLibrary.Normal` (`self.DashDir`)) (`self.DashSpeedMultiplier`)))) true true)
            (goto _label_4)))))))

(event `EnhancedInput|/Game/Blueprints/Input/Player/IA_Interact`
  (params (ActionValue :type Boolean) (ElapsedSeconds :type "Float (double-precision)") (TriggeredSeconds :type "Float (double-precision)") (InputAction :type "InputAction Object Reference" :default "/Game/Blueprints/Input/Player/IA_Interact.IA_Interact"))
  (:`Triggered`
    (for _array_element (`self.GetOverlappingActors` "/Script/Engine.Actor")
      (if (`KismetSystemLibrary.DoesImplementInterface` _array_element "/Game/Blueprints/Interfaces_Enums/Interactable.Interactable_C")
        (message `/Game/Blueprints/Interfaces_Enums/Interactable.interact` _array_element self null (`self.Inventory`))
        (break)))))

(event `EnhancedInput|/Game/Blueprints/Input/Player/IA_Vertical_Movement`
  (params (ActionValue :type "Float (double-precision)") (ElapsedSeconds :type "Float (double-precision)") (TriggeredSeconds :type "Float (double-precision)") (InputAction :type "InputAction Object Reference" :default "/Game/Blueprints/Input/Player/IA_Vertical_Movement.IA_Vertical_Movement"))
  (bind (_returnvalue_roll _returnvalue_pitch _returnvalue_yaw) (`KismetMathLibrary.BreakRotator` (`SceneComponent.K2_GetComponentRotation` (`self.Sprite`))))
  (bind _mainweapon (`/Game/Blueprints/Inventory/BP_Inventory.MainWeapon` (`self.Inventory`)))
  (:`Triggered`
    (`SceneComponent.K2_SetWorldRotation` (`self.GunSection`) (`KismetMathLibrary.MakeRotator` 0.0 (* (`KismetMathLibrary.SignOfFloat` ActionValue) 90.0) _returnvalue_yaw) false false :!label _label_5)
    (`/Engine/EditorBlueprintResources/StandardMacros.IsValid` _mainweapon :!label _label_6
      (:`Is Valid`
        (if (== ActionValue 0.0)
          (if (`self.FacingRight`)
            (set `self.FirePoint` (`Weapon.m_RFirePoint` _mainweapon))
            (else
              (set `self.FirePoint` (`Weapon.m_LFirePoint` _mainweapon))))
          (elif (> ActionValue 0.0)
            (set `self.FirePoint` (`Weapon.m_UFirePoint` _mainweapon))
            (else
              (set `self.FirePoint` (`Weapon.m_DFirePoint` _mainweapon))))))))
  (:`Completed`
    (goto _label_5)))

(event `EnhancedInput|/Game/Blueprints/Input/Player/IA_Horizontal_Movement`
  (params (ActionValue :type "Float (double-precision)") (ElapsedSeconds :type "Float (double-precision)") (TriggeredSeconds :type "Float (double-precision)") (InputAction :type "InputAction Object Reference" :default "/Game/Blueprints/Input/Player/IA_Horizontal_Movement.IA_Horizontal_Movement"))
  (:`Triggered`
    (goto _label_6)))

(event `EnhancedInput|/Game/Blueprints/Input/Player/IA_FireGun`
  (params (ActionValue :type Boolean) (ElapsedSeconds :type "Float (double-precision)") (TriggeredSeconds :type "Float (double-precision)") (InputAction :type "InputAction Object Reference" :default "/Game/Blueprints/Input/Player/IA_FireGun.IA_FireGun"))
  (:`Triggered`
    (bind (_fireagain _delay) (`/Game/Blueprints/Weapons/Gun/BP_Gun.FireGun` (`/Game/Blueprints/Inventory/BP_Inventory.Gun` (`self.Inventory`)) (`KismetMathLibrary.MakeTransform` (+ (`self.K2_GetActorLocation`) (`self.FirePoint`)) (`SceneComponent.K2_GetComponentRotation` (`self.GunSection`))) true :!label _label_7))
    (if _fireagain
      (`KismetSystemLibrary.Delay` _delay)
      (goto _label_7)))
  (:`Canceled`
    (bind (_fireagain_2 _delay_2) (`/Game/Blueprints/Weapons/Gun/BP_Gun.FireGun` (`/Game/Blueprints/Inventory/BP_Inventory.Gun` (`self.Inventory`)) (`KismetMathLibrary.MakeTransform` (+ (`self.K2_GetActorLocation`) (`self.FirePoint`)) (`SceneComponent.K2_GetComponentRotation` (`self.GunSection`))) false :!label _label_8))
    (if _fireagain_2
      (`KismetSystemLibrary.Delay` _delay_2)
      (goto _label_8)))
  (:`Completed`
    (goto _label_8)))

(event `EnhancedInput|/Game/Blueprints/Input/Player/IA_Vertical_Movement`
  (params (ActionValue :type "Float (double-precision)") (ElapsedSeconds :type "Float (double-precision)") (TriggeredSeconds :type "Float (double-precision)") (InputAction :type "InputAction Object Reference" :default "/Game/Blueprints/Input/Player/IA_Vertical_Movement.IA_Vertical_Movement"))
  (bind _returnvalue (< ActionValue 0.0))
  (bind (_velocity_x _velocity_y _velocity_z) (`KismetMathLibrary.BreakVector` (`MovementComponent.Velocity` (`self.CharacterMovement`))))
  (:`Triggered`
    (if (`self.HasBubblePower`)
      (if (or (and _returnvalue (> TriggeredSeconds (`self.BubbleCreationTime`))) (and _returnvalue (< _velocity_z 0.0)))
        (set `self.InBubble` true)))))

(event `EnhancedInput|/Game/Blueprints/Input/Player/IA_Horizontal_Movement`
  (params (ActionValue :type "Float (double-precision)") (ElapsedSeconds :type "Float (double-precision)") (TriggeredSeconds :type "Float (double-precision)") (InputAction :type "InputAction Object Reference" :default "/Game/Blueprints/Input/Player/IA_Horizontal_Movement.IA_Horizontal_Movement"))
  (:`Triggered`
    (set `self.AimDir` (`KismetMathLibrary.MakeVector` ActionValue 0.0 (stale `EnhancedInput|/Game/Blueprints/Input/Player/IA_Vertical_Movement` ActionValue)) :!label _label_9))
  (:`Completed`
    (goto _label_9)))

(event `EnhancedInput|/Game/Blueprints/Input/Player/IA_Vertical_Movement`
  (params (ActionValue :type "Float (double-precision)") (ElapsedSeconds :type "Float (double-precision)") (TriggeredSeconds :type "Float (double-precision)") (InputAction :type "InputAction Object Reference" :default "/Game/Blueprints/Input/Player/IA_Vertical_Movement.IA_Vertical_Movement"))
  (:`Triggered`
    (goto _label_9))
  (:`Completed`
    (goto _label_9)))

(event `EnhancedInput|/Game/Blueprints/Input/Player/IA_Inventory`
  (params (ActionValue :type Boolean) (ElapsedSeconds :type "Float (double-precision)") (TriggeredSeconds :type "Float (double-precision)") (InputAction :type "InputAction Object Reference" :default "/Game/Blueprints/Input/Player/IA_Inventory.IA_Inventory"))
  (:`Triggered`
    (`/Game/Blueprints/Inventory/BP_Inventory.SpawnAndControlPlayer` (`self.Inventory`) (`self.GetTransform`) self)))

(fn `SetWaterVars`
  (params (InWater :type Boolean) (WaterHeight :type "Float (double-precision)") (WaterOrigin :type "Float (double-precision)") (PlatformingBlock :type Boolean))
  (bind (_returnvalue_x _returnvalue_y _returnvalue_z) (`KismetMathLibrary.BreakVector` (`self.K2_GetActorLocation`)))
  (bind (_returnvalue_x_2 _returnvalue_y_2 _returnvalue_z_2) (`KismetMathLibrary.BreakVector` (`self.K2_GetActorLocation`)))
  (bind _maxwaterexitvelocity (`self.MaxWaterExitVelocity`))
  (bind _charactermovement (`self.CharacterMovement`))
  (bind (_aimdir_x _aimdir_y _aimdir_z) (`KismetMathLibrary.BreakVector` (`self.AimDir`)))
  (bind (_velocity_x _velocity_y _velocity_z) (`KismetMathLibrary.BreakVector` (`MovementComponent.Velocity` _charactermovement)))
  (bind (_velocity_x_2 _velocity_y_2 _velocity_z_2) (`KismetMathLibrary.BreakVector` (`MovementComponent.Velocity` _charactermovement)))
  (bind (_velocity_x_3 _velocity_y_3 _velocity_z_3) (`KismetMathLibrary.BreakVector` (`MovementComponent.Velocity` (`self.CharacterMovement`))))
  (if (and (> WaterOrigin _returnvalue_z_2) (not PlatformingBlock) (`self.HasBubblePower`))
    (set `self.InBubble` true))
  (if InWater
    (set `self.InWater` true)
    (set `self.EnteredWater` true)
    (bind _output_get (set `self.WaterHeight` WaterHeight))
    (bind _output_get_2 (set `self.WaterOrigin` WaterOrigin))
    (if (and (< (`KismetMathLibrary.Abs` _velocity_z_3) 600.0) (not (`self.Dashing`)) (> _returnvalue_z (+ _output_get_2 _output_get -20.0)))
      ;[1 1 1] Stops the player at the top of the water and allows them to jump
      (set `self.IsJumping` false)
      (set `self.CanDash` true)
      (set `MovementComponent.Velocity` (`KismetMathLibrary.MakeVector` _velocity_x_3) _charactermovement)
      (set `CharacterMovementComponent.GravityScale` 0.0 _charactermovement)
      (set `self.WaterImpactsHeight` false)
      (set `self.JumpsAvailable` (`self.MaxPlayerJumps`))
      (set `self.JumpLength` (`self.MaxJumpLength`))
      (set `self.EnteredWater` false)
      (else
        (set `self.WaterImpactsHeight` true)))
    (else
      (set `self.InWater` false)
      (set `self.WaterHeight` 0.0)
      (set `self.WaterOrigin` 0.0)
      (set `self.DistFromTop` 0.0)
      (set `CharacterMovementComponent.GravityScale` (`self.OGravityScale`) _charactermovement)
      (set `self.InBubble` false)
      (if (and (`self.WaterImpactsHeight`) (<= _aimdir_z 0.0))
        (set `MovementComponent.Velocity` (`KismetMathLibrary.MakeVector` _velocity_x_2 0.0 (* _velocity_z_2 0.01)) _charactermovement)
        (else
          (set `self.CanDash` true)
          (set `self.Dashing` false)
          (set `self.JumpsAvailable` (`self.MaxPlayerJumps`))
          (if (> _velocity_z _maxwaterexitvelocity)
            (set `MovementComponent.Velocity` (`KismetMathLibrary.MakeVector` _velocity_x 0.0 _maxwaterexitvelocity) _charactermovement))))
      (set `self.EnteredWater` false))))

(fn `UserConstructionScript`)