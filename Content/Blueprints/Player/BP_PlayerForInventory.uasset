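; BP_PlayerForInventory is the controllable sprite avatar used to move around and select items in the inventory.
; On possession or BeginPlay it finds BP_Inventory and adds IMC_Inventory at that inventory's priority.
; Movement input drives it on the world X/Y plane and flips the sprite by rotation.
; Confirm and cancel send Interactable main or sub messages to overlapped menu items, while exit has the inventory despawn it and return.
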(event `self.ReceiveBeginPlay`
  (bind _asbp_player_controller (cast `/Game/Blueprints/Player/BP_PlayerController` (`self.GetController`) :!label _label))
  (bind _returnvalue (`GameplayStatics.GetActorOfClass` "/Game/Blueprints/Player/BP_Inventory.BP_Inventory_C"))
  (bind _output_get (set `self.Inventory` _returnvalue))
  (`EnhancedInputSubsystemInterface.AddMappingContext` (pcsubsystem `EnhancedInputLocalPlayerSubsystem` _asbp_player_controller) "/Game/Blueprints/Input/Inventory/IMC_Inventory.IMC_Inventory" (`/Game/Blueprints/Player/BP_Inventory.ControlPriority` _output_get) (struct)))

(event `self.ReceivePossessed`
  (params (NewController :type "Controller Object Reference"))
  (goto _label))

(event `EnhancedInput|/Game/Blueprints/Input/Inventory/IA_InvMovement`
  (params (ActionValue :type "Vector2D Structure") (ElapsedSeconds :type "Float (double-precision)") (TriggeredSeconds :type "Float (double-precision)") (InputAction :type "InputAction Object Reference" :default "/Game/Blueprints/Input/Inventory/IA_InvMovement.IA_InvMovement"))
  (bind _returnvalue (* ActionValue_Y 600.0))
  (bind _sprite (`self.Sprite`))
  (:`Triggered`
    (`self.AddMovementInput` (0.0 1.0 0.0) (* ActionValue_X 600.0))
    (`self.AddMovementInput` (1.0 0.0 0.0) _returnvalue)
    (if (or (> _returnvalue 0.0) (and (== _returnvalue 0.0) (`self.FacingRight`)))
      (`SceneComponent.K2_SetWorldRotation` _sprite (`KismetMathLibrary.MakeRotator` -90.0) false false)
      (set `self.FacingRight` true)
      (else
        (`SceneComponent.K2_SetWorldRotation` _sprite (`KismetMathLibrary.MakeRotator` -90.0 -180.0) false false)
        (set `self.FacingRight` false)))))

(event `EnhancedInput|/Game/Blueprints/Input/Inventory/IA_InvExit`
  (params (ActionValue :type Boolean) (ElapsedSeconds :type "Float (double-precision)") (TriggeredSeconds :type "Float (double-precision)") (InputAction :type "InputAction Object Reference" :default "/Game/Blueprints/Input/Inventory/IA_InvExit.IA_InvExit"))
  (:`Triggered`
    (`/Game/Blueprints/Player/BP_Inventory.DespawnPlayerAndReturn` (`self.Inventory`) self)))

(event `EnhancedInput|/Game/Blueprints/Input/Inventory/IA_InvConfirm`
  (params (ActionValue :type Boolean) (ElapsedSeconds :type "Float (double-precision)") (TriggeredSeconds :type "Float (double-precision)") (InputAction :type "InputAction Object Reference" :default "/Game/Blueprints/Input/Inventory/IA_InvConfirm.IA_InvConfirm"))
  (:`Triggered`
    (for _array_element (`self.GetOverlappingActors` "/Game/Blueprints/Inventory/BP_MenuItem_Base.BP_MenuItem_Base_C")
      (if (`KismetSystemLibrary.DoesImplementInterface` _array_element "/Game/Blueprints/Interfaces_Enums/Interactable.Interactable_C")
        (message `/Game/Blueprints/Interfaces_Enums/Interactable.InteractMain` _array_element (`self.Inventory`))))))

(event `EnhancedInput|/Game/Blueprints/Input/Inventory/IA_InvCancel`
  (params (ActionValue :type Boolean) (ElapsedSeconds :type "Float (double-precision)") (TriggeredSeconds :type "Float (double-precision)") (InputAction :type "InputAction Object Reference" :default "/Game/Blueprints/Input/Inventory/IA_InvCancel.IA_InvCancel"))
  (:`Triggered`
    (for _array_element (`self.GetOverlappingActors` "/Game/Blueprints/Inventory/BP_MenuItem_Base.BP_MenuItem_Base_C")
      (if (`KismetSystemLibrary.DoesImplementInterface` _array_element "/Game/Blueprints/Interfaces_Enums/Interactable.Interactable_C")
        (message `/Game/Blueprints/Interfaces_Enums/Interactable.InteractSub` _array_element (`self.Inventory`))))))

(fn `UserConstructionScript`)