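; The player's hat companion in a 2D game, which trails the player and grabs, absorbs or throws nearby enemies and food.
; CheckTarget picks the closest unobstructed overlap as a hover target, and Tick eases the hat toward it or the player.
; A held item follows the hat along the aim direction until LaunchTarget throws it with added player velocity.
; InteractUp grabs and cancels InteractDown's timer; AbsorbTarget converts interactable targets into healing.
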(event `self.ReceiveBeginPlay`
  (`self.Flip` true)
  (bind _returnvalue (`KismetSystemLibrary.K2_SetTimerDelegate` (`|CreateDelegate` :!event `CheckTarget`) 0.1 true))
  (set `self.CheckTargetTimer` _returnvalue))

(event `self.ReceiveTick`
  (params (DeltaSeconds :type "Float (single-precision)"))
  (bind (_returnvalue_x _returnvalue_y _returnvalue_z) (`KismetMathLibrary.BreakVector` (`self.K2_GetActorLocation`)))
  (bind (_returnvalue_x_2 _returnvalue_y_2 _returnvalue_z_2) (`KismetMathLibrary.BreakVector` (`self.K2_GetActorLocation`)))
  (bind (_returnvalue_x_3 _returnvalue_y_3 _returnvalue_z_3) (`KismetMathLibrary.BreakVector` (`self.K2_GetActorLocation`)))
  (bind _playerref (`self.PlayerRef`))
  (bind _playerref_2 (`self.PlayerRef`))
  (bind (_returnvalue_x_4 _returnvalue_y_4 _returnvalue_z_4) (`KismetMathLibrary.BreakVector` (`self.K2_GetActorLocation` (`self.CurrentFollowTarget`))))
  (bind (_returnvalue_x_5 _returnvalue_y_5 _returnvalue_z_5) (`KismetMathLibrary.BreakVector` (`self.K2_GetActorLocation` (`self.PlayerRef`))))
  (bind (_aimdir_x _aimdir_y _aimdir_z) (`KismetMathLibrary.BreakVector` (`/Game/Blueprints/Player/BP_PlayerWithHat.AimDir` _playerref_2)))
  (if (not (`self.HoldingItem`))
    (`/Game/Blueprints/Player/BP_PlayerWithHat.GainHat` _playerref (`/Game/Blueprints/Player/BP_PlayerWithHat.HasHat` _playerref)))
  (if (`self.FollowingPlayer`)
    (`self.K2_SetActorLocation` (`KismetMathLibrary.MakeVector` (`KismetMathLibrary.FInterpTo` _returnvalue_x_2 (+ _returnvalue_x_5 (select `bool` (`self.HoldingItem`) :`true` (select `bool` (and (== _aimdir_x 0.0) (== _aimdir_z 0.0)) :`false` (* _aimdir_x 100.0) :`true` (select `bool` (`/Game/Blueprints/Player/BP_PlayerWithHat.FacingRight` _playerref_2) :`false` -100.0 :`true` 100.0)))) DeltaSeconds 15.0) 1.0 (`KismetMathLibrary.FInterpTo` _returnvalue_z_2 (+ _returnvalue_z_5 (select `bool` (`self.HoldingItem`) :`false` 75.0 :`true` (+ (* _aimdir_z 100.0) 20.0))) DeltaSeconds 15.0)) false true)
    (if (`self.HoldingItem`)
      (`self.K2_SetActorLocation` (`self.CurrentFollowTarget`) (`KismetMathLibrary.MakeVector` _returnvalue_x_3 0.0 _returnvalue_z_3) false false))
    (else
      (`self.K2_SetActorLocation` (`KismetMathLibrary.MakeVector` (`KismetMathLibrary.FInterpTo` _returnvalue_x _returnvalue_x_4 DeltaSeconds 10.0) 0.0 (`KismetMathLibrary.FInterpTo` _returnvalue_z (+ _returnvalue_z_4 75.0) DeltaSeconds 10.0)) false true))))

(event `AbsorbTarget`
  (bind _currentfollowtarget (`self.CurrentFollowTarget`))
  (bind _playerref (`self.PlayerRef`))
  (if (`KismetSystemLibrary.DoesImplementInterface` _currentfollowtarget "/Game/Blueprints/Interfaces_Enums/Interactable.Interactable_C")
    (bind _health (message `/Game/Blueprints/Interfaces_Enums/Interactable.Absorb` _currentfollowtarget (`/Game/Blueprints/Player/BP_PlayerWithHat.Inventory` _playerref)))
    (`/Game/Blueprints/Player/BP_PlayerWithHat.Heal` _playerref _health)
    (set `self.FollowingPlayer` true)
    (`self.K2_DestroyActor` _currentfollowtarget)
    (set `self.CurrentFollowTarget` null)))

(event `CheckTarget`
  (if (not (`self.HoldingItem`))
    (set `self.OnObject` false)
    (set `self.Closest` 700.0)
    (bind (_outactors _returnvalue) (`KismetSystemLibrary.SphereOverlapActors` (`self.K2_GetActorLocation` (`self.PlayerRef`)) 400.0 (`self.HoverCheck`)))
    (if _returnvalue
      (for _array_element _outactors
        (bind (_outhit _returnvalue_2) (`KismetSystemLibrary.LineTraceSingleForObjects` (`self.K2_GetActorLocation` (`self.PlayerRef`)) (`self.K2_GetActorLocation` _array_element) (`self.StaticObjects`)))
        (if (not _returnvalue_2)
          (bind _asbp_enemy_base (cast `/Game/Blueprints/Enemies/BP_Enemy_Base` _array_element)
            (:`then`
              (if (`/Game/Blueprints/Enemies/BP_Enemy_Base.CanBePickedUp` _asbp_enemy_base)
                (bind _returnvalue_3 (`KismetMathLibrary.Vector_Distance` (`self.K2_GetActorLocation` _array_element) (`self.K2_GetActorLocation` (`self.PlayerRef`))))
                (if (< _returnvalue_3 (`self.Closest`)) :!label _label
                  (set `self.Closest` _returnvalue_3)
                  (set `self.CurrentFollowTarget` _array_element)
                  (set `self.OnObject` true))))
            (:`CastFailed`
              (goto _label)))))
      (if (`self.OnObject`)
        (set `self.FollowingPlayer` false)
        (else
          (set `self.FollowingPlayer` true)
          (set `self.CurrentFollowTarget` null)))
      (else
        (set `self.CurrentFollowTarget` null)
        (set `self.FollowingPlayer` true)
        (set `self.OnObject` false)))))

(fn `Flip`
  (params (FaceRight :type Boolean))
  (if (`self.FollowingPlayer`)
    (if FaceRight
      (`SceneComponent.K2_SetWorldRotation` (`self.Sprite`) (struct :`Yaw` 180.0) false true)
      (else
        (`SceneComponent.K2_SetWorldRotation` :`self` (`self.Sprite`) :`bTeleport` true)))))

(fn `InteractDown`
  (if (not (`self.FollowingPlayer`))
    (bind _returnvalue (`KismetSystemLibrary.K2_SetTimerDelegate` (`|CreateDelegate` :!event `AbsorbTarget`) 1.0))
    (set `self.InteractTimer` _returnvalue)))

(fn `InteractUp`
  (bind _currentfollowtarget (`self.CurrentFollowTarget`))
  (bind _playerref (`self.PlayerRef`))
  (`/Engine/EditorBlueprintResources/StandardMacros.IsValid` (`self.CurrentFollowTarget`)
    (:`Is Valid`
      (if (`self.HoldingItem`)
        (`KismetSystemLibrary.K2_ClearAndInvalidateTimerHandle` (`self.InteractTimer`) :!label _label)
        (else
          (`KismetSystemLibrary.K2_ClearAndInvalidateTimerHandle` (`self.InteractTimer`))
          (set `self.HoldingItem` true)
          (set `self.FollowingPlayer` true)
          (bind _asbp_enemy_base (cast `/Game/Blueprints/Enemies/BP_Enemy_Base` _currentfollowtarget)
            (:`then`
              (`/Game/Blueprints/Enemies/BP_Enemy_Base.DisablePlayerCollision` _asbp_enemy_base 0.0))
            (:`CastFailed`
              (bind _asbp_food_base (cast `/Game/Blueprints/World/BP_Food_Base` _currentfollowtarget))
              (`/Game/Blueprints/World/BP_Food_Base.DisableGravity` _asbp_food_base)))
          (`/Game/Blueprints/Player/BP_PlayerWithHat.Lose Hat` (`self.PlayerRef`)))))
    (:`Is Not Valid`
      (`/Game/Blueprints/Player/BP_PlayerWithHat.GainHat` _playerref (`/Game/Blueprints/Player/BP_PlayerWithHat.HasHat` _playerref))
      (goto _label))))

(fn `LaunchTarget`
  (params (Released :type Boolean))
  (bind _currentfollowtarget (`self.CurrentFollowTarget`))
  (bind _playerref (`self.PlayerRef`))
  (bind _playerref_2 (`self.PlayerRef`))
  (if Released
    (if (`self.HoldingItem`)
      (bind (_outactors _returnvalue) (`KismetSystemLibrary.SphereOverlapActors` (`self.K2_GetActorLocation`) 5.0 (`self.StaticObjects`)))
      (if (not _returnvalue)
        (`KismetSystemLibrary.K2_ClearAndInvalidateTimerHandle` (`self.InteractTimer`))
        (bind _aspaper_character (cast `PaperCharacter` (`self.CurrentFollowTarget`)))
        (`self.LaunchCharacter` _aspaper_character (+ (* (`/Game/Blueprints/Player/BP_PlayerWithHat.AimDir` _playerref) (`self.HatLaunchPower`)) (* (`self.GetVelocity` _playerref) 0.5)) true true)
        (bind _asbp_enemy_base (cast `/Game/Blueprints/Enemies/BP_Enemy_Base` _currentfollowtarget)
          (:`then`
            (`/Game/Blueprints/Enemies/BP_Enemy_Base.EnablePlayerCollision` _asbp_enemy_base 0.0))
          (:`CastFailed`
            (bind _asbp_food_base (cast `/Game/Blueprints/World/BP_Food_Base` _currentfollowtarget))
            (`/Game/Blueprints/World/BP_Food_Base.GrabbedByPlayer` _asbp_food_base)
            (`/Game/Blueprints/World/BP_Food_Base.GiveGravity` _asbp_food_base)))
        (set `self.CurrentFollowTarget` null)
        (set `self.HoldingItem` false)
        (set `self.FollowingPlayer` true)
        (`/Game/Blueprints/Player/BP_PlayerWithHat.GainHat` _playerref_2 (`/Game/Blueprints/Player/BP_PlayerWithHat.HasHat` _playerref_2) :!label _label))
      (else
        (goto _label)))))

(fn `UserConstructionScript`)