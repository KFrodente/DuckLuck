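; Title-screen player pawn that turns inventory input into menu navigation.
; On BeginPlay it adds the inventory mapping, aligns BP_Title to BP_PlayerWithHat and teleports to its spawn point.
; Move, confirm and secret inputs go to BP_Title, while cancel and remove message overlapping interactable menu items.
; FadeOut spawns a pop effect and destroys it; leftover inventory-duck functions change time dilation and mapping priority, and free-movement code is disconnected.
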(event `Fade Out`
  (bind (_returnvalue_location _returnvalue_rotation _returnvalue_scale) (`KismetMathLibrary.BreakTransform` (`self.GetTransform`)))
  (`NiagaraFunctionLibrary.SpawnSystemAtLocation` "/Game/Assets/Particles/NS_TitleScreenPop.NS_TitleScreenPop" _returnvalue_location _returnvalue_rotation _returnvalue_scale)
  (`self.K2_DestroyActor`))

(event `self.ReceiveBeginPlay`
  (bind _asbp_player_controller (cast `/Game/Blueprints/Player/BP_PlayerController` (`GameplayStatics.GetPlayerController` 0)))
  (`EnhancedInputSubsystemInterface.AddMappingContext` (pcsubsystem `EnhancedInputLocalPlayerSubsystem` _asbp_player_controller) "/Game/Blueprints/Input/Inventory/IMC_Inventory.IMC_Inventory" 1 (struct))
  (bind _returnvalue (`GameplayStatics.GetActorOfClass` "/Game/Blueprints/Inventory/BP_Title.BP_Title_C"))
  (set `self.TitleRef` _returnvalue)
  (bind _returnvalue_2 (`GameplayStatics.GetActorOfClass` "/Game/Blueprints/Player/BP_PlayerWithHat.BP_PlayerWithHat_C"))
  (bind (_returnvalue_x _returnvalue_y _returnvalue_z) (`KismetMathLibrary.BreakVector` (`self.K2_GetActorLocation` _returnvalue_2)))
  (`self.K2_SetActorLocation` _returnvalue (`KismetMathLibrary.MakeVector` _returnvalue_x 1.0 _returnvalue_z) false true)
  (`self.K2_SetActorLocation` (`SceneComponent.K2_GetComponentLocation` (`/Game/Blueprints/Inventory/BP_Title.PlayerSpawn` _returnvalue)) false true)
  (`/Game/Blueprints/Inventory/BP_Title.SetButtonLocations` (`self.TitleRef`)))

(event `EnhancedInput|/Game/Blueprints/Input/Inventory/IA_TitleSecret`
  (params (ActionValue :type Boolean) (ElapsedSeconds :type "Float (double-precision)") (TriggeredSeconds :type "Float (double-precision)") (InputAction :type "InputAction Object Reference" :default "/Game/Blueprints/Input/Inventory/IA_TitleSecret.IA_TitleSecret"))
  (:`Triggered`
    (`/Game/Blueprints/Inventory/BP_Title.Secret` (`self.TitleRef`))))

(event `EnhancedInput|/Game/Blueprints/Input/Inventory/IA_InvMovement`
  (params (ActionValue :type "Vector2D Structure") (ElapsedSeconds :type "Float (double-precision)") (TriggeredSeconds :type "Float (double-precision)") (InputAction :type "InputAction Object Reference" :default "/Game/Blueprints/Input/Inventory/IA_InvMovement.IA_InvMovement"))
  (:`Started`
    (`/Game/Blueprints/Inventory/BP_Title.GetNextBox` (`self.TitleRef`) (`KismetMathLibrary.MakeVector` ActionValue_Y ActionValue_X))))

(event `EnhancedInput|/Game/Blueprints/Input/Inventory/IA_InvConfirm`
  (params (ActionValue :type Boolean) (ElapsedSeconds :type "Float (double-precision)") (TriggeredSeconds :type "Float (double-precision)") (InputAction :type "InputAction Object Reference" :default "/Game/Blueprints/Input/Inventory/IA_InvConfirm.IA_InvConfirm"))
  (:`Triggered`
    (`/Game/Blueprints/Inventory/BP_Title.ConfirmSelected` (`self.TitleRef`))))

(event `EnhancedInput|/Game/Blueprints/Input/Inventory/IA_InvCancel`
  (params (ActionValue :type Boolean) (ElapsedSeconds :type "Float (double-precision)") (TriggeredSeconds :type "Float (double-precision)") (InputAction :type "InputAction Object Reference" :default "/Game/Blueprints/Input/Inventory/IA_InvCancel.IA_InvCancel"))
  (:`Triggered`
    (for _array_element (`self.GetOverlappingActors` "/Game/Blueprints/Inventory/Boxes/BP_MenuItem_Base.BP_MenuItem_Base_C")
      (if (`KismetSystemLibrary.DoesImplementInterface` _array_element "/Game/Blueprints/Interfaces_Enums/Interactable.Interactable_C")
        (message `/Game/Blueprints/Interfaces_Enums/Interactable.InteractSub` _array_element null false)))))

(event `EnhancedInput|/Game/Blueprints/Input/Inventory/IA_InvRemove`
  (params (ActionValue :type Boolean) (ElapsedSeconds :type "Float (double-precision)") (TriggeredSeconds :type "Float (double-precision)") (InputAction :type "InputAction Object Reference" :default "/Game/Blueprints/Input/Inventory/IA_InvRemove.IA_InvRemove"))
  (:`Triggered`
    (for _array_element (`self.GetOverlappingActors` "/Game/Blueprints/Inventory/Boxes/BP_MenuItem_Base.BP_MenuItem_Base_C")
      (if (`KismetSystemLibrary.DoesImplementInterface` _array_element "/Game/Blueprints/Interfaces_Enums/Interactable.Interactable_C")
        (message `/Game/Blueprints/Interfaces_Enums/Interactable.InteractSub` _array_element null true)))))

(fn `SetInventoryDuckActive`
  (bind _returnvalue (pcsubsystem `EnhancedInputLocalPlayerSubsystem` (`GameplayStatics.GetPlayerController` 0)))
  (set `self.CustomTimeDilation` 10100.0)
  (`EnhancedInputSubsystemInterface.RemoveMappingContext` _returnvalue "/Game/Blueprints/Input/Inventory/IMC_Inventory.IMC_Inventory" (struct))
  (`EnhancedInputSubsystemInterface.AddMappingContext` _returnvalue "/Game/Blueprints/Input/Inventory/IMC_Inventory.IMC_Inventory" 1 (struct)))

(fn `SetInventoryDuckInactive`
  (bind _returnvalue (pcsubsystem `EnhancedInputLocalPlayerSubsystem` (`GameplayStatics.GetPlayerController` 0)))
  (set `self.CustomTimeDilation` 0.0)
  (`EnhancedInputSubsystemInterface.RemoveMappingContext` _returnvalue "/Game/Blueprints/Input/Inventory/IMC_Inventory.IMC_Inventory" (struct))
  (`EnhancedInputSubsystemInterface.AddMappingContext` _returnvalue "/Game/Blueprints/Input/Inventory/IMC_Inventory.IMC_Inventory" 0 (struct)))

(fn `UserConstructionScript`)