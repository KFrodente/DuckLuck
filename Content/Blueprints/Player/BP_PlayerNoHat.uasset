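; BP_PlayerNoHat is a side-view sprite player character with Enhanced Input horizontal movement, facing flips, jumping and water buoyancy.
; Each tick, a short downward line trace sets grounded and jump state, then water logic adds height-scaled vertical velocity below the surface.
; SetWaterVars stores water bounds, zeroes gravity and vertical speed on slow entry, and restores gravity on exit, damping vertical speed after fast impacts.
; Jumping launches the character from ground or water.
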(event `self.ReceiveTick`
  (params (DeltaSeconds :type "Float (single-precision)"))
  (bind (_returnvalue_x _returnvalue_y _returnvalue_z) (`KismetMathLibrary.BreakVector` (`self.K2_GetActorLocation`)))
  (bind (_returnvalue_x_2 _returnvalue_y_2 _returnvalue_z_2) (`KismetMathLibrary.BreakVector` (`self.K2_GetActorLocation`)))
  (bind _charactermovement (`self.CharacterMovement`))
  (bind (_velocity_x _velocity_y _velocity_z) (`KismetMathLibrary.BreakVector` (`MovementComponent.Velocity` _charactermovement)))
  (`self.CheckGrounded`
    (:`FinishExecute`
      (if (`self.EnteredWater`)
        (if (< _returnvalue_z_2 (+ (`self.WaterHeight`) (`self.WaterOrigin`)))
          (set `MovementComponent.Velocity` (`KismetMathLibrary.MakeVector` _velocity_x 0.0 (+ _velocity_z (* 250.0 (+ 0.0 (/ _returnvalue_z (- (`self.WaterOrigin`) (`self.DistFromTop`))))))) _charactermovement))))))

(event `self.ReceiveBeginPlay`
  (bind _asbp_player_controller (cast `/Game/Blueprints/Player/BP_PlayerController` (`self.GetController`)))
  (`EnhancedInputSubsystemInterface.AddMappingContext` (pcsubsystem `EnhancedInputLocalPlayerSubsystem` _asbp_player_controller) "/Game/Blueprints/Input/IMC_Default.IMC_Default" 0 (struct)))

(event `EnhancedInput|/Game/Blueprints/Input/IA_Horizontal_Movement`
  (params (ActionValue :type "Float (double-precision)") (ElapsedSeconds :type "Float (double-precision)") (TriggeredSeconds :type "Float (double-precision)") (InputAction :type "InputAction Object Reference" :default "/Game/Blueprints/Input/IA_Horizontal_Movement.IA_Horizontal_Movement"))
  (bind _sprite (`self.Sprite`))
  (:`Triggered`
    (if (`self.PlayerHasInputControl`)
      (`self.AddMovementInput` (`self.GetActorForwardVector`) ActionValue)
      (if (> ActionValue 0.0)
        (`SceneComponent.K2_SetWorldRotation` _sprite (`KismetMathLibrary.MakeRotator` 0.0) false false)
        (set `self.FacingRight` true)
        (else
          (`SceneComponent.K2_SetWorldRotation` _sprite (`KismetMathLibrary.MakeRotator` 0.0 0.0 180.0) false false)
          (set `self.FacingRight` false))))))

(event `EnhancedInput|/Game/Blueprints/Input/IA_Jump`
  (params (ActionValue :type Boolean) (ElapsedSeconds :type "Float (double-precision)") (TriggeredSeconds :type "Float (double-precision)") (InputAction :type "InputAction Object Reference" :default "/Game/Blueprints/Input/IA_Jump.IA_Jump"))
  (:`Triggered`
    (if (and (not (`self.IsJumping`)) (or (`self.OnGround`) (`self.InWater`)))
      (`self.LaunchCharacter` (`KismetMathLibrary.MakeVector` 0.0 0.0 (`CharacterMovementComponent.JumpZVelocity` (`self.CharacterMovement`))) false true)
      (set `self.IsJumping` true)
      (if (not (`self.InWater`))
        (set `self.EnteredWater` false)))))

(fn `SetWaterVars`
  (params (InWater :type Boolean) (WaterHeight :type "Float (double-precision)") (WaterOrigin :type "Float (double-precision)"))
  (bind _charactermovement (`self.CharacterMovement`))
  (bind (_velocity_x _velocity_y _velocity_z) (`KismetMathLibrary.BreakVector` (`MovementComponent.Velocity` _charactermovement)))
  (bind (_velocity_x_2 _velocity_y_2 _velocity_z_2) (`KismetMathLibrary.BreakVector` (`MovementComponent.Velocity` (`self.CharacterMovement`))))
  (if InWater
    (set `self.InWater` true)
    (set `self.CanSetWaterBounces` true)
    (set `self.EnteredWater` true)
    (set `self.WaterHeight` WaterHeight)
    (set `self.WaterOrigin` WaterOrigin)
    (set `self.DistFromTop` (* (`self.WaterHeight`) 0.2))
    (if (< (`KismetMathLibrary.Abs` _velocity_z_2) 500.0)
      ;[1 1 1] Stops the player at the top of the water and allows them to jump
      (set `self.IsJumping` false)
      (set `MovementComponent.Velocity` (`KismetMathLibrary.MakeVector` _velocity_x_2) _charactermovement)
      (set `CharacterMovementComponent.GravityScale` 0.0 _charactermovement)
      (set `self.WaterImpactsHeight` false)
      (else
        (set `self.WaterImpactsHeight` true)))
    (else
      (set `self.InWater` false)
      (set `self.WaterHeight` 0.0)
      (set `self.WaterOrigin` 0.0)
      (set `self.DistFromTop` 0.0)
      (set `CharacterMovementComponent.GravityScale` (`self.OGravityScale`) _charactermovement)
      (if (`self.WaterImpactsHeight`)
        (set `MovementComponent.Velocity` (`KismetMathLibrary.MakeVector` _velocity_x 0.0 (* _velocity_z 0.1)) _charactermovement)))))

(fn `UserConstructionScript`)