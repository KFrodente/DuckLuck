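; Player character for a sprite-based side-on shooter, handling movement, jumping, directional dashing and gun firing through Enhanced Input.
; Dashes launch along the aim direction with gravity off, then diminish velocity; Tick blocks damage while dashing and uses a ground trace to restore dash and jump.
; Power dash boosts horizontal speed, easing back via timeline.
; BeginPlay spawns pistol and shotgun using WeaponStats, equipping the shotgun; aim rotates the gun and selects its fire point.
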(event `self.ReceiveTick`
  (params (DeltaSeconds :type "Float (single-precision)"))
  (set `self.FireRateTimer` (- (`self.FireRateTimer`) DeltaSeconds))
  (`self.DashInvincibility`)
  (`self.CheckGrounded`))

(event `self.ReceiveBeginPlay`
  (bind _mainweapon (`self.MainWeapon`))
  (bind _asbp_player_controller (cast `/Game/Blueprints/Player/BP_PlayerController` (`self.GetController`)))
  (`EnhancedInputSubsystemInterface.AddMappingContext` (pcsubsystem `EnhancedInputLocalPlayerSubsystem` _asbp_player_controller) "/Game/Blueprints/Input/IMC_Default.IMC_Default" 0 (struct))
  (set `CharacterMovementComponent.MaxWalkSpeed` (`self.OWalkSpeed`) (`self.CharacterMovement`))
  (`self.MakePistol`)
  (`self.MakeShotgun`)
  (set `self.MainWeapon` (`self.Shotgun`))
  (`|ExecutionSequence`
    (:`then_0`
      (add `self.WeaponSwapped` (delegate `WeaponSwapped_Event`))
      (set `self.FirePoint` (`Weapon.m_RFirePoint` _mainweapon))
      (`PaperSpriteComponent.SetSprite` (`self.GunSection`) (`PaperSpriteComponent.GetSprite` (`PaperSpriteActor.RenderComponent` _mainweapon))))
    (:`then_1`
      (if true
        (`self.WeaponSwapped`)
        (`WeaponStatsComponent.ReCheckWeaponStats` (`self.WeaponStats`) (`Weapon.m_WeaponNumber` (`self.MainWeapon`)) 0)))))

(event `WeaponSwapped_Event`)

(event `EnhancedInput|/Game/Blueprints/Input/IA_Horizontal_Movement`
  (params (ActionValue :type "Float (double-precision)") (ElapsedSeconds :type "Float (double-precision)") (TriggeredSeconds :type "Float (double-precision)") (InputAction :type "InputAction Object Reference" :default "/Game/Blueprints/Input/IA_Horizontal_Movement.IA_Horizontal_Movement"))
  (:`Triggered`
    (if (`self.PlayerHasInputControl`)
      (`self.AddMovementInput` (`self.GetActorForwardVector`) ActionValue)
      (if (> ActionValue 0.0)
        (`SceneComponent.K2_SetWorldRotation` (`self.Sprite`) (`KismetMathLibrary.MakeRotator` 0.0) false false)
        (set `self.FacingRight` true)
        (else
          (`SceneComponent.K2_SetWorldRotation` (`self.Sprite`) (`KismetMathLibrary.MakeRotator` 0.0 0.0 180.0) false false)
          (set `self.FacingRight` false))))))

(event `EnhancedInput|/Game/Blueprints/Input/IA_Jump`
  (params (ActionValue :type Boolean) (ElapsedSeconds :type "Float (double-precision)") (TriggeredSeconds :type "Float (double-precision)") (InputAction :type "InputAction Object Reference" :default "/Game/Blueprints/Input/IA_Jump.IA_Jump"))
  (bind _charactermovement (`self.CharacterMovement`))
  (:`Triggered`
    (if (not (`self.IsJumping`))
      (if (`NavMovementComponent.IsFalling` _charactermovement)
        (`self.LaunchCharacter` (`KismetMathLibrary.MakeVector` 0.0 0.0 (* (`CharacterMovementComponent.JumpZVelocity` _charactermovement) 2.0)) false true)
        (else
          (`self.Jump`)))
      (set `self.IsJumping` true)))
  (:`Canceled`
    (`self.StopJumping` :!label _label))
  (:`Completed`
    (goto _label)))

(event `EnhancedInput|/Game/Blueprints/Input/IA_Dash`
  (params (ActionValue :type Boolean) (ElapsedSeconds :type "Float (double-precision)") (TriggeredSeconds :type "Float (double-precision)") (InputAction :type "InputAction Object Reference" :default "/Game/Blueprints/Input/IA_Dash.IA_Dash"))
  (bind _charactermovement (`self.CharacterMovement`))
  (bind (_velocity_x _velocity_y _velocity_z) (`KismetMathLibrary.BreakVector` (`MovementComponent.Velocity` _charactermovement)))
  (:`Triggered`
    (if (`self.CanDash`)
      (bind _output_get (set `self.DashDir` (`self.AimDir`)))
      (if (and (!= (.x _output_get) 0.0) (!= (.z _output_get) 0.0))
        (set `self.NVerticalDashDiminish` (* (`self.OVerticalDashDiminish`) 0.8))
        (set `self.NHorizontalDashDiminish` (* (`self.OHorizontalDashDiminish`) 0.8)))
      (if (and (!= (.x _output_get) 0.0) (== (.z _output_get) 0.0))
        (if (not (`self.Dashing`))
          (set `self.Dashing` true)
          (set `self.CanDash` false)
          (set `CharacterMovementComponent.GravityScale` 0.0 (`self.CharacterMovement`))
          (`self.LaunchCharacter` (`KismetMathLibrary.MakeVector` (* (.x (* (`KismetMathLibrary.Normal` (`self.DashDir`)) (`self.DashSpeedMultiplier`))) (`self.DashHorizontalSpeedMult`))) true true)
          (`KismetSystemLibrary.Delay` (`self.DashLength`) :!label _label_2)
          (set `self.Dashing` false)
          (set `CharacterMovementComponent.GravityScale` (`self.OGravityScale`) _charactermovement)
          (bind _output_get_2 (set `MovementComponent.Velocity` (`KismetMathLibrary.MakeVector` (* _velocity_x (`self.NHorizontalDashDiminish`)) 0.0 (* _velocity_z (`self.NVerticalDashDiminish`))) _charactermovement))
          (`self.LaunchCharacter` _output_get_2 true true)
          (set `self.NHorizontalDashDiminish` (`self.OHorizontalDashDiminish`))
          (set `self.NVerticalDashDiminish` (`self.OVerticalDashDiminish`)))
        (elif (not (`self.Dashing`))
          (set `self.Dashing` true)
          (set `self.CanDash` false)
          (set `CharacterMovementComponent.GravityScale` 0.0 (`self.CharacterMovement`))
          (`self.LaunchCharacter` (`KismetMathLibrary.MakeVector` (* (.x (* (`KismetMathLibrary.Normal` (`self.DashDir`)) (`self.DashSpeedMultiplier`))) (`self.DashHorizontalSpeedMult`)) (.y (* (`KismetMathLibrary.Normal` (`self.DashDir`)) (`self.DashSpeedMultiplier`))) (.z (* (`KismetMathLibrary.Normal` (`self.DashDir`)) (`self.DashSpeedMultiplier`)))) true true)
          (goto _label_2))))))

(event `EnhancedInput|/Game/Blueprints/Input/IA_Power_Dash`
  (params (ActionValue :type Boolean) (ElapsedSeconds :type "Float (double-precision)") (TriggeredSeconds :type "Float (double-precision)") (InputAction :type "InputAction Object Reference" :default "/Game/Blueprints/Input/IA_Power_Dash.IA_Power_Dash"))
  (bind (_dashdir_x _dashdir_y _dashdir_z) (`KismetMathLibrary.BreakVector` (`self.DashDir`)))
  (bind _charactermovement (`self.CharacterMovement`))
  (bind _x (.x (* (`MovementComponent.Velocity` _charactermovement) (`KismetMathLibrary.MakeVector` (`self.PowerDashMult`) 1.0 1.0))))
  (:`Triggered`
    (if (== _dashdir_z 0.0)
      (set `MovementComponent.Velocity` (`KismetMathLibrary.MakeVector` _x 0.0 (.z (* (`MovementComponent.Velocity` _charactermovement) (`KismetMathLibrary.MakeVector` (`self.PowerDashMult`) 1.0 1.0)))) _charactermovement)
      (bind _output_get (set `CharacterMovementComponent.MaxWalkSpeed` (`KismetMathLibrary.Abs` _x) _charactermovement)) ; output should be sent in as the "A" value in the lerp function
      (bind (_direction _newtrack_0) (`Timeline|powerdash slowdown` :!via `PlayFromStart`)
        (:`Update`
          (set `CharacterMovementComponent.MaxWalkSpeed` (`KismetMathLibrary.Lerp` _output_get (`self.OWalkSpeed`) _newtrack_0) _charactermovement))))))

(event `EnhancedInput|/Game/Blueprints/Input/IA_FireGun`
  (params (ActionValue :type Boolean) (ElapsedSeconds :type "Float (double-precision)") (TriggeredSeconds :type "Float (double-precision)") (InputAction :type "InputAction Object Reference" :default "/Game/Blueprints/Input/IA_FireGun.IA_FireGun"))
  (:`Triggered`
    (if (not (> (`self.FireRateTimer`) 0.0))
      (set `self.FireRateTimer` (`WeaponStatsComponent.firerate` (`self.WeaponStats`)))
      (bind (_fireagain _delay) (`/Game/Blueprints/Weapons/BP_WeaponParent.FireWeapon` (`self.MainWeapon`) (`KismetMathLibrary.MakeTransform` (+ (`self.K2_GetActorLocation`) (`self.FirePoint`)) (`SceneComponent.K2_GetComponentRotation` (`self.GunSection`))) (`WeaponStatsComponent.bulletVelocity` (`self.WeaponStats`)) :!label _label_3))
      (if _fireagain
        (`KismetSystemLibrary.Delay` _delay)
        (goto _label_3)))))

(event `EnhancedInput|/Game/Blueprints/Input/IA_Vertical_Movement`
  (params (ActionValue :type "Float (double-precision)") (ElapsedSeconds :type "Float (double-precision)") (TriggeredSeconds :type "Float (double-precision)") (InputAction :type "InputAction Object Reference" :default "/Game/Blueprints/Input/IA_Vertical_Movement.IA_Vertical_Movement"))
  (bind _mainweapon (`self.MainWeapon`))
  (bind (_returnvalue_roll _returnvalue_pitch _returnvalue_yaw) (`KismetMathLibrary.BreakRotator` (`SceneComponent.K2_GetComponentRotation` (`self.Sprite`))))
  (:`Triggered`
    (`SceneComponent.K2_SetWorldRotation` (`self.GunSection`) (`KismetMathLibrary.MakeRotator` 0.0 (* (`KismetMathLibrary.SignOfFloat` ActionValue) 90.0) _returnvalue_yaw) false false :!label _label_4)
    (if (== ActionValue 0.0) :!label _label_5
      (if (`self.FacingRight`)
        (set `self.FirePoint` (`Weapon.m_RFirePoint` _mainweapon))
        (else
          (set `self.FirePoint` (`Weapon.m_LFirePoint` _mainweapon))))
      (elif (> ActionValue 0.0)
        (set `self.FirePoint` (`Weapon.m_UFirePoint` _mainweapon))
        (else
          (set `self.FirePoint` (`Weapon.m_DFirePoint` _mainweapon))))))
  (:`Completed`
    (goto _label_4)))

(event `EnhancedInput|/Game/Blueprints/Input/IA_Horizontal_Movement`
  (params (ActionValue :type "Float (double-precision)") (ElapsedSeconds :type "Float (double-precision)") (TriggeredSeconds :type "Float (double-precision)") (InputAction :type "InputAction Object Reference" :default "/Game/Blueprints/Input/IA_Horizontal_Movement.IA_Horizontal_Movement"))
  (:`Triggered`
    (goto _label_5))
  (:`Completed`
    (goto _label_5)))

(event `EnhancedInput|/Game/Blueprints/Input/IA_Horizontal_Movement`
  (params (ActionValue :type "Float (double-precision)") (ElapsedSeconds :type "Float (double-precision)") (TriggeredSeconds :type "Float (double-precision)") (InputAction :type "InputAction Object Reference" :default "/Game/Blueprints/Input/IA_Horizontal_Movement.IA_Horizontal_Movement"))
  (:`Triggered`
    (set `self.AimDir` (`KismetMathLibrary.MakeVector` ActionValue 0.0 (stale `EnhancedInput|/Game/Blueprints/Input/IA_Vertical_Movement` ActionValue)) :!label _label_6))
  (:`Completed`
    (goto _label_6)))

(event `EnhancedInput|/Game/Blueprints/Input/IA_Vertical_Movement`
  (params (ActionValue :type "Float (double-precision)") (ElapsedSeconds :type "Float (double-precision)") (TriggeredSeconds :type "Float (double-precision)") (InputAction :type "InputAction Object Reference" :default "/Game/Blueprints/Input/IA_Vertical_Movement.IA_Vertical_Movement"))
  (:`Triggered`
    (goto _label_6))
  (:`Completed`
    (goto _label_6)))

(fn `NewFunction`
  (returns (CharacterMovement :type "CharacterMovementComponent Object Reference") (CharacterMovement2 :type "CharacterMovementComponent Object Reference")))

(fn `UserConstructionScript`)