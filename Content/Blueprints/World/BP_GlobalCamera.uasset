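; Global camera actor that follows a target, starting with the player character, at a configurable offset and copies its rotation.
; Every Tick it teleports to an interpolated position using per-axis speeds; FollowNewActor swaps target, offset and inventory mode.
; Inventory mode swaps the Y/Z offsets, snaps Z and skips shake.
; ScreenShake adds X/Z offsets, with looping timer-driven random sign flips and a second timer to stop it.
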(event `self.ReceiveBeginPlay`
  (set `self.CurrentFollowTarget` (`GameplayStatics.GetPlayerCharacter` 0))
  (set `self.CurrentFollowDistance` (0.0 1000.0 0.0)))

(event `self.ReceiveTick`
  (params (DeltaSeconds :type "Float (single-precision)"))
  (bind (_returnvalue_x _returnvalue_y) (`KismetMathLibrary.BreakVector` (`self.K2_GetActorLocation`)))
  (bind _returnvalue_x_2 (`KismetMathLibrary.BreakVector` (`self.K2_GetActorLocation`)))
  (bind _returnvalue (`GameplayStatics.GetWorldDeltaSeconds`))
  (bind (_returnvalue_x_3 _returnvalue_y_2 _returnvalue_z) (`KismetMathLibrary.BreakVector` (`self.K2_GetActorLocation`)))
  (bind (_returnvalue_x_4 _returnvalue_y_3) (`KismetMathLibrary.BreakVector` (`self.K2_GetActorLocation`)))
  (bind (_currentfollowdistance_x _currentfollowdistance_y _currentfollowdistance_z) (`KismetMathLibrary.BreakVector` (`self.CurrentFollowDistance`)))
  (bind (_currentfollowdistance_x_2 _currentfollowdistance_y_2 _currentfollowdistance_z_2) (`KismetMathLibrary.BreakVector` (`self.CurrentFollowDistance`)))
  (bind _returnvalue_2 (`self.GetTransform` (`self.CurrentFollowTarget`)))
  (bind _returnvalue_3 (`self.GetTransform` (`self.CurrentFollowTarget`)))
  (if (`self.TargetIsInventory`)
    (`self.K2_SetActorTransform` (`KismetMathLibrary.MakeTransform` (`KismetMathLibrary.MakeVector` (`KismetMathLibrary.FInterpTo` _returnvalue_x_2 (+ (.x (.location _returnvalue_2)) _currentfollowdistance_x) (`GameplayStatics.GetWorldDeltaSeconds`) 15.0) (`KismetMathLibrary.FInterpTo` _returnvalue_y (+ (.y (.location _returnvalue_2)) _currentfollowdistance_z) (`GameplayStatics.GetWorldDeltaSeconds`) 10.0) (+ (.z (.location _returnvalue_2)) _currentfollowdistance_y)) (`KismetMathLibrary.MakeRotator` (.roll (.rotation _returnvalue_2)) (.pitch (.rotation _returnvalue_2)) (.yaw (.rotation _returnvalue_2)))) false true)
    (else
      (`self.K2_SetActorTransform` (`KismetMathLibrary.MakeTransform` (`KismetMathLibrary.MakeVector` (`KismetMathLibrary.FInterpTo` _returnvalue_x_4 (+ (.x (.location _returnvalue_3)) _currentfollowdistance_x_2 (`self.SHXVal`)) _returnvalue 15.0) (`KismetMathLibrary.FInterpTo` _returnvalue_y_3 (+ (.y (.location _returnvalue_3)) _currentfollowdistance_y_2) _returnvalue 1.0) (`KismetMathLibrary.FInterpTo` _returnvalue_z (+ (.z (.location _returnvalue_3)) _currentfollowdistance_z_2 (`self.SHZVal`)) (`GameplayStatics.GetWorldDeltaSeconds`) 10.0)) (`KismetMathLibrary.MakeRotator` (.roll (.rotation _returnvalue_3)) (.pitch (.rotation _returnvalue_3)) (.yaw (.rotation _returnvalue_3)))) false true))))

(event `ScreenShake`
  (params (XAmount :type "Float (double-precision)") (ZAmount :type "Float (double-precision)") (Speed :type "Float (double-precision)") (Length :type "Float (double-precision)"))
  (set `self.SHXVal` XAmount)
  (set `self.SHZVal` ZAmount)
  (bind _returnvalue (`KismetSystemLibrary.K2_SetTimerDelegate` (delegate `FlipScreenShake`) Speed true))
  (set `self.SHFlipTimer` _returnvalue)
  (bind _returnvalue_2 (`KismetSystemLibrary.K2_SetTimerDelegate` (delegate `StopScreenShake`) Length))
  (set `self.SHStopTimer` _returnvalue_2))

(event `FlipScreenShake`
  (`/Game/BasicFunctions.*= (float)` (`self.SHXVal`) (`KismetMathLibrary.SelectFloat` 1.0 -1.0 (`KismetMathLibrary.RandomBool`)))
  (`/Game/BasicFunctions.*= (float)` (`self.SHZVal`) (`KismetMathLibrary.SelectFloat` 1.0 -1.0 (`KismetMathLibrary.RandomBool`))))

(event `StopScreenShake`
  (`KismetSystemLibrary.K2_ClearAndInvalidateTimerHandle` (`self.SHFlipTimer`))
  (set `self.SHXVal` 0.0)
  (set `self.SHZVal` 0.0))

(fn `FollowNewActor`
  (params (WantedActor :type "Actor Object Reference") (FollowDistance :type "Vector Structure") (InventoryDuck :type Boolean))
  (set `self.CurrentFollowTarget` WantedActor)
  (set `self.CurrentFollowDistance` FollowDistance)
  (set `self.TargetIsInventory` InventoryDuck))

(fn `UserConstructionScript`)