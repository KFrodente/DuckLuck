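; Inventory camera actor that follows a target, by its name serving the inventory view.
; Each Tick, while CurrentFollowTarget is valid, it snaps to that target's world location with a fixed -90 degree rotation.
; Two smoothed-follow graphs, one for inventory and one for everything else, interpolate different axes with offsets, but their branch never runs.
; FollowNewActor is an empty stub, so nothing here assigns the target.
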(event `self.ReceiveBeginPlay`)

(event `self.ReceiveTick`
  (params (DeltaSeconds :type "Float (single-precision)"))
  (bind _currentfollowtarget (`self.CurrentFollowTarget`))
  (`/Engine/EditorBlueprintResources/StandardMacros.IsValid` _currentfollowtarget
    (:`Is Valid`
      (`self.K2_SetActorTransform` (`KismetMathLibrary.MakeTransform` (`SceneComponent.K2_GetComponentLocation` _currentfollowtarget) (struct :`Roll` -90.0))))))

(fn `FollowNewActor`
  (params (WantedActor :type "Actor Object Reference") (FollowDistance :type "Vector Structure") (InventoryDuck :type Boolean)))

(fn `UserConstructionScript`)