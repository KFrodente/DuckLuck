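; One-way platform that lets the BP_PlayerWithHat player pass through from one side, using an Open trigger box to toggle a Collision box.
; Entering Open disables collision on the Collision box; leaving it restores query and physics collision.
; The construction script sizes Open, Close and Collision from Width in 32-unit steps, with Open slightly wider, and keeps only the actor's X and Z location.
; The Close box has no event logic.
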(event `self.Open.OnComponentBeginOverlap`
  (params (OverlappedComponent :type "PrimitiveComponent Object Reference") (OtherActor :type "Actor Object Reference") (OtherComp :type "PrimitiveComponent Object Reference") (OtherBodyIndex :type Integer) (bFromSweep :type Boolean) (SweepResult :type "HitResult Structure (by ref)"))
  (cast `/Game/Blueprints/Player/BP_PlayerWithHat` OtherActor)
  (`PrimitiveComponent.SetCollisionEnabled` (`self.Collision`) "NoCollision"))

(event `self.Open.OnComponentEndOverlap`
  (params (OverlappedComponent :type "PrimitiveComponent Object Reference") (OtherActor :type "Actor Object Reference") (OtherComp :type "PrimitiveComponent Object Reference") (OtherBodyIndex :type Integer))
  (cast `/Game/Blueprints/Player/BP_PlayerWithHat` OtherActor)
  (`PrimitiveComponent.SetCollisionEnabled` (`self.Collision`) "QueryAndPhysics"))

(fn `UserConstructionScript`
  (bind (_returnvalue_x _returnvalue_y _returnvalue_z) (`KismetMathLibrary.BreakVector` (`self.K2_GetActorLocation`)))
  (bind _open (`self.Open`))
  (bind _close (`self.Close`))
  (bind _collision (`self.Collision`))
  (bind (_boxextent_x _boxextent_y _boxextent_z) (`KismetMathLibrary.BreakVector` (`BoxComponent.BoxExtent` _open)))
  (bind (_boxextent_x_2 _boxextent_y_2 _boxextent_z_2) (`KismetMathLibrary.BreakVector` (`BoxComponent.BoxExtent` _collision)))
  (bind (_boxextent_x_3 _boxextent_y_3 _boxextent_z_3) (`KismetMathLibrary.BreakVector` (`BoxComponent.BoxExtent` _close)))
  (`BoxComponent.SetBoxExtent` _open (`KismetMathLibrary.MakeVector` (`KismetMathLibrary.Conv_IntToDouble` (* (+ (`self.Width`) 1) 32)) _boxextent_y _boxextent_z) true)
  (`BoxComponent.SetBoxExtent` _close (`KismetMathLibrary.MakeVector` (`KismetMathLibrary.Conv_IntToDouble` (* (`self.Width`) 32)) _boxextent_y_3 _boxextent_z_3) true)
  (`BoxComponent.SetBoxExtent` _collision (`KismetMathLibrary.MakeVector` (`KismetMathLibrary.Conv_IntToDouble` (* (`self.Width`) 32)) _boxextent_y_2 _boxextent_z_2) true)
  (`self.K2_SetActorLocation` (`KismetMathLibrary.MakeVector` _returnvalue_x 0.0 _returnvalue_z)))