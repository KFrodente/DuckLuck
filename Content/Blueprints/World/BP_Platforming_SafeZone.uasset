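; BP_Platforming_SafeZone is a checkpoint for platforming sections that can send the player back to its marked spot.
; When BP_PlayerWithHat overlaps it, it registers itself as the current safe space on the platforming manager.
; ReturnToZone makes the connected zone the active view and launches the player along a given direction.
; A short timer then teleports player character 0 to the zone's Arrow location.
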(event `self.ReceiveBeginPlay`
  (bind _returnvalue (`GameplayStatics.GetActorOfClass` "/Game/Blueprints/Player/BP_PlayerWithHat.BP_PlayerWithHat_C"))
  (set `self.PlayerRef` _returnvalue))

(event `self.ReceiveActorBeginOverlap`
  (params (OtherActor :type "Actor Object Reference"))
  (bind _platformingmanagerref (`self.PlatformingManagerRef`))
  (cast `/Game/Blueprints/Player/BP_PlayerWithHat` OtherActor)
  (`/Engine/EditorBlueprintResources/StandardMacros.IsValid` _platformingmanagerref
    (:`Is Valid`
      (set `/Game/Blueprints/World/BP_PlatformingManager.CurrentSafeSpace` self _platformingmanagerref))))

(fn `ReturnToZone`
  (params (PlayerLaunchDir :type "Vector Structure"))
  (`/Game/Blueprints/World/BP_PlatformingZone.SetAsActiveView` (`self.ConnectedZone`))
  (`Character.LaunchCharacter` (`self.PlayerRef`) (* (`local.PlayerLaunchDir`) 2000.0) true true)
  (`KismetSystemLibrary.K2_SetTimer` null "TeleportPlayer" 0.2))

(fn `TeleportPlayer`
  (`self.K2_SetActorLocation` (`GameplayStatics.GetPlayerCharacter` 0) (`SceneComponent.K2_GetComponentLocation` (`self.Arrow`)) false false))

(fn `UserConstructionScript`)