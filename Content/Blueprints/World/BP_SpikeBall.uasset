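; BP_SpikeBall is a world hazard that deals one point of non-age damage to any BP_PlayerWithHat that overlaps it.
; The overlap event casts the other actor to the player and calls TakeDamage with itself as the dealer.
; The construction script sizes the collision box from BaseSize and a Tiles count along X and Z, and resets the actor's Y location to zero, keeping it on the 2D plane.
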(event `self.ReceiveActorBeginOverlap`
  (params (OtherActor :type "Actor Object Reference"))
  (bind _asbp_player_with_hat (cast `/Game/Blueprints/Player/BP_PlayerWithHat` OtherActor))
  (`/Game/Blueprints/Interfaces_Enums/I_Damagable.Take Damage` _asbp_player_with_hat 1 self false))

(fn `UserConstructionScript`
  (bind (_returnvalue_x _returnvalue_y _returnvalue_z) (`KismetMathLibrary.BreakVector` (`self.K2_GetActorLocation`)))
  (bind (_basesize_x _basesize_y _basesize_z) (`KismetMathLibrary.BreakVector` (`self.BaseSize`)))
  (bind (_tiles_x _tiles_y) (`KismetMathLibrary.BreakVector2D` (`self.Tiles`)))
  (`BoxComponent.SetBoxExtent` (`self.Box`) (`KismetMathLibrary.MakeVector` (+ _basesize_x (* (- _tiles_x 1.0) 32.0)) _basesize_y (+ _basesize_z (* (- _tiles_y 1.0) 32.0))) true)
  (`self.K2_SetActorLocation` (`KismetMathLibrary.MakeVector` _returnvalue_x 0.0 _returnvalue_z)))