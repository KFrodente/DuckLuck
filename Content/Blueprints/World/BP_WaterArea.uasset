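; BP_WaterArea is a box volume that tells player characters when they are in water.
; On actor overlap it casts to BP_PlayerNoHat, falling back to BP_PlayerWithHat, and ignores other actors.
; Entering passes the Box's vertical extent and center Z to the player's SetWaterVars with the in-water flag set; leaving clears the flag and zeroes both values.
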(event `self.ReceiveActorBeginOverlap`
  (params (OtherActor :type "Actor Object Reference"))
  (bind (_origin _boxextent) (`KismetSystemLibrary.GetComponentBounds` (`self.Box`)))
  (bind _asbp_player_no_hat (cast `/Game/Blueprints/Player/BP_PlayerNoHat` OtherActor)
    (:`then`
      (`/Game/Blueprints/Player/BP_PlayerNoHat.SetWaterVars` _asbp_player_no_hat true (.z _boxextent) (.z _origin)))
    (:`CastFailed`
      (bind _asbp_player_with_hat (cast `/Game/Blueprints/Player/BP_PlayerWithHat` OtherActor))
      (`/Game/Blueprints/Player/BP_PlayerWithHat.SetWaterVars` _asbp_player_with_hat true (.z _boxextent) (.z _origin)))))

(event `self.ReceiveActorEndOverlap`
  (params (OtherActor :type "Actor Object Reference"))
  (bind _asbp_player_no_hat (cast `/Game/Blueprints/Player/BP_PlayerNoHat` OtherActor)
    (:`then`
      (`/Game/Blueprints/Player/BP_PlayerNoHat.SetWaterVars` _asbp_player_no_hat false 0.0 0.0))
    (:`CastFailed`
      (bind _asbp_player_with_hat (cast `/Game/Blueprints/Player/BP_PlayerWithHat` OtherActor))
      (`/Game/Blueprints/Player/BP_PlayerWithHat.SetWaterVars` _asbp_player_with_hat false 0.0 0.0))))

(fn `UserConstructionScript`)