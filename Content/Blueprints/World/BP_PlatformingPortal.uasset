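; BP_PlatformingPortal is a world portal that teleports player character 0 to its ConnectedPortal's location via TeleportPlayer, then prints a debug message.
; With LaunchesPlayer set, it first launches the character along the player-to-portal direction.
; That direction snaps per X and Z axis to a signed half-unit or zero using a dead zone, then scales by horizontal and vertical strengths.
; No trigger calls TeleportPlayer within this Blueprint.
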(fn `TeleportPlayer`
  (bind _returnvalue (`GameplayStatics.GetPlayerCharacter` 0))
  (bind (_returnvalue_x _returnvalue_y _returnvalue_z) (`KismetMathLibrary.BreakVector` (`KismetMathLibrary.Normal` (- (`self.K2_GetActorLocation`) (`self.K2_GetActorLocation` _returnvalue)))))
  (if (`self.LaunchesPlayer`)
    (`Character.LaunchCharacter` _returnvalue (`KismetMathLibrary.MakeVector` (* (select `bool` (> (- (`KismetMathLibrary.Abs` _returnvalue_x) 0.4) 0.0) :`true` (* (`KismetMathLibrary.SignOfFloat` _returnvalue_x) 0.5)) (`self.HoriLaunchStrength`)) 0.0 (* (select `bool` (> (- (`KismetMathLibrary.Abs` _returnvalue_z) 0.4) 0.0) :`true` (* (`KismetMathLibrary.SignOfFloat` _returnvalue_z) 0.5)) (`self.VertLaunchStrength`))) false false))
  (`self.K2_SetActorLocation` (`GameplayStatics.GetPlayerCharacter` 0) (`self.K2_GetActorLocation` (`self.ConnectedPortal`)) false true)
  (`KismetSystemLibrary.PrintString` "teleported"))

(fn `UserConstructionScript`)