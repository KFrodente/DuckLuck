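; FoodSource is a component that holds a consumable food supply, optionally regenerating over time.
; RemoveFood deducts up to the requested amount and marks the source inactive when empty, but destroys a non-regenerating component on any call, returning zero.
; On Tick, regenerating sources below maximum start a randomized countdown, whose expiry flags the next Tick to add a fixed amount and reactivate the source.
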(event `self.ReceiveTick`
  (params (DeltaSeconds :type "Float (single-precision)"))
  (if (`self.CanRegenerate`)
    (set `self.FoodRemaining` (+ (`self.FoodRemaining`) (`self.RegenerationAmount`)))
    (set `self.CanRegenerate` false)
    (set `self.ActiveFoodSource` true))
  (`self.CheckRegeneration`)
  (if (>= (`self.RegenerationTimer`) 0.0)
    (bind _output_get (set `self.RegenerationTimer` (- (`self.RegenerationTimer`) DeltaSeconds)))
    (if (<= _output_get 0.0)
      (set `self.CanRegenerate` true))))

(fn `CheckRegeneration`
  (if (`self.Regenerates`)
    (if (and (< (`self.FoodRemaining`) (`self.MaxFoodAmount`)) (<= (`self.RegenerationTimer`) 0.0))
      (set `self.RegenerationTimer` (`KismetMathLibrary.RandomFloatInRange` 25.0 40.0)))))

(fn `RemoveFood`
  (params (Amount :type "Float (double-precision)"))
  (returns (WhatWasUsed :type "Float (double-precision)"))
  (bind _foodremaining (`self.FoodRemaining`))
  (bind _returnvalue (- _foodremaining Amount))
  (set `self.What Was Used` 0.0)
  (if (<= _returnvalue 0.0)
    (set `self.What Was Used` _foodremaining)
    (set `self.FoodRemaining` 0.0)
    (set `self.ActiveFoodSource` false)
    (else
      (set `self.What Was Used` Amount)
      (set `self.FoodRemaining` _returnvalue)))
  (if (not (`self.Regenerates`))
    (`self.K2_DestroyComponent`)
    (return 0.0)))