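; BP_WaterArea is a water volume that tells player characters when they are in water.
; When a BP_PlayerWithHat enters, it receives the box's vertical extent and origin plus a PlatformingBlock value via SetWaterVars, and a randomly pitched splash plays.
; On exit, either BP_PlayerNoHat or BP_PlayerWithHat has SetWaterVars called with default values.
; Only the hat player is handled on entry.
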(event `self.ReceiveBeginPlay`)

(event `self.ReceiveActorBeginOverlap`
  (params (OtherActor :type "Actor Object Reference"))
  (bind (_origin _boxextent) (`KismetSystemLibrary.GetComponentBounds` (`self.Box`)))
  (bind _asbp_player_with_hat (cast `/Game/Blueprints/Player/BP_PlayerWithHat` OtherActor))
  (`/Game/Blueprints/Player/BP_PlayerWithHat.SetWaterVars` _asbp_player_with_hat true (.z _boxextent) (.z _origin) (`self.PlatformingBlock`))
  (`GameplayStatics.PlaySound2D` "/Game/Assets/Audio/Player/snd_littleplatformer_watersplash_Cue.snd_littleplatformer_watersplash_Cue" 1.0 (`KismetMathLibrary.RandomFloatInRange` 0.8 1.2) 0.0 null null))

(event `self.ReceiveActorEndOverlap`
  (params (OtherActor :type "Actor Object Reference"))
  (bind _asbp_player_no_hat (cast `/Game/Blueprints/Player/BP_PlayerNoHat` OtherActor)
    (:`then`
      (`/Game/Blueprints/Player/BP_PlayerNoHat.SetWaterVars` _asbp_player_no_hat false 0.0 0.0 false))
    (:`CastFailed`
      (bind _asbp_player_with_hat (cast `/Game/Blueprints/Player/BP_PlayerWithHat` OtherActor))
      (`/Game/Blueprints/Player/BP_PlayerWithHat.SetWaterVars` _asbp_player_with_hat false 0.0 0.0 false))))

(fn `UserConstructionScript`)