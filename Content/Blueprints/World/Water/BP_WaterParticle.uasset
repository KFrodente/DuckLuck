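; BP_WaterParticle is an actor that tracks vertical disturbance at one point of water, relative to its starting height.
; It stores its Z location on BeginPlay and accumulates vertical velocity from overlapping actors or through AddVelocity.
; While that velocity is non-zero, Tick only updates whether the particle sits below its base height; no movement is applied in these graphs.
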(event `self.ReceiveBeginPlay`
  (bind (_returnvalue_x _returnvalue_y _returnvalue_z) (`KismetMathLibrary.BreakVector` (`self.K2_GetActorLocation`)))
  (set `self.BaseHeight` _returnvalue_z))

(event `self.ReceiveActorBeginOverlap`
  (params (OtherActor :type "Actor Object Reference"))
  (bind (_returnvalue_x _returnvalue_y _returnvalue_z) (`KismetMathLibrary.BreakVector` (`self.GetVelocity` OtherActor)))
  (set `self.ZVelocity` (+ _returnvalue_z (`self.ZVelocity`))))

(event `self.ReceiveTick`
  (params (DeltaSeconds :type "Float (single-precision)"))
  (bind (_returnvalue_x _returnvalue_y _returnvalue_z) (`KismetMathLibrary.BreakVector` (`self.K2_GetActorLocation`)))
  (if (!= (`self.ZVelocity`) 0.0)
    (set `self.BelowSurface` (< _returnvalue_z (`self.BaseHeight`)))))

(fn `AddVelocity`
  (params (velocity :type "Float (double-precision)"))
  (set `self.ZVelocity` (+ velocity (`self.ZVelocity`))))

(fn `UserConstructionScript`)