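; World text actor that grows its text as the player approaches inside a detection sphere.
; Overlap begin starts a fast looping timer; overlap end stops it and shrinks the text to zero.
; Each tick of that timer converts the player's distance relative to the sphere radius into proximity, shaped by a power expression and multiplier.
; That value scrubs the TextSize timeline, used as a curve lookup to scale the text up to MaxSize.
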(event Custom|TextAlpha
  (bind _text_size__ (Timeline|TextSize SetNewTime)
    (:Update
      (Rendering|Components|TextRender|SetWorldSize (Variables|Default|GetText) (* (Variables|Default|GetMaxSize) _text_size__)))))

(event Collision|EventActorBeginOverlap
  (params (OtherActor :type Actor%20Object%20Reference))
  (bind _returnvalue (Utilities|Time|SetTimerbyEvent (delegate Custom|TextAlpha) 0.02 true))
  (Variables|Default|SetTextAlphaTimer _returnvalue))

(event EventBeginPlay
  (bind _returnvalue (Actor|GetActorOfClass "/Game/Blueprints/Player/BP_PlayerWithHat.BP_PlayerWithHat_C"))
  (Variables|Default|SetPlayerRef _returnvalue))

(event Collision|EventActorEndOverlap
  (params (OtherActor :type Actor%20Object%20Reference))
  (Utilities|Time|ClearandInvalidateTimerbyHandle (Variables|Default|GetTextAlphaTimer))
  (Rendering|Components|TextRender|SetWorldSize (Variables|Default|GetText) 0.0))

(fn ConstructionScript)