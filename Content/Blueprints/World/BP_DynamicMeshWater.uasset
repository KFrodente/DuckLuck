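; BP_DynamicMeshWater is a Geometry Script actor that builds a tessellated, twisted dynamic mesh from an input static mesh, presumably for water going by its name.
; The construction script copies the mesh into its DynamicMeshComponent, then applies uniform tessellation and a twist warp driven by tessellation, angle and extent variables.
; It reuses the source mesh's first material.
; All work happens at construction; the event graph is empty.
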(fn `UserConstructionScript`
  (bind _inputmesh (`self.InputMesh`))
  (bind _returnvalue (`BaseDynamicMeshComponent.GetDynamicMesh` (`self.DynamicMeshComponent`)))
  (bind _returnvalue_2 (`GeometryScriptLibrary_StaticMeshFunctions.CopyMeshFromStaticMesh` _inputmesh _returnvalue (struct) (struct) null)
    (:`Success`
      (bind _returnvalue_3 (`GeometryScriptLibrary_MeshSubdivideFunctions.ApplyUniformTessellation` _returnvalue_2 (`self.tessellation`) null))
      (`GeometryScriptLibrary_MeshDeformFunctions.ApplyTwistWarpToMesh` _returnvalue_3 (struct) (struct) (`self.Angle`) (`self.Extent`) null)
      (`PrimitiveComponent.SetMaterial` (`self.DynamicMeshComponent`) 0 (`StaticMesh.GetMaterial` _inputmesh 0)))))