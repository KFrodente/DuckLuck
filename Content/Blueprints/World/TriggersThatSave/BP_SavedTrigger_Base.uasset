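; Base Blueprint for world triggers whose triggered state persists in the game's save data.
; On BeginPlay it searches the WorldTriggers array from the Game Instance's game data for an entry matching its ID and copies that Triggered flag.
; GetSaveData returns the flag and ID, while UseSaveData restores the flag from supplied data.
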(event `self.ReceiveBeginPlay`
  (bind _savegamedata (message `/Game/Blueprints/SaveGame/BPI_SaveGame.GetGameData` (`GameplayStatics.GetGameInstance`)))
  (for _array_element (`/Game/Blueprints/SaveGame/BP_SaveGame.WorldTriggers` _savegamedata)
    (if (== (`.ID_Num_4_36532EE34CACCF60194FDD8A9423A78C` (break `/Game/Blueprints/SaveGame/S_WorldTriggerData` _array_element)) (`self.ID`))
      (set `self.Triggered` (break `/Game/Blueprints/SaveGame/S_WorldTriggerData` _array_element))
      (break))))

(fn `GetSaveData`
  (returns (Data :type "/Game/Blueprints/SaveGame/S_WorldTriggerData Structure"))
  (return (make `/Game/Blueprints/SaveGame/S_WorldTriggerData` (`self.Triggered`) (`self.ID`))))

(fn `UserConstructionScript`)

(fn `UseSaveData`
  (params (Data :type "/Game/Blueprints/SaveGame/S_WorldTriggerData Structure"))
  (set `self.Triggered` Data_Triggered_1_038EE126441EDF6EB23B57893748B104))