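; WeaponFireType is a weapon fire-type Blueprint that expects its owner to be a BP_Player.
; On BeginPlay it casts the owner to BP_Player and caches it as Parent.
; PistolFire takes a fire position and iteration but has an empty body.
; Disconnected nodes would set projectile speed from the player's BulletVelocity stat and return whether Iteration is below two, but they never run.
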(event `self.ReceiveBeginPlay`
  (bind _asbp_player (cast `/Game/Blueprints/Player/BP_Player` (`self.GetOwner`)))
  (set `self.parent` _asbp_player))

(fn `PistolFire`
  (params (FirePosition :type "Transform Structure") (Iteration :type Integer))
  (returns (FireAgain :type Boolean)))