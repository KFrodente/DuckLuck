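; Homing bullet that periodically re-aims at its HomingTarget and damages only that actor.
; After a short delay, a looping timer sets pitch toward the target, snaps yaw left or right along X and resets velocity forward.
; A kill through I_Damagable grants Dominance to the owner, reduced for the player.
; When an enemy target is dead, homing stops and EnemyCollision ignores all channels.
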(event `self.ReceiveActorBeginOverlap`
  (params (OtherActor :type "Actor Object Reference"))
  (bind _returnvalue (`self.GetOwner`))
  (if (and (!= OtherActor _returnvalue) (== OtherActor (`self.HomingTarget`)))
    (cast `/Game/Blueprints/Bullets/BP_Bullet_Base` OtherActor
      (:`CastFailed`
        (bind _asi_damagable (cast `/Game/Blueprints/Interfaces_Enums/I_Damagable` OtherActor)
          (:`then`
            (bind (_damagedealt _killedenemy _dominance) (`/Game/Blueprints/Interfaces_Enums/I_Damagable.Take Damage` _asi_damagable (`KismetMathLibrary.FTrunc` (`self.PhysicalDamage`)) _returnvalue))
            (if _killedenemy
              (bind _asbp_enemy_base (cast `/Game/Blueprints/Enemies/BP_Enemy_Base` _returnvalue)
                (:`then`
                  (set `/Game/Blueprints/Enemies/BP_Enemy_Base.Dominance` (+ (`/Game/Blueprints/Enemies/BP_Enemy_Base.Dominance` _asbp_enemy_base) _dominance) _asbp_enemy_base))
                (:`CastFailed`
                  (bind _asbp_player_with_hat (cast `/Game/Blueprints/Player/BP_PlayerWithHat` _returnvalue)
                    (:`then`
                      (set `/Game/Blueprints/Player/BP_PlayerWithHat.Dominance` (+ (`/Game/Blueprints/Player/BP_PlayerWithHat.Dominance` _asbp_player_with_hat) (`KismetMathLibrary.FTrunc` (* _dominance 0.25))) _asbp_player_with_hat))
                    (:`CastFailed`
                      _)))))
            (`self.K2_DestroyActor`))
          (:`CastFailed`
            (`self.K2_DestroyActor`)))))))

(event `self.ReceiveTick`
  (params (DeltaSeconds :type "Float (single-precision)"))
  (`parent.ReceiveTick` DeltaSeconds))

(event `self.ReceiveBeginPlay`
  (`parent.ReceiveBeginPlay`)
  (`KismetSystemLibrary.K2_SetTimerDelegate` (delegate `StartHoming`) 0.2))

(event `StartHoming`
  (bind _returnvalue (`KismetSystemLibrary.K2_SetTimerDelegate` (delegate `Home`) 0.75 true))
  (set `self.HomingTimer` _returnvalue))

(event `Home`
  (bind _returnvalue (`self.K2_GetActorLocation`))
  (bind _returnvalue_2 (`self.K2_GetActorLocation` (`self.HomingTarget`)))
  (bind (_returnvalue_roll _returnvalue_pitch) (`KismetMathLibrary.BreakRotator` (`KismetMathLibrary.FindLookAtRotation` _returnvalue _returnvalue_2)))
  (`self.K2_SetActorRotation` (`KismetMathLibrary.MakeRotator` 0.0 _returnvalue_pitch (select `bool` (> (.x _returnvalue) (.x _returnvalue_2)) :`true` 180.0 :!type "Float (single-precision)")))
  (`/Engine/EditorBlueprintResources/StandardMacros.IsValid` self
    (:`Is Valid`
      (set `MovementComponent.Velocity` (* (`self.GetActorForwardVector`) (`self.StartVelocity`)) (`self.ProjectileMovement`))
      (bind _asbp_enemy_base (cast `/Game/Blueprints/Enemies/BP_Enemy_Base` (`self.HomingTarget`)))
      (if (`/Game/Blueprints/Components/BPC_Health.isDead` (`/Game/Blueprints/Enemies/BP_Enemy_Base.BPC_Health` _asbp_enemy_base))
        (`KismetSystemLibrary.K2_ClearAndInvalidateTimerHandle` (`self.HomingTimer`))
        (`PrimitiveComponent.SetCollisionResponseToAllChannels` (`self.EnemyCollision`) "ECR_Ignore")))))

(fn `UserConstructionScript`
  (`parent.UserConstructionScript`))