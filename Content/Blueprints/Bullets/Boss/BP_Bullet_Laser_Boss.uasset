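; Boss laser projectile that shows a beam, then fires a hit-scan shot at the player after a short delay.
; On BeginPlay a line trace against static objects sets the beam's end, and actor scale sets its width.
; After the delay it spawns the laser Niagara effect and sphere-traces along the beam once.
; A non-invincible player hit is passed to the parent's overlap handler, while normal overlaps do nothing.
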(event `self.ReceiveTick`
  (params (DeltaSeconds :type "Float (single-precision)"))
  (`parent.ReceiveTick` DeltaSeconds))

(event `self.ReceiveActorBeginOverlap`
  (params (OtherActor :type "Actor Object Reference")))

(event `self.ReceiveBeginPlay`
  (bind _returnvalue (`self.K2_GetActorLocation`))
  (bind _returnvalue_x (`KismetMathLibrary.BreakVector` (`self.GetActorScale3D`)))
  (bind _niagara (`self.Niagara`))
  (bind _returnvalue_2 (* _returnvalue_x 50.0))
  (bind _returnvalue_3 (+ _returnvalue (* (`self.GetActorForwardVector`) 10000.0)))
  (`parent.ReceiveBeginPlay`)
  (bind (_outhit _returnvalue_4) (`KismetSystemLibrary.LineTraceSingleForObjects` _returnvalue _returnvalue_3 (`self.StaticCheck`)))
  (bind _returnvalue_5 (select `bool` _returnvalue_4 :`false` _returnvalue_3 :`true` (`.Location` (`GameplayStatics.BreakHitResult` _outhit))))
  (`FXSystemComponent.SetVectorParameter` _niagara "EndOfBeam" _returnvalue_5)
  (`FXSystemComponent.SetFloatParameter` _niagara "BeamSize" _returnvalue_2)
  (`KismetSystemLibrary.Delay` 0.7)
  (set `self.CurrentWidth` _returnvalue_x)
  (bind _returnvalue_6 (`NiagaraFunctionLibrary.SpawnSystemAtLocation` "/Game/Particles/Boss/NS_LaserBeamBoss.NS_LaserBeamBoss" (`self.K2_GetActorLocation`)))
  (`FXSystemComponent.SetVectorParameter` _returnvalue_6 "EndOfBeam" _returnvalue_5)
  (`FXSystemComponent.SetFloatParameter` _returnvalue_6 "BeamSize" _returnvalue_2)
  (bind _outhit_2 (`KismetSystemLibrary.SphereTraceSingleForObjects` (`self.K2_GetActorLocation`) _returnvalue_5 (* _returnvalue_2 0.4) (`self.EnemyCheck`)))
  (bind (_bblockinghit _binitialoverlap _time _distance _location _impactpoint _normal _impactnormal _physmat _hitactor) (`GameplayStatics.BreakHitResult` _outhit_2))
  (bind _asbp_player_with_hat (cast `/Game/Blueprints/Player/BP_PlayerWithHat` _hitactor))
  (if (not (`/Game/Blueprints/Player/BP_PlayerWithHat.Invincible` _asbp_player_with_hat))
    (`parent.ReceiveActorBeginOverlap` _hitactor)))

(fn `UserConstructionScript`
  (`parent.UserConstructionScript`))