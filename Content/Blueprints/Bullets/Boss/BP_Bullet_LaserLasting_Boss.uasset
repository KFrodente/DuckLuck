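; Boss bullet that fires a lasting laser beam, shown as a warning beam before it becomes active.
; A fast looping timer line-traces forward against static objects to update the beam end on both Niagara effects.
; After the warning delay it spawns the laser effect and repeatedly sphere-traces along the beam.
; A hit on a non-invincible player calls the parent's overlap logic, replacing the disabled actor overlap.
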(event `self.ReceiveTick`
  (params (DeltaSeconds :type "Float (single-precision)"))
  (`parent.ReceiveTick` DeltaSeconds))

(event `self.ReceiveActorBeginOverlap`
  (params (OtherActor :type "Actor Object Reference")))

(event `self.ReceiveBeginPlay`
  (bind _returnvalue (`self.K2_GetActorLocation`))
  (bind _niagara (`self.Niagara`))
  (bind _returnvalue_2 (+ _returnvalue (* (`self.GetActorForwardVector`) 10000.0)))
  (`parent.ReceiveBeginPlay`)
  (`self.SetLifeSpan` (`self.Lifespan`))
  (`KismetSystemLibrary.K2_SetTimerDelegate` (delegate `FindEndPoint`) 0.02 true)
  (bind (_outhit _returnvalue_3) (`KismetSystemLibrary.LineTraceSingleForObjects` _returnvalue _returnvalue_2 (`self.StaticCheck`)))
  (bind _output_get (set `self.LaserEnd` (select `bool` _returnvalue_3 :`false` _returnvalue_2 :`true` (`.Location` (`GameplayStatics.BreakHitResult` _outhit)))))
  (`FXSystemComponent.SetVectorParameter` _niagara "EndOfBeam" _output_get)
  (`FXSystemComponent.SetFloatParameter` _niagara "BeamLifetime" (`self.WarningDelay`))
  (`FXSystemComponent.SetFloatParameter` _niagara "BeamSize" (`self.Width`))
  (`KismetSystemLibrary.Delay` (`self.WarningDelay`))
  (bind _returnvalue_4 (`NiagaraFunctionLibrary.SpawnSystemAtLocation` "/Game/Particles/Boss/NS_LaserBeamLastingBoss.NS_LaserBeamLastingBoss" (`self.K2_GetActorLocation`)))
  (set `self.Laser` _returnvalue_4)
  (`FXSystemComponent.SetFloatParameter` _returnvalue_4 "BeamLifetime" (- (`self.Lifespan`) (`self.WarningDelay`)))
  (`FXSystemComponent.SetVectorParameter` _returnvalue_4 "EndOfBeam" (`self.LaserEnd`))
  (`FXSystemComponent.SetFloatParameter` _returnvalue_4 "BeamSize" (`self.Width`))
  (`KismetSystemLibrary.K2_SetTimerDelegate` (delegate `CollisionCheck`) 0.1 true))

(event `CollisionCheck`
  (bind _outhit (`KismetSystemLibrary.SphereTraceSingleForObjects` (`self.K2_GetActorLocation`) (`self.LaserEnd`) (* (`self.Width`) 0.5) (`self.EnemyCheck`)))
  (bind (_bblockinghit _binitialoverlap _time _distance _location _impactpoint _normal _impactnormal _physmat _hitactor) (`GameplayStatics.BreakHitResult` _outhit))
  (bind _asbp_player_with_hat (cast `/Game/Blueprints/Player/BP_PlayerWithHat` _hitactor))
  (if (not (`/Game/Blueprints/Player/BP_PlayerWithHat.Invincible` _asbp_player_with_hat))
    (`parent.ReceiveActorBeginOverlap` _hitactor)))

(event `FindEndPoint`
  (bind _returnvalue (`self.K2_GetActorLocation`))
  (bind _laser (`self.Laser`))
  (bind _niagara (`self.Niagara`))
  (bind _returnvalue_2 (+ _returnvalue (* (`self.GetActorForwardVector`) 10000.0)))
  (bind (_outhit _returnvalue_3) (`KismetSystemLibrary.LineTraceSingleForObjects` _returnvalue _returnvalue_2 (`self.StaticCheck`)))
  (bind _output_get (set `self.LaserEnd` (select `bool` _returnvalue_3 :`false` _returnvalue_2 :`true` (`.Location` (`GameplayStatics.BreakHitResult` _outhit)))))
  (`/Engine/EditorBlueprintResources/StandardMacros.IsValid` _laser
    (:`Is Valid`
      (`FXSystemComponent.SetVectorParameter` _laser "EndOfBeam" _output_get))
    (:`Is Not Valid`
      _))
  (`/Engine/EditorBlueprintResources/StandardMacros.IsValid` _niagara
    (:`Is Valid`
      (`FXSystemComponent.SetVectorParameter` _niagara "EndOfBeam" _output_get))))

(fn `UserConstructionScript`
  (`parent.UserConstructionScript`))