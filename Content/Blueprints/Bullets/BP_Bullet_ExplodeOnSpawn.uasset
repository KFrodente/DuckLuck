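; Bullet variant that explodes the moment it spawns, then destroys itself.
; On BeginPlay it sphere-overlaps a radius scaled from ExplosiveDamage and feeds each found actor into the parent's ActorBeginOverlap, reusing the inherited hit logic.
; It then spawns BP_Explosion with damage-scaled radius and impulse, plus the SimpleExplosion effect.
; A debug sphere briefly draws the blast radius.
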(event `self.ReceiveBeginPlay`
  (bind _returnvalue (`self.K2_GetActorLocation`))
  (bind _returnvalue_2 (`self.K2_GetActorLocation`))
  (bind _explosivedamage (`self.ExplosiveDamage`))
  (bind _returnvalue_3 (* (`self.ExplosiveDamage`) 15.0))
  (`KismetSystemLibrary.DrawDebugSphere` _returnvalue _returnvalue_3 12 (struct :`R` 1.0 :`G` 1.0 :`B` 1.0 :`A` 1.0) 1.0 2.0)
  (bind (_outactors _returnvalue_4) (`KismetSystemLibrary.SphereOverlapActors` _returnvalue _returnvalue_3 (`self.Object Types`)))
  (if _returnvalue_4
    (for _array_element _outactors
      (`parent.ReceiveActorBeginOverlap` _array_element)))
  (`|SpawnActorFromClass` "/Game/Blueprints/Bullets/BP_Explosion.BP_Explosion_C" (`KismetMathLibrary.MakeTransform` _returnvalue_2) "Undefined" "MultiplyWithRoot" null (* _explosivedamage 15.0) (* _explosivedamage 30.0) null)
  (`NiagaraFunctionLibrary.SpawnSystemAtLocation` "/Niagara/DefaultAssets/Templates/Systems/SimpleExplosion.SimpleExplosion" _returnvalue_2)
  (`self.K2_DestroyActor`))

(fn `UserConstructionScript`
  (`parent.UserConstructionScript`))