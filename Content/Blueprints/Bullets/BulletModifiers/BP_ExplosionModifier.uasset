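; BP_ExplosionModifier is a bullet modifier that gives bullets a chance to become explosive.
; DoModFunction validates the bullet and, when the activation chance check passes, adds a fraction of its physical damage to its explosive damage.
; It then flags the bullet as explosive if that damage is positive and prints the new value as on-screen debug text.
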(fn `DoModFunction`
  (params (bullet :type "/Game/Blueprints/Bullets/BP_Bullet_Base Object Reference"))
  (bind _bullet (`local.bullet`))
  (`/Engine/EditorBlueprintResources/StandardMacros.IsValid` bullet
    (:`Is Valid`
      (bind _returnvalue (`self.CheckActivationChance`))
      (if _returnvalue
        (bind _output_get (set `/Game/Blueprints/Bullets/BP_Bullet_Base.ExplosiveDamage` (+ (* (`/Game/Blueprints/Bullets/BP_Bullet_Base.PhysicalDamage` _bullet) 0.2) (`/Game/Blueprints/Bullets/BP_Bullet_Base.ExplosiveDamage` _bullet)) _bullet))
        (set `/Game/Blueprints/Bullets/BP_Bullet_Base.IsExplosive` (> _output_get 0.0) _bullet)
        (`KismetSystemLibrary.PrintString` (`KismetStringLibrary.Conv_DoubleToString` (`/Game/Blueprints/Bullets/BP_Bullet_Base.ExplosiveDamage` _bullet)) true true (struct :`R` 1.0 :`B` 0.135502 :`A` 1.0))))))

(fn `UserConstructionScript`
  (`parent.UserConstructionScript`))