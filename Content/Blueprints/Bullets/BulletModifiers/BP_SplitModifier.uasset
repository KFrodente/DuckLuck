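; BP_SplitModifier is a bullet modifier that splits a bullet into two smaller bullets.
; DoModFunction runs only for bullets at 0.75 X scale or larger that pass an activation chance check.
; BulletManager spawns a two-bullet spread of the same class with reduced physical damage, inheriting velocity, homing target and other damage types.
; The children start at the next modifier index, and the original bullet is destroyed.
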(fn `DoModFunction`
  (params (bullet :type "/Game/Blueprints/Bullets/BP_Bullet_Base Object Reference"))
  (bind (_returnvalue_location _returnvalue_rotation _returnvalue_scale) (`KismetMathLibrary.BreakTransform` (`self.GetTransform` bullet)))
  (bind _bullet (`local.bullet`))
  (bind _bullet_2 (`local.bullet`))
  (if (>= (.x _returnvalue_scale) 0.75)
    (bind _returnvalue (`self.CheckActivationChance`))
    (if _returnvalue
      (`/Engine/EditorBlueprintResources/StandardMacros.IsValid` (`local.bullet`)
        (:`Is Valid`
          (`/Game/Blueprints/Bullets/BP_BulletManager.SpawnBullet` (`self.BulletManager`) (`KismetMathLibrary.MakeTransform` _returnvalue_location _returnvalue_rotation _returnvalue_scale) (`/Game/Blueprints/Bullets/BP_Bullet_Base.StartVelocity` _bullet_2) (* (`/Game/Blueprints/Bullets/BP_Bullet_Base.PhysicalDamage` _bullet_2) 0.75) 0 2 0.0 20.0 -0.3 0.0 0.0 (+ (`/Game/Blueprints/Bullets/BP_Bullet_Base.modIndex` _bullet) 1) true 0 (`self.GetOwner` _bullet) (`GameplayStatics.GetObjectClass` _bullet) (`/Game/Blueprints/Bullets/BP_Bullet_Base.HomingTarget` _bullet) (`/Game/Blueprints/Bullets/BP_Bullet_Base.FireDamage` _bullet) (`/Game/Blueprints/Bullets/BP_Bullet_Base.ExplosiveDamage` _bullet) (`/Game/Blueprints/Bullets/BP_Bullet_Base.WaterDamage` _bullet) (`/Game/Blueprints/Bullets/BP_Bullet_Base.LightDamage` _bullet) (`/Game/Blueprints/Bullets/BP_Bullet_Base.HealingDamage` _bullet) (`/Game/Blueprints/Bullets/BP_Bullet_Base.FearDamage` _bullet) (`/Game/Blueprints/Bullets/BP_Bullet_Base.AggressiveDamage` _bullet) true)
          (`self.K2_DestroyActor` (`local.bullet`))
          (return))))))

(fn `UserConstructionScript`
  (`parent.UserConstructionScript`))