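; Bullet modifier that gives a bullet a chance to grow larger and deal more physical damage.
; DoModFunction validates the bullet and rolls CheckActivationChance, then on success multiplies its PhysicalDamage and adds a fixed amount to its actor scale.
; The construction script only calls its parent.
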(fn `DoModFunction`
  (params (bullet :type "/Game/Blueprints/Bullets/BP_Bullet_Base Object Reference"))
  (`/Engine/EditorBlueprintResources/StandardMacros.IsValid` bullet
    (:`Is Valid`
      (bind _returnvalue (`self.CheckActivationChance`))
      (if _returnvalue
        (set `/Game/Blueprints/Bullets/BP_Bullet_Base.PhysicalDamage` (* (`/Game/Blueprints/Bullets/BP_Bullet_Base.PhysicalDamage` bullet) 1.5) bullet)
        (`self.SetActorScale3D` bullet (+ (`self.GetActorScale3D` bullet) 0.3))))))

(fn `UserConstructionScript`
  (`parent.UserConstructionScript`))