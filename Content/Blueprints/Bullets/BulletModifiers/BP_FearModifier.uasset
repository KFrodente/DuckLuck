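; BP_FearModifier is a bullet modifier that adds fear damage to bullets.
; When applied to a valid bullet, it rolls an activation chance and, on success, adds a fraction of the bullet's physical damage to its existing fear damage.
; It then flags the bullet as fearful if the resulting fear damage is positive.
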(fn `DoModFunction`
  (params (bullet :type "/Game/Blueprints/Bullets/BP_Bullet_Base Object Reference"))
  (bind _bullet (`local.bullet`))
  (`/Engine/EditorBlueprintResources/StandardMacros.IsValid` bullet
    (:`Is Valid`
      (bind _returnvalue (`self.CheckActivationChance`))
      (if _returnvalue
        (bind _output_get (set `/Game/Blueprints/Bullets/BP_Bullet_Base.FearDamage` (+ (* (`/Game/Blueprints/Bullets/BP_Bullet_Base.PhysicalDamage` _bullet) 0.2) (`/Game/Blueprints/Bullets/BP_Bullet_Base.FearDamage` _bullet)) _bullet))
        (set `/Game/Blueprints/Bullets/BP_Bullet_Base.IsFearful` (> _output_get 0.0) _bullet)))))

(fn `UserConstructionScript`
  (`parent.UserConstructionScript`))