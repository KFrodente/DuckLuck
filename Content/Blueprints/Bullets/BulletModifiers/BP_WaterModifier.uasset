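; BP_WaterModifier is a bullet modifier that can add water damage to a bullet.
; Its mod function validates the bullet, rolls an activation chance, then adds a fraction of physical damage to water damage and subtracts fire damage.
; Water damage is floored at zero, and the bullet's water flag is set from whether that same formula is positive.
; Fire damage itself is left unchanged.
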(fn `DoModFunction`
  (params (bullet :type "/Game/Blueprints/Bullets/BP_Bullet_Base Object Reference"))
  (bind _bullet (`local.bullet`))
  (bind _returnvalue (- (+ (* (`/Game/Blueprints/Bullets/BP_Bullet_Base.PhysicalDamage` _bullet) 0.2) (`/Game/Blueprints/Bullets/BP_Bullet_Base.WaterDamage` _bullet)) (`/Game/Blueprints/Bullets/BP_Bullet_Base.FireDamage` _bullet)))
  (bind _returnvalue_2 (> _returnvalue 0.0))
  (`/Engine/EditorBlueprintResources/StandardMacros.IsValid` bullet
    (:`Is Valid`
      (bind _returnvalue_3 (`self.CheckActivationChance`))
      (if _returnvalue_3
        (set `/Game/Blueprints/Bullets/BP_Bullet_Base.WaterDamage` (select `bool` _returnvalue_2 :`true` _returnvalue) _bullet)
        (set `/Game/Blueprints/Bullets/BP_Bullet_Base.IsWater` _returnvalue_2 _bullet)))))

(fn `UserConstructionScript`
  (`parent.UserConstructionScript`))