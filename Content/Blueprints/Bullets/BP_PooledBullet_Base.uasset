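; Base pooled projectile that toggles between active and dormant instead of spawning, dealing typed damage and status effects through I_Damagable.
; SetInUse drives visibility, tick and timers for lifetime, static-geometry sphere checks and player distance.
; As an apparent optimization, collision is enabled only near the player.
; Overlaps ignore the owner, other bullets and water areas, otherwise return it to the pool, crediting Dominance to the owner on kills.
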(event `self.ReceiveBeginPlay`
  (`self.SetInUse` false)
  (bind _asbp_player_with_hat (cast `/Game/Blueprints/Player/BP_PlayerWithHat` (`GameplayStatics.GetPlayerCharacter` 0)))
  (set `self.PlayerRef` _asbp_player_with_hat))

(event `SetInUse`
  (params (InUse :type Boolean))
  (set `self.InUse` InUse)
  (`self.SetActorHiddenInGame` (not InUse))
  (`self.SetActorTickEnabled` InUse)
  (`KismetSystemLibrary.K2_ClearAndInvalidateTimerHandle` (`self.WallCheckTimer`))
  (`KismetSystemLibrary.K2_ClearAndInvalidateTimerHandle` (`self.PlayerDistCheck`))
  (`KismetSystemLibrary.K2_ClearAndInvalidateTimerHandle` (`self.TimeToLiveTimer`))
  (if InUse
    (bind _returnvalue (`KismetSystemLibrary.K2_SetTimerDelegate` (delegate `ReturnToPool`) (`self.TimeToLive`)))
    (set `self.TimeToLiveTimer` _returnvalue)
    (bind _returnvalue_2 (`KismetSystemLibrary.K2_SetTimerDelegate` (delegate `CheckPlayerDist`) 0.1 true))
    (set `self.PlayerDistCheck` _returnvalue_2)
    (bind _returnvalue_3 (`KismetSystemLibrary.K2_SetTimerDelegate` (delegate `WallCheck`) 0.05 true))
    (set `self.WallCheckTimer` _returnvalue_3)
    (else
      (set `MovementComponent.Velocity` (0.0 0.0 0.0) (`self.ProjectileMovement`))
      (`self.SetActorEnableCollision` false))))

(event `WallCheck`
  (bind (_outactors _returnvalue) (`KismetSystemLibrary.SphereOverlapActors` (`self.K2_GetActorLocation`) (`SphereComponent.SphereRadius` (`self.Sphere`)) (`self.StaticCheck`)))
  (if _returnvalue
    (`self.SetInUse` false)))

(event `ReturnToPool`
  (`self.SetInUse` false))

(event `CheckPlayerDist`
  (`self.SetActorEnableCollision` (< (`KismetMathLibrary.Vector_Distance` (`self.K2_GetActorLocation` (`self.PlayerRef`)) (`self.K2_GetActorLocation`)) 400.0)))

(event `self.ReceiveActorBeginOverlap`
  (params (OtherActor :type "Actor Object Reference"))
  (bind _returnvalue (`self.GetOwner`))
  (if (!= OtherActor (`self.GetOwner`))
    (cast `/Game/Blueprints/Bullets/BP_Bullet_Base` OtherActor
      (:`CastFailed`
        (cast `/Game/Blueprints/Bullets/BP_PooledBullet_Base` OtherActor
          (:`CastFailed`
            (bind _asi_damagable (cast `/Game/Blueprints/Interfaces_Enums/I_Damagable` OtherActor)
              (:`then`
                (`/Game/Blueprints/Interfaces_Enums/I_Damagable.FireDamage` _asi_damagable (`self.FireDamage`))
                (`/Game/Blueprints/Interfaces_Enums/I_Damagable.ExplosiveDamage` _asi_damagable (`self.ExplosiveDamage`))
                (`/Game/Blueprints/Interfaces_Enums/I_Damagable.WaterDamage` _asi_damagable (`self.WaterDamage`))
                (`/Game/Blueprints/Interfaces_Enums/I_Damagable.LightDamage` _asi_damagable (`self.LightDamage`))
                (`/Game/Blueprints/Interfaces_Enums/I_Damagable.HealingDamage` _asi_damagable (`self.HealingDamage`))
                (if (`self.IsFearful`)
                  (`/Game/Blueprints/Interfaces_Enums/I_Damagable.FearApply` _asi_damagable (`self.FearDamage`)))
                (if (`self.IsAggressive`)
                  (`/Game/Blueprints/Interfaces_Enums/I_Damagable.AggressionApply` _asi_damagable (`self.AggressiveDamage`)))
                (bind (_damagedealt _killedenemy _dominance) (`/Game/Blueprints/Interfaces_Enums/I_Damagable.Take Damage` _asi_damagable (`KismetMathLibrary.FTrunc` (`self.PhysicalDamage`)) _returnvalue (`self.IsAge`)))
                (if _killedenemy
                  (bind _asbp_enemy_base (cast `/Game/Blueprints/Enemies/BP_Enemy_Base` _returnvalue)
                    (:`then`
                      (set `/Game/Blueprints/Enemies/BP_Enemy_Base.Dominance` (+ (`/Game/Blueprints/Enemies/BP_Enemy_Base.Dominance` _asbp_enemy_base) _dominance) _asbp_enemy_base))
                    (:`CastFailed`
                      (bind _asbp_player_with_hat (cast `/Game/Blueprints/Player/BP_PlayerWithHat` _returnvalue)
                        (:`then`
                          (set `/Game/Blueprints/Player/BP_PlayerWithHat.Dominance` (+ (`/Game/Blueprints/Player/BP_PlayerWithHat.Dominance` _asbp_player_with_hat) (`KismetMathLibrary.FFloor` (* _dominance 0.5))) _asbp_player_with_hat))
                        (:`CastFailed`
                          _)))))
                (`self.SetInUse` false))
              (:`CastFailed`
                (cast `/Game/Blueprints/World/Water/BP_WaterArea` OtherActor
                  (:`CastFailed`
                    (`self.SetInUse` false)))))))))))

(fn `GiveModList`
  (params (list :type "Array of /Game/Blueprints/Bullets/BulletModifiers/BP_Modifier_Base Object Reference") (index :type Integer))
  (set `self.ModList` list)
  (set `self.modIndex` index))

(fn `SetCollision`
  (params (Enabled :type Boolean)))

(fn `UserConstructionScript`
  (set `self.IsFire` (> (`self.FireDamage`) 0.0))
  (set `self.IsWater` (> (`self.WaterDamage`) 0.0))
  (set `self.IsLight` (> (`self.LightDamage`) 0.0))
  (set `self.IsExplosive` (> (`self.ExplosiveDamage`) 0.0))
  (set `self.IsHealing` (> (`self.HealingDamage`) 0.0)))