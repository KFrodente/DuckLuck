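; BP_SplitModifier is a bullet modifier that splits a bullet into a spread of smaller ones.
; When a bullet is large enough and passes the activation chance check, BulletManager spawns a spread at its transform with its start velocity, half damage and reduced size, then the original is destroyed.
; Spawns are flagged as modifier-created and carry incremented mod index and pass count.
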(fn `DoModFunction`
  (params (bullet :type "/Game/Blueprints/Bullets/BaseBullets_Modifiers/BP_Bullet_Base Object Reference"))
  (bind (_returnvalue_location _returnvalue_rotation _returnvalue_scale) (`KismetMathLibrary.BreakTransform` (`self.GetTransform` bullet)))
  (if (>= (.x _returnvalue_scale) 0.75)
    (bind _returnvalue (`self.CheckActivationChance`))
    (if _returnvalue
      (`/Engine/EditorBlueprintResources/StandardMacros.IsValid` bullet
        (:`Is Valid`
          (`/Game/Blueprints/Bullets/BP_BulletManager.SpawnBullet` (`self.BulletManager`) (`KismetMathLibrary.MakeTransform` _returnvalue_location _returnvalue_rotation _returnvalue_scale) (`/Game/Blueprints/Bullets/BaseBullets_Modifiers/BP_Bullet_Base.StartVelocity` bullet) (* (`/Game/Blueprints/Bullets/BaseBullets_Modifiers/BP_Bullet_Base.ProjectileDamage` bullet) 0.5) 0 (`self.BulletsPerSpread`) (`self.SpreadAngle`) -0.3 0.0 0.0 (+ (`Bullet.modIndex` bullet) 1) true (+ (`/Game/Blueprints/Bullets/BaseBullets_Modifiers/BP_Bullet_Base.CurrentTimesThrough` bullet) 1))
          (`self.K2_DestroyActor` bullet))))))

(fn `UserConstructionScript`
  (`parent.UserConstructionScript`))