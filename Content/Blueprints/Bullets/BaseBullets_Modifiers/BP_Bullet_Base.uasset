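; Base bullet actor that damages actors implementing I_PlayerDamagable on hit, then destroys itself, and runs a list of modifiers on itself.
; GiveModList supplies the list and starting index, and CheckCurrentMod recursively applies each valid modifier's DoModFunction in order.
; A modifier that uses an activation time pauses the chain until a Tick countdown expires, then fires and lets the sequence continue.
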(event `self.ReceiveTick`
  (params (DeltaSeconds :type "Float (single-precision)"))
  (if (`self.DoTimer`)
    (bind _output_get (set `self.CurrentTimer` (- (`self.CurrentTimer`) DeltaSeconds)))
    (if (<= _output_get 0.0)
      (`self.CheckCurrentMod`))))

(event `self.ReceiveHit`
  (params (MyComp :type "PrimitiveComponent Object Reference") (Other :type "Actor Object Reference") (OtherComp :type "PrimitiveComponent Object Reference") (bSelfMoved :type Boolean) (HitLocation :type "Vector Structure") (HitNormal :type "Vector Structure") (NormalImpulse :type "Vector Structure") (Hit :type "HitResult Structure (by ref)"))
  (cast `/Game/Blueprints/Interfaces_Enums/I_PlayerDamagable` Other)
  (`GameplayStatics.ApplyDamage` Other (`self.ProjectileDamage`))
  (`self.K2_DestroyActor`))

(fn `CheckCurrentMod`
  (bind _output (`|GetArrayItem` (`self.ModList`) (`self.modIndex`)))
  (if (`KismetSystemLibrary.IsValid` (`|GetArrayItem` (`self.ModList`) (`self.modIndex`)))
    (if (`Modifier.usesActivationTime` _output)
      (if (`self.DoTimer`)
        (set `self.DoTimer` false)
        (`/Game/Blueprints/Bullets/BaseBullets_Modifiers/BP_Modifier_Base.DoModFunction` _output self :!label _label)
        (`KismetSystemLibrary.PrintString` (`KismetStringLibrary.Conv_DoubleToString` (`self.multiplier`)))
        (bind _result (`/Engine/EditorBlueprintResources/StandardMacros.IncrementInt` (`self.modIndex`))
          (:`  `
            (if (not (> _result (`KismetArrayLibrary.Array_Length` (`self.ModList`))))
              (`self.CheckCurrentMod`))))
        (else
          (set `self.CurrentTimer` (`Modifier.activationTime` _output))
          (set `self.DoTimer` true)))
      (else
        (goto _label)))))

(fn `GiveModList`
  (params (list :type "Array of /Game/Blueprints/Bullets/BaseBullets_Modifiers/BP_Modifier_Base Object Reference") (index :type Integer))
  (set `self.ModList` list)
  (set `self.modIndex` index))

(fn `UserConstructionScript`)