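; BP_BulletManager spawns the projectiles for the main bullet and applies bullet stats to each one.
; SpawnBullet, its only active logic, spawns a copy of MainBullet's class at SpawnTransform when MainBullet is valid, launching it along that transform's forward axis at the given speed.
; Damage is BulletStats' total scaled by DamageMultiplier, with zero treated as unscaled, and BulletStats.CheckForElement sets whether the shot applies its element.
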(fn `SpawnBullet`
  (params (SpawnTransform :type "Transform Structure") (Velocity :type "Float (double-precision)") (DamageMultiplier :type "Float (double-precision)"))
  (bind _mainbullet (`self.MainBullet`))
  (bind _totaldamage (`BulletStats.totalDamage` (`self.BulletStats`)))
  (`/Engine/EditorBlueprintResources/StandardMacros.IsValid` _mainbullet
    (:`Is Valid`
      (bind _returnvalue (`|SpawnActorFromClass` (`GameplayStatics.GetObjectClass` _mainbullet) (`KismetMathLibrary.MakeTransform` SpawnTransform_Location SpawnTransform_Rotation SpawnTransform_Scale) "Undefined" "MultiplyWithRoot" null null))
      (set `MovementComponent.Velocity` (* (`KismetMathLibrary.Conv_RotatorToVector` SpawnTransform_Rotation) Velocity) (`/Game/Blueprints/Bullets/BP_Bullet_Base.ProjectileMovement` _returnvalue))
      (if (== DamageMultiplier 0.0)
        (set `/Game/Blueprints/Bullets/BP_Bullet_Base.ProjectileDamage` _totaldamage _returnvalue)
        (else
          (set `/Game/Blueprints/Bullets/BP_Bullet_Base.ProjectileDamage` (* _totaldamage DamageMultiplier) _returnvalue)))
      (set `/Game/Blueprints/Bullets/BP_Bullet_Base.WillDoElement` (`BulletStats.CheckForElement` (`self.BulletStats`)) _returnvalue))))

(fn `UserConstructionScript`)