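; Boss laser projectile that fires an instant beam along its forward vector after a short delay.
; On BeginPlay a line trace finds the beam's end point, which feeds the Niagara component along with a width taken from actor scale.
; After the delay it spawns the laser beam effect and sphere-traces the same path, with debug drawing left on.
; Each traced actor is passed to the parent's overlap handler, reusing inherited hit logic.
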(event `self.ReceiveTick`
  (params (DeltaSeconds :type "Float (single-precision)"))
  (`parent.ReceiveTick` DeltaSeconds))

(event `self.ReceiveActorBeginOverlap`
  (params (OtherActor :type "Actor Object Reference"))
  (`parent.ReceiveActorBeginOverlap` OtherActor))

(event `self.ReceiveBeginPlay`
  (bind _returnvalue (`self.K2_GetActorLocation`))
  (bind _returnvalue_x (`KismetMathLibrary.BreakVector` (`self.GetActorScale3D`)))
  (bind _niagara (`self.Niagara`))
  (bind _returnvalue_2 (* _returnvalue_x 50.0))
  (bind _returnvalue_3 (+ _returnvalue (* (`self.GetActorForwardVector`) 10000.0)))
  (`parent.ReceiveBeginPlay`)
  (bind (_outhit _returnvalue_4) (`KismetSystemLibrary.LineTraceSingleForObjects` _returnvalue _returnvalue_3 (`self.StaticCheck`)))
  (bind _returnvalue_5 (select `bool` _returnvalue_4 :`false` _returnvalue_3 :`true` (`.Location` (`GameplayStatics.BreakHitResult` _outhit))))
  (`FXSystemComponent.SetVectorParameter` _niagara "EndOfBeam" _returnvalue_5)
  (`FXSystemComponent.SetFloatParameter` _niagara "BeamSize" _returnvalue_2)
  (`KismetSystemLibrary.Delay` 0.7)
  (set `self.CurrentWidth` _returnvalue_x)
  (bind _returnvalue_6 (`NiagaraFunctionLibrary.SpawnSystemAtLocation` "/Game/Particles/NS_LaserBeam.NS_LaserBeam" (`self.K2_GetActorLocation`)))
  (`FXSystemComponent.SetVectorParameter` _returnvalue_6 "EndOfBeam" _returnvalue_5)
  (`FXSystemComponent.SetFloatParameter` _returnvalue_6 "BeamSize" _returnvalue_2)
  (bind _outhits (`KismetSystemLibrary.SphereTraceMultiForObjects` :`Start` (`self.K2_GetActorLocation`) :`End` _returnvalue_5 :`Radius` (* _returnvalue_2 0.5) :`ObjectTypes` (`self.EnemyCheck`) :`DrawDebugType` "ForDuration" :`TraceColor` (struct :`G` 1.0 :`B` 0.794348 :`A` 1.0) :`TraceHitColor` (struct :`R` 1.0 :`G` 0.598716 :`A` 1.0)))
  (for _array_element _outhits
    (`parent.ReceiveActorBeginOverlap` (`.HitActor` (`GameplayStatics.BreakHitResult` _array_element)))))

(fn `UserConstructionScript`
  (`parent.UserConstructionScript`))