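; Base projectile actor that damages I_Damagable targets and runs a chain of bullet mods.
; GiveModList supplies the list and start index; CheckCurrentMod recursively fires each mod, pausing on a Tick countdown for those with activation times.
; Overlaps ignore the owner and other bullets, otherwise destroying the bullet.
; Kills add the victim's Dominance to the owner: fully for enemies, a quarter for the player.
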(event `self.ReceiveBeginPlay`)

(event `self.ReceiveTick`
  (params (DeltaSeconds :type "Float (single-precision)"))
  (if (`self.DoTimer`)
    (bind _output_get (set `self.CurrentTimer` (- (`self.CurrentTimer`) DeltaSeconds)))
    (if (<= _output_get 0.0)
      (`self.CheckCurrentMod`))))

(event `self.ReceiveActorBeginOverlap`
  (params (OtherActor :type "Actor Object Reference"))
  (bind _returnvalue (`self.GetOwner`))
  (if (!= OtherActor _returnvalue)
    (cast `/Game/Blueprints/Bullets/BP_Bullet_Base` OtherActor
      (:`CastFailed`
        (bind _asi_damagable (cast `/Game/Blueprints/Interfaces_Enums/I_Damagable` OtherActor)
          (:`then`
            (bind (_damagedealt _killedenemy _dominance) (`/Game/Blueprints/Interfaces_Enums/I_Damagable.Take Damage` _asi_damagable (`KismetMathLibrary.FTrunc` (`self.ProjectileDamage`)) _returnvalue))
            (if _killedenemy
              (bind _asbp_enemy_base (cast `/Game/Blueprints/Enemies/BP_Enemy_Base` _returnvalue)
                (:`then`
                  (set `/Game/Blueprints/Enemies/BP_Enemy_Base.Dominance` (+ (`/Game/Blueprints/Enemies/BP_Enemy_Base.Dominance` _asbp_enemy_base) _dominance) _asbp_enemy_base))
                (:`CastFailed`
                  (bind _asbp_player_with_hat (cast `/Game/Blueprints/Player/BP_PlayerWithHat` _returnvalue)
                    (:`then`
                      (set `/Game/Blueprints/Player/BP_PlayerWithHat.Dominance` (+ (`/Game/Blueprints/Player/BP_PlayerWithHat.Dominance` _asbp_player_with_hat) (`KismetMathLibrary.FTrunc` (* _dominance 0.25))) _asbp_player_with_hat))
                    (:`CastFailed`
                      _)))))
            (`self.K2_DestroyActor`))
          (:`CastFailed`
            (`self.K2_DestroyActor`)))))))

(fn `CheckCurrentMod`
  (bind _output (`|GetArrayItem` (`self.ModList`) (`self.modIndex`)))
  (if (`KismetSystemLibrary.IsValid` (`|GetArrayItem` (`self.ModList`) (`self.modIndex`)))
    (if (`Modifier.usesActivationTime` _output)
      (if (`self.DoTimer`)
        (set `self.DoTimer` false)
        (`/Game/Blueprints/Bullets/BulletModifiers/BP_Modifier_Base.DoModFunction` _output self :!label _label)
        (bind _result (`/Engine/EditorBlueprintResources/StandardMacros.IncrementInt` (`self.modIndex`) :!label _label_2)
          (:`  `
            (if (not (> _result (`KismetArrayLibrary.Array_Length` (`self.ModList`))))
              (`self.CheckCurrentMod`)
              (return))))
        (else
          (set `self.CurrentTimer` (`Modifier.activationTime` _output))
          (set `self.DoTimer` true)))
      (else
        (goto _label)))
    (else
      (goto _label_2))))

(fn `GiveModList`
  (params (list :type "Array of /Game/Blueprints/Bullets/BulletModifiers/BP_Modifier_Base Object Reference") (index :type Integer))
  (set `self.ModList` list)
  (set `self.modIndex` index))

(fn `UserConstructionScript`)