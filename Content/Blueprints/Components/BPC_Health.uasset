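; BPC_Health is a health component whose maximum health scales with its owner's age.
; SetHealthFromAge scales MaxHealth linearly up to TotalMaxHealth at GoldenAge, rounded up, then clamps CurrentHealth or fills it on first call.
; RefillHealth restores full health, while GainHealth only writes CurrentHealth when the result exceeds MaxHealth, so smaller gains are not stored.
; BeginPlay and Tick do nothing, leaving an initial health assignment unconnected.
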(event `self.ReceiveBeginPlay`)

(fn `GainHealth`
  (params (Amount :type Integer))
  (bind _val (`/Game/BasicFunctions.+= (int)` (`self.CurrentHealth`) Amount))
  (if (> _val (`self.MaxHealth`))
    (set `self.CurrentHealth` (`self.MaxHealth`))))

(fn `RefillHealth`
  (set `self.CurrentHealth` (`self.MaxHealth`)))

(fn `SetHealthFromAge`
  (params (CurrentAge :type Integer) (GoldenAge :type Integer) (FirstTime :type Boolean))
  (bind _output_get (set `self.MaxHealth` (select `bool` (<= CurrentAge GoldenAge) :`false` (`self.TotalMaxHealth`) :`true` (`KismetMathLibrary.FCeil` (* (`self.TotalMaxHealth`) (/ CurrentAge GoldenAge))))))
  (if (> (`self.CurrentHealth`) _output_get)
    (set `self.CurrentHealth` _output_get))
  (if (`local.FirstTime`)
    (set `self.CurrentHealth` (`self.MaxHealth`))))