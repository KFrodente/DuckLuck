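; Object pool component that pre-spawns actors of a configurable class for reuse.
; After BeginPlay, a looping timer spawns inactive actors in batches of about 5% of the pool size, spreading the cost over time until the pool is full.
; SpawnFromPool linearly searches for the first unused actor, teleports it to the requested transform and marks it in use.
; An exhausted pool only prints a warning rather than growing.
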(event `self.ReceiveBeginPlay`
  (set `self.SpawnRate` (`KismetMathLibrary.FCeil` (* (`self.PoolSize`) 0.05)))
  (bind _returnvalue (`KismetSystemLibrary.K2_SetTimerDelegate` (delegate `InitializePool`) 0.1 true))
  (set `self.InitializationTimer` _returnvalue))

(event `InitializePool`
  (for _ (range (+ (`self.SpawnRate`) 1))
    (bind _returnvalue (`|SpawnActorFromClass` (`self.PooledActorClass`) (`KismetMathLibrary.MakeTransform` (0.0 0.0 0.0)) "AdjustIfPossibleButAlwaysSpawn" "MultiplyWithRoot" null 0.0 0.0 null 0.0 0.0 0.0 0.0 false false false false false false false 0.0 0.0 0.0 false 3.0 null))
    (`KismetArrayLibrary.Array_AddUnique` (`self.ObjectPool`) _returnvalue)
    (`/Game/Blueprints/Bullets/BP_PooledBullet_Base.SetInUse` _returnvalue false)
    (`/Engine/EditorBlueprintResources/StandardMacros.IncrementInt` (`self.SpawnedObjects`)))
  (if (>= (`self.SpawnedObjects`) (`self.PoolSize`))
    (`KismetSystemLibrary.K2_ClearAndInvalidateTimerHandle` (`self.InitializationTimer`))))

(fn `FindFirstAvailableActor`
  (returns (FoundActor :type "/Game/Blueprints/Bullets/BP_PooledBullet_Base Object Reference"))
  (for _array_element (`self.ObjectPool`)
    (if (not (`/Game/Blueprints/Bullets/BP_PooledBullet_Base.InUse` _array_element))
      (return _array_element))))

(fn `SpawnFromPool`
  (params (SpawnTransform :type "Transform Structure"))
  (returns (PooledActor :type "/Game/Blueprints/Bullets/BP_PooledBullet_Base Object Reference"))
  (bind _foundactor (`self.FindFirstAvailableActor`))
  (`/Engine/EditorBlueprintResources/StandardMacros.IsValid` _foundactor
    (:`Is Valid`
      (`Actor.K2_SetActorTransform` _foundactor SpawnTransform false true)
      (`/Game/Blueprints/Bullets/BP_PooledBullet_Base.SetInUse` _foundactor true)
      (return _foundactor))
    (:`Is Not Valid`
      (`KismetSystemLibrary.PrintString` "Ran out of pooled actors!"))))