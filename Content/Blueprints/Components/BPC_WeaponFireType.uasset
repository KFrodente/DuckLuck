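; Component meant to hold weapon fire-type logic for BP_PlayerWithHat, currently an unfinished stub.
; On BeginPlay it casts its owner to BP_PlayerWithHat and caches it as Parent.
; PistolFire accepts a fire position and iteration but does nothing.
; Disconnected nodes, which never run, would set projectile speed from the parent's weapon stats and return whether the iteration is below a small limit.
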(event `self.ReceiveBeginPlay`
  (bind _asbp_player_with_hat (cast `/Game/Blueprints/Player/BP_PlayerWithHat` (`self.GetOwner`)))
  (set `self.parent` _asbp_player_with_hat))

(fn `PistolFire`
  (params (FirePosition :type "Transform Structure") (Iteration :type Integer))
  (returns (FireAgain :type Boolean)))