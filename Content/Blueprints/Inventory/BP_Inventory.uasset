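; Inventory screen actor where the player equips main and sub weapons and modifiers, swapping control to a separate inventory pawn and back.
; On BeginPlay it spawns the BulletManager, modifiers and three weapons, each as an inventory display actor plus a working instance wired to shared WeaponStats.
; Entering spawns evenly spaced slot boxes.
; Slot changes update sprites, recheck stats and weapon combos, or write modifiers into the BulletManager.
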(event `self.ReceiveBeginPlay`
  (bind _returnvalue (`|SpawnActorFromClass` "/Game/Blueprints/Bullets/BP_BulletManager.BP_BulletManager_C" (`KismetMathLibrary.MakeTransform` (`self.K2_GetActorLocation`)) "Undefined" "MultiplyWithRoot" null null))
  (set `self.BulletManager` _returnvalue)
  (`self.SpawnModifiers`)
  (`self.SpawnWeapons`))

(fn `ChangeModifiers`
  (params (ModifierNum :type Integer) (BoxNum :type Integer))
  (switch `int` ModifierNum
    (:`1`
      (`KismetArrayLibrary.Array_Set` (`/Game/Blueprints/Bullets/BP_BulletManager.ModifierList` (`self.BulletManager`)) BoxNum (`self.CritMod`) true))))

(fn `ChangeWeapon`
  (params (MainWeaponNum :type Integer) (SubWeaponNum :type Integer))
  (bind _shotgun (`self.Shotgun`))
  (bind _charge (`self.Charge`))
  (bind _pistol (`self.Pistol`))
  (bind _shotgun_2 (`self.Shotgun`))
  (bind _charge_2 (`self.Charge`))
  (bind _pistol_2 (`self.Pistol`))
  (bind _rendercomponent (`PaperSpriteActor.RenderComponent` _charge_2))
  (bind _rendercomponent_2 (`PaperSpriteActor.RenderComponent` _charge))
  (bind _rendercomponent_3 (`PaperSpriteActor.RenderComponent` _shotgun_2))
  (bind _rendercomponent_4 (`PaperSpriteActor.RenderComponent` _pistol))
  (bind _rendercomponent_5 (`PaperSpriteActor.RenderComponent` _pistol_2))
  (bind _rendercomponent_6 (`PaperSpriteActor.RenderComponent` _shotgun))
  (bind _itemslot (`/Game/Blueprints/Inventory/BP_InventoryBox_Base.ItemSlot` (`|GetArrayItem` (`self.WeaponBoxes`))))
  (bind _itemslot_2 (`/Game/Blueprints/Inventory/BP_InventoryBox_Base.ItemSlot` (`|GetArrayItem` (`self.WeaponBoxes`) 1)))
  (if (and (`self.CanUseSubWeapons`) (`KismetSystemLibrary.IsValid` (`self.MainWeapon`)))
    (switch `int` SubWeaponNum
      (:`Default`
        (switch `int` MainWeaponNum :!label _label
          (:`1`
            (set `self.MainWeapon` _pistol_2)
            (`PaperSpriteComponent.SetSprite` _itemslot (`PaperSpriteComponent.GetSprite` _rendercomponent_5))
            (`PaperSpriteComponent.SetSpriteColor` _itemslot (`PaperSpriteComponent.SpriteColor` _rendercomponent_5)))
          (:`2`
            (set `self.MainWeapon` _shotgun)
            (`PaperSpriteComponent.SetSprite` _itemslot (`PaperSpriteComponent.GetSprite` _rendercomponent_6))
            (`PaperSpriteComponent.SetSpriteColor` _itemslot (`PaperSpriteComponent.SpriteColor` _rendercomponent_6)))
          (:`3`
            (set `self.MainWeapon` _charge)
            (`PaperSpriteComponent.SetSprite` _itemslot (`PaperSpriteComponent.GetSprite` _rendercomponent_2))
            (`PaperSpriteComponent.SetSpriteColor` _itemslot (`PaperSpriteComponent.SpriteColor` _rendercomponent_2))))
        (`WeaponStatsComponent.ReCheckWeaponStats` (`self.WeaponStats`) (`Weapon.m_WeaponNumber` (`self.MainWeapon`)) 0)
        (`/Engine/EditorBlueprintResources/StandardMacros.IsValid` (`self.SubWeapon`)
          (:`Is Valid`
            _)))
      (:`0`
        (goto _label))
      (:`1`
        (set `self.SubWeapon` _pistol)
        (`PaperSpriteComponent.SetSprite` _itemslot_2 (`PaperSpriteComponent.GetSprite` _rendercomponent_4))
        (`PaperSpriteComponent.SetSpriteColor` _itemslot_2 (`PaperSpriteComponent.SpriteColor` _rendercomponent_4))
        (`WeaponStatsComponent.ReCheckWeaponStats` (`self.WeaponStats`) (`Weapon.m_WeaponNumber` (`self.MainWeapon`)) (`Weapon.m_WeaponNumber` (`self.SubWeapon`)) :!label _label_2))
      (:`2`
        (set `self.SubWeapon` _shotgun_2)
        (`PaperSpriteComponent.SetSprite` _itemslot_2 (`PaperSpriteComponent.GetSprite` _rendercomponent_3))
        (`PaperSpriteComponent.SetSpriteColor` _itemslot_2 (`PaperSpriteComponent.SpriteColor` _rendercomponent_3))
        (goto _label_2))
      (:`3`
        (set `self.SubWeapon` _charge_2)
        (`PaperSpriteComponent.SetSprite` _itemslot_2 (`PaperSpriteComponent.GetSprite` _rendercomponent))
        (`PaperSpriteComponent.SetSpriteColor` _itemslot_2 (`PaperSpriteComponent.SpriteColor` _rendercomponent))
        (goto _label_2)))
    (else
      (goto _label)))
  (bind (_wascombofound _combo) (`/Game/Blueprints/Weapons/Combos/BPC_WeaponCombos.CheckForProCombo` (`self.WeaponCombos`) (`Weapon.m_WeaponNumber` (`self.MainWeapon`)) (`Weapon.m_WeaponNumber` (`self.SubWeapon`)) (`self.WeaponStats`)))
  (if _wascombofound
    (set `self.CurrentProCombo` _combo)))

(fn `DespawnPlayerAndReturn`
  (params (Player :type "/Game/Blueprints/Player/BP_PlayerForInventory Object Reference"))
  (bind _weaponboxes (`self.WeaponBoxes`))
  (bind _modifierboxes (`self.ModifierBoxes`))
  (for _array_element _weaponboxes
    (`self.K2_DestroyActor` _array_element))
  (`KismetArrayLibrary.Array_Clear` _weaponboxes)
  (for _array_element_2 _modifierboxes
    (`self.K2_DestroyActor` _array_element_2))
  (`KismetArrayLibrary.Array_Clear` _modifierboxes)
  (`self.K2_DestroyActor` Player)
  (`/Engine/EditorBlueprintResources/StandardMacros.IncrementInt` (`self.ControlPriority`)
    (:`  `
      (bind _returnvalue (`|SpawnActorFromClass` "/Game/Blueprints/Player/BP_PlayerWithHat.BP_PlayerWithHat_C" (`self.SwapTransform`) "Undefined" "MultiplyWithRoot" null null))
      (`Controller.Possess` (`GameplayStatics.GetPlayerController` 0) _returnvalue))))

(fn `SetModifierInvBoxesActive`
  (params (Active :type Boolean))
  (for _array_element (`self.ModifierBoxes`)
    (`/Game/Blueprints/Inventory/BP_InventoryBox_Base.SetSelectable` _array_element Active)))

(fn `SetWeaponInvBoxesActive`
  (params (Active :type Boolean))
  (for _array_element (`self.WeaponBoxes`)
    (`/Game/Blueprints/Inventory/BP_InventoryBox_Base.SetSelectable` _array_element Active)))

(fn `SpawnAndControlPlayer`
  (params (SwapTransform :type "Transform Structure") (Player :type "/Game/Blueprints/Player/BP_PlayerWithHat Object Reference"))
  (bind (_returnvalue_x _returnvalue_y _returnvalue_z) (`KismetMathLibrary.BreakVector` (`SceneComponent.K2_GetComponentLocation` (`self.LuckySpawn`))))
  (`self.SpawnBoxes`)
  (set `self.SwapTransform` SwapTransform)
  (`self.K2_DestroyActor` Player)
  (bind _result (`/Engine/EditorBlueprintResources/StandardMacros.IncrementInt` (`self.ControlPriority`))
    (:`  `
      (bind _returnvalue (`|SpawnActorFromClass` "/Game/Blueprints/Player/BP_PlayerForInventory.BP_PlayerForInventory_C" (`KismetMathLibrary.MakeTransform` (`KismetMathLibrary.MakeVector` _returnvalue_x _returnvalue_y (+ _returnvalue_z 1.0)) (struct :`Roll` -90.0)) "Undefined" "MultiplyWithRoot" null null))
      (set `/Game/Blueprints/Player/BP_PlayerForInventory.ControlPriority` _result _returnvalue)
      (`Controller.Possess` (`GameplayStatics.GetPlayerController` 0) _returnvalue))))

(fn `SpawnBoxes`
  (bind _mainweapon (`self.MainWeapon`))
  (bind _subweapon (`self.SubWeapon`))
  (bind (_returnvalue_x _returnvalue_y _returnvalue_z) (`KismetMathLibrary.BreakVector` (`SceneComponent.K2_GetComponentLocation` (`self.WeaponInvBoxMin`))))
  (bind _returnvalue_x_2 (`KismetMathLibrary.BreakVector` (`SceneComponent.K2_GetComponentLocation` (`self.WeaponInvBoxMax`))))
  (bind (_returnvalue_x_3 _returnvalue_y_2 _returnvalue_z_2) (`KismetMathLibrary.BreakVector` (`SceneComponent.K2_GetComponentLocation` (`self.WeaponInvBoxMin`))))
  (bind _returnvalue_x_4 (`KismetMathLibrary.BreakVector` (`SceneComponent.K2_GetComponentLocation` (`self.WeaponInvBoxMax`))))
  (bind (_returnvalue_x_5 _returnvalue_y_3 _returnvalue_z_3) (`KismetMathLibrary.BreakVector` (`SceneComponent.K2_GetComponentLocation` (`self.ModBoxMin`))))
  (bind _returnvalue_x_6 (`KismetMathLibrary.BreakVector` (`SceneComponent.K2_GetComponentLocation` (`self.ModBoxMax`))))
  (bind _returnvalue (/ (+ (`KismetMathLibrary.Abs` _returnvalue_x_3) (`KismetMathLibrary.Abs` _returnvalue_x_4)) 3.0))
  (for _index (range 1 (+ (`Inventory.ModifierSlots` (`self.Inventory`)) 1))
    (bind _returnvalue_2 (`|SpawnActorFromClass` "/Game/Blueprints/Inventory/BP_ModifierBox.BP_ModifierBox_C" (`KismetMathLibrary.MakeTransform` (`KismetMathLibrary.MakeVector` (+ _returnvalue_x_5 (* (/ (+ (`KismetMathLibrary.Abs` _returnvalue_x_5) (`KismetMathLibrary.Abs` _returnvalue_x_6)) (+ (`Inventory.ModifierSlots` (`self.Inventory`)) 1)) _index)) _returnvalue_y_3 _returnvalue_z_3) (struct :`Roll` -90.0)) "Undefined" "MultiplyWithRoot" null null))
    (set `/Game/Blueprints/Inventory/BP_ModifierBox.BoxNum` (- _index 1) _returnvalue_2)
    (`KismetArrayLibrary.Array_Add` (`self.ModifierBoxes`) _returnvalue_2))
  (if (`self.CanUseSubWeapons`)
    (bind _returnvalue_3 (`|SpawnActorFromClass` "/Game/Blueprints/Inventory/BP_MWeaponInventoryBox.BP_MWeaponInventoryBox_C" (`KismetMathLibrary.MakeTransform` (`KismetMathLibrary.MakeVector` (+ _returnvalue_x_3 _returnvalue) _returnvalue_y_2 _returnvalue_z_2) (struct :`Roll` -90.0)) "Undefined" "MultiplyWithRoot" null null))
    (`KismetArrayLibrary.Array_Add` (`self.WeaponBoxes`) _returnvalue_3)
    (bind _returnvalue_4 (`|SpawnActorFromClass` "/Game/Blueprints/Inventory/BP_SWeaponInventoryBox.BP_SWeaponInventoryBox_C" (`KismetMathLibrary.MakeTransform` (`KismetMathLibrary.MakeVector` (+ _returnvalue_x_3 (* _returnvalue 2.0)) _returnvalue_y_2 _returnvalue_z_2) (struct :`Roll` -90.0)) "Undefined" "MultiplyWithRoot" null null))
    (`KismetArrayLibrary.Array_Add` (`self.WeaponBoxes`) _returnvalue_4)
    (else
      (bind _returnvalue_5 (`|SpawnActorFromClass` "/Game/Blueprints/Inventory/BP_MWeaponInventoryBox.BP_MWeaponInventoryBox_C" (`KismetMathLibrary.MakeTransform` (`KismetMathLibrary.MakeVector` (+ _returnvalue_x (/ (+ (`KismetMathLibrary.Abs` _returnvalue_x) (`KismetMathLibrary.Abs` _returnvalue_x_2)) 2.0)) _returnvalue_y _returnvalue_z) (struct :`Roll` -90.0)) "Undefined" "MultiplyWithRoot" null null))
      (`KismetArrayLibrary.Array_Add` (`self.WeaponBoxes`) _returnvalue_5)))
  (`/Engine/EditorBlueprintResources/StandardMacros.IsValid` _mainweapon
    (:`Is Valid`
      (`/Engine/EditorBlueprintResources/StandardMacros.IsValid` _subweapon
        (:`Is Valid`
          (`self.ChangeWeapon` 0 (`Weapon.m_WeaponNumber` _subweapon)))
        (:`Is Not Valid`
          _))
      (`self.ChangeWeapon` (`Weapon.m_WeaponNumber` _mainweapon)))))

(fn `SpawnModifiers`
  (bind _returnvalue_location (`KismetMathLibrary.BreakTransform` (`SceneComponent.K2_GetComponentToWorld` (`self.NormalModifierSpawn`))))
  (`|SpawnActorFromClass` "/Game/Blueprints/Inventory/BulletThings/BP_InvCritModifier.BP_InvCritModifier_C" (`KismetMathLibrary.MakeTransform` _returnvalue_location (struct :`Roll` -90.0)) "Undefined" "MultiplyWithRoot" null null)
  (bind _returnvalue (`|SpawnActorFromClass` "/Game/Blueprints/Bullets/BaseBullets_Modifiers/BP_CritModifier.BP_CritModifier_C" (`KismetMathLibrary.MakeTransform` (0.0 5000.0 0.0)) "Undefined" "MultiplyWithRoot" null null))
  (bind _output_get (set `self.CritMod` _returnvalue))
  (`Modifier.SetChanceAndTime` _output_get))

(fn `SpawnWeapons`
  (bind _weaponstats (`self.WeaponStats`))
  (bind _pistol (`self.Pistol`))
  (bind _weaponstats_2 (`self.WeaponStats`))
  (bind _charge (`self.Charge`))
  (bind _shotgun (`self.Shotgun`))
  (bind _weaponstats_3 (`self.WeaponStats`))
  (bind _returnvalue_location (`KismetMathLibrary.BreakTransform` (`SceneComponent.K2_GetComponentToWorld` (`self.PistolSpawn`))))
  (bind _returnvalue_location_2 (`KismetMathLibrary.BreakTransform` (`SceneComponent.K2_GetComponentToWorld` (`self.ChargeSpawn`))))
  (bind _returnvalue_location_3 (`KismetMathLibrary.BreakTransform` (`SceneComponent.K2_GetComponentToWorld` (`self.ShotgunSpawn`))))
  (`|SpawnActorFromClass` "/Game/Blueprints/Inventory/WeaponThings/BP_InvPistol.BP_InvPistol_C" (`KismetMathLibrary.MakeTransform` _returnvalue_location (struct :`Roll` -90.0)) "Undefined" "MultiplyWithRoot" null null)
  (bind _returnvalue (`|SpawnActorFromClass` "/Game/Blueprints/Weapons/BaseWeapons/BP_Pistol.BP_Pistol_C" (`KismetMathLibrary.MakeTransform` (0.0 6000.0 0.0)) "Undefined" "MultiplyWithRoot" null null))
  (set `self.Pistol` _returnvalue)
  (`WeaponStatsComponent.SetPistolStats` _weaponstats)
  (set `/Game/Blueprints/Weapons/BaseWeapons/BP_WeaponParent.WeaponStats` _weaponstats _pistol)
  (set `/Game/Blueprints/Weapons/BaseWeapons/BP_WeaponParent.BulletManager` (`self.BulletManager`) _pistol)
  (`|SpawnActorFromClass` "/Game/Blueprints/Inventory/WeaponThings/BP_InvShotgun.BP_InvShotgun_C" (`KismetMathLibrary.MakeTransform` _returnvalue_location_3 (struct :`Roll` -90.0)) "Undefined" "MultiplyWithRoot" null null)
  (bind _returnvalue_2 (`|SpawnActorFromClass` "/Game/Blueprints/Weapons/BaseWeapons/BP_Shotgun.BP_Shotgun_C" (`KismetMathLibrary.MakeTransform` (0.0 6020.0 0.0)) "Undefined" "MultiplyWithRoot" null null))
  (set `self.Shotgun` _returnvalue_2)
  (`WeaponStatsComponent.SetShotgunStats` _weaponstats_3)
  (set `/Game/Blueprints/Weapons/BaseWeapons/BP_WeaponParent.WeaponStats` _weaponstats_3 _shotgun)
  (set `/Game/Blueprints/Weapons/BaseWeapons/BP_WeaponParent.BulletManager` (`self.BulletManager`) _shotgun)
  (`|SpawnActorFromClass` "/Game/Blueprints/Inventory/WeaponThings/BP_InvCharge.BP_InvCharge_C" (`KismetMathLibrary.MakeTransform` _returnvalue_location_2 (struct :`Roll` -90.0)) "Undefined" "MultiplyWithRoot" null null)
  (bind _returnvalue_3 (`|SpawnActorFromClass` "/Game/Blueprints/Weapons/BaseWeapons/BP_Charge.BP_Charge_C" (`KismetMathLibrary.MakeTransform` (0.0 6040.0 0.0)) "Undefined" "MultiplyWithRoot" null null))
  (set `self.Charge` _returnvalue_3)
  (`WeaponStatsComponent.SetChargeStats` _weaponstats_2)
  (set `/Game/Blueprints/Weapons/BaseWeapons/BP_WeaponParent.WeaponStats` _weaponstats_2 _charge)
  (set `/Game/Blueprints/Weapons/BaseWeapons/BP_WeaponParent.BulletManager` (`self.BulletManager`) _charge))

(fn `UserConstructionScript`
  (bind _weaponstats (`self.WeaponStats`))
  (`WeaponStatsComponent.SetStatComponents` _weaponstats (`self.PistolVariables`) (`self.ShotgunVariables`) (`self.ChargeVariables`))
  (`Inventory.SetVars` (`self.Inventory`) _weaponstats))