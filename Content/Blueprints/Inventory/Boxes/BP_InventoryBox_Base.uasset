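; Base inventory box actor that highlights itself as selectable while a BP_PlayerForInventory actor overlaps it.
; Tick polls the overlaps and calls SetSelectable on a change, using the current sprite as the state check.
; SetSelectable swaps the Paper2D sprite between yellow and white and updates the Selectable flag.
; InteractMain and InteractRemove are empty stubs, with InteractMain returning zero.
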(event `self.ReceiveTick`
  (params (DeltaSeconds :type "Float (single-precision)"))
  (bind _returnvalue (!= (`PaperSpriteComponent.GetSprite` (`self.PaperSprite`)) "/Game/Assets/Inventory/InventoryBox_Yellow_Sprite.InventoryBox_Yellow_Sprite"))
  (if (> (`KismetArrayLibrary.Array_Length` (`self.GetOverlappingActors` "/Game/Blueprints/Player/BP_PlayerForInventory.BP_PlayerForInventory_C")) 0)
    (if _returnvalue
      (`self.SetSelectable` true))
    (elif (not _returnvalue)
      (`self.SetSelectable` false))))

(event `/Game/Blueprints/Interfaces_Enums/Interactable.InteractRemove`
  (params (Inventory :type "/Game/Blueprints/Inventory/BP_Inventory Object Reference")))

(fn `InteractMain`
  (params (Inventory :type "/Game/Blueprints/Inventory/BP_Inventory Object Reference") (ItemNumIn :type Integer))
  (returns (ItemNumberOut :type Integer))
  (return 0))

(fn `SetSelectable`
  (params (Selectable :type Boolean))
  (bind _papersprite (`self.PaperSprite`))
  (if Selectable
    (`PaperSpriteComponent.SetSprite` _papersprite "/Game/Assets/Inventory/InventoryBox_Yellow_Sprite.InventoryBox_Yellow_Sprite")
    (set `self.Selectable` true)
    (else
      (`PaperSpriteComponent.SetSprite` _papersprite "/Game/Assets/Inventory/InventoryBox_White_Sprite.InventoryBox_White_Sprite")
      (set `self.Selectable` false))))

(fn `UserConstructionScript`
  (`parent.UserConstructionScript`))