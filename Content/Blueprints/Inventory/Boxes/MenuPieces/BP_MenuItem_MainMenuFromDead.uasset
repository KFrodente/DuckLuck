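; BP_MenuItem_MainMenuFromDead is an inventory-box menu piece that, judging by its name, returns the player to the main menu after death.
; InteractMain simply opens the MainGame level by object reference, ignoring its inventory and item number inputs.
; An unreachable leftover chain would have switched possession to BP_PlayerWithHat, faded the title and turned off DevTesting.
; The EventGraph events are empty.
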(event `/Game/Blueprints/Inventory/Boxes/BP_MenuItem_Base.interact`
  (params (PlayerWithHat :type "/Game/Blueprints/Player/BP_PlayerWithHat Object Reference") (Inventory :type "/Game/Blueprints/Inventory/BP_Inventory Object Reference") (HatPowered :type Boolean)))

(fn `InteractMain`
  (params (Inventory :type "/Game/Blueprints/Inventory/BP_Inventory Object Reference") (ItemNumIn :type Integer))
  (returns (ItemNumberOut :type Integer))
  (`GameplayStatics.OpenLevelBySoftObjectPtr` "/Game/Levels/MainGame.MainGame"))

(fn `UserConstructionScript`
  (`parent.UserConstructionScript`))