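; BP_MenuItem_Sandbox is an inventory menu item that switches the game into a sandbox editor mode.
; Its InteractMain finds the BP_PlaceholdPlayer, unpauses it, removes the default input mapping context and has the player controller possess it.
; It then sets the DevTesting flag on BP_GlobalTickSystem and enables the editor on that player.
; The event graph holds only empty events.
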(event `/Game/Blueprints/Inventory/Boxes/BP_MenuItem_Base.interact`
  (params (PlayerWithHat :type "/Game/Blueprints/Player/BP_PlayerWithHat Object Reference") (Inventory :type "/Game/Blueprints/Inventory/BP_Inventory Object Reference") (HatPowered :type Boolean)))

(fn `InteractMain`
  (params (Inventory :type "/Game/Blueprints/Inventory/BP_Inventory Object Reference") (ItemNumIn :type Integer))
  (returns (ItemNumberOut :type Integer))
  (bind _returnvalue (`GameplayStatics.GetPlayerController` 0))
  (bind _returnvalue_2 (`GameplayStatics.GetActorOfClass` "/Game/Editor/Blueprints/BP_PlaceholdPlayer.BP_PlaceholdPlayer_C"))
  (`/Game/Editor/Blueprints/BP_PlaceholdPlayer.UnPause` _returnvalue_2)
  (message `EnhancedInputSubsystemInterface.RemoveMappingContext` (pcsubsystem `EnhancedInputLocalPlayerSubsystem` _returnvalue) "/Game/Blueprints/Input/Player/IMC_Default.IMC_Default" (struct))
  (`Controller.Possess` _returnvalue _returnvalue_2)
  (bind _returnvalue_3 (`GameplayStatics.GetActorOfClass` "/Game/Blueprints/Enemies/BP_GlobalTickSystem.BP_GlobalTickSystem_C"))
  (set `/Game/Blueprints/Enemies/BP_GlobalTickSystem.DevTesting` true _returnvalue_3)
  (`/Game/Editor/Blueprints/BP_PlaceholdPlayer.EnableEditor` _returnvalue_2)
  (return 0))

(fn `UserConstructionScript`
  (`parent.UserConstructionScript`))