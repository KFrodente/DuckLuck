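; Inventory menu item for the main menu that, when interacted with, hands control to the hatted player.
; InteractMain disables the editor and calls Pause on BP_PlaceholdPlayer, fades out BP_Title if present, then possesses BP_PlayerWithHat.
; It also turns off DevTesting on BP_GlobalTickSystem and calls SetHatDuckActive on the new pawn.
; All target actors are found by class at interaction time.
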(event `/Game/Blueprints/Inventory/Boxes/BP_MenuItem_Base.interact`
  (params (PlayerWithHat :type "/Game/Blueprints/Player/BP_PlayerWithHat Object Reference") (Inventory :type "/Game/Blueprints/Inventory/BP_Inventory Object Reference") (HatPowered :type Boolean)))

(fn `InteractMain`
  (params (Inventory :type "/Game/Blueprints/Inventory/BP_Inventory Object Reference") (ItemNumIn :type Integer))
  (returns (ItemNumberOut :type Integer))
  (bind _returnvalue (`GameplayStatics.GetActorOfClass` "/Game/Editor/Blueprints/BP_PlaceholdPlayer.BP_PlaceholdPlayer_C"))
  (`/Game/Editor/Blueprints/BP_PlaceholdPlayer.DisableEditor` _returnvalue)
  (`/Game/Editor/Blueprints/BP_PlaceholdPlayer.Pause` _returnvalue)
  (bind _returnvalue_2 (`GameplayStatics.GetActorOfClass` "/Game/Blueprints/Player/BP_PlayerWithHat.BP_PlayerWithHat_C"))
  (bind _returnvalue_3 (`GameplayStatics.GetActorOfClass` "/Game/Blueprints/Inventory/BP_Title.BP_Title_C"))
  (`/Engine/EditorBlueprintResources/StandardMacros.IsValid` _returnvalue_3
    (:`Is Valid`
      (`/Game/Blueprints/Inventory/BP_Title.Fade Out` _returnvalue_3))
    (:`Is Not Valid`
      _))
  (`Controller.Possess` (`GameplayStatics.GetPlayerController` 0) _returnvalue_2)
  (bind _returnvalue_4 (`GameplayStatics.GetActorOfClass` "/Game/Blueprints/Enemies/BP_GlobalTickSystem.BP_GlobalTickSystem_C"))
  (set `/Game/Blueprints/Enemies/BP_GlobalTickSystem.DevTesting` false _returnvalue_4)
  (`/Game/Blueprints/Player/BP_PlayerWithHat.SetHatDuckActive` _returnvalue_2 0.0)
  (return 0))

(fn `UserConstructionScript`
  (`parent.UserConstructionScript`))