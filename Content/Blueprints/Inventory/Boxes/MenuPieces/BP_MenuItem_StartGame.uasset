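; BP_MenuItem_StartGame is an inventory-style menu item that starts the game from the title screen.
; Its InteractMain finds the title player and title actors by class and fades both out.
; If a BP_PlayerWithHat exists, it removes the inventory input mapping context, has the player controller possess that pawn and calls SetHatDuckActive on it.
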(event `/Game/Blueprints/Interfaces_Enums/Interactable.interact`
  (params (PlayerWithHat :type "/Game/Blueprints/Player/BP_PlayerWithHat Object Reference") (Inventory :type "/Game/Blueprints/Inventory/BP_Inventory Object Reference") (HatPowered :type Boolean)))

(fn `InteractMain`
  (params (Inventory :type "/Game/Blueprints/Inventory/BP_Inventory Object Reference") (ItemNumIn :type Integer))
  (returns (ItemNumberOut :type Integer))
  (bind _returnvalue (`GameplayStatics.GetActorOfClass` "/Game/Blueprints/Player/BP_PlayerForTitle.BP_PlayerForTitle_C"))
  (`/Game/Blueprints/Player/BP_PlayerForTitle.Fade Out` _returnvalue)
  (bind _returnvalue_2 (`GameplayStatics.GetActorOfClass` "/Game/Blueprints/Inventory/BP_Title.BP_Title_C"))
  (`/Game/Blueprints/Inventory/BP_Title.Fade Out` _returnvalue_2)
  (bind _returnvalue_3 (`GameplayStatics.GetActorOfClass` "/Game/Blueprints/Player/BP_PlayerWithHat.BP_PlayerWithHat_C"))
  (`/Engine/EditorBlueprintResources/StandardMacros.IsValid` _returnvalue_3
    (:`Is Valid`
      (`EnhancedInputSubsystemInterface.RemoveMappingContext` (pcsubsystem `EnhancedInputLocalPlayerSubsystem` (`GameplayStatics.GetPlayerController` 0)) "/Game/Blueprints/Input/Inventory/IMC_Inventory.IMC_Inventory" (struct))
      (`Controller.Possess` (`GameplayStatics.GetPlayerController` 0) _returnvalue_3)
      (`/Game/Blueprints/Player/BP_PlayerWithHat.SetHatDuckActive` _returnvalue_3 2.0)
      (return 0))))

(fn `UserConstructionScript`
  (`parent.UserConstructionScript`))