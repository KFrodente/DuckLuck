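; BP_GunPartBox_Grip is an inventory box for grip gun parts, a child Blueprint that overrides the box interaction functions.
; Main interaction calls SwitchGrip on the inventory with the held item index and box number, switching rightward.
; Sub interaction calls the same function without that direction flag and passes a remove option through.
; Events and construction add no logic of their own.
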(fn `InteractMain`
  (params (Inventory :type "/Game/Blueprints/Inventory/BP_Inventory Object Reference") (ItemNumIn :type Integer))
  (returns (ItemNumberOut :type Integer))
  (`/Game/Blueprints/Inventory/BP_Inventory.SwitchGrip` Inventory (`self.HeldItemIndex`) true (`self.BoxNumber`) false)
  (return 0))

(fn `InteractSub`
  (params (Inventory :type "/Game/Blueprints/Inventory/BP_Inventory Object Reference") (Remove :type Boolean))
  (returns (ItemNumber :type Integer))
  (`/Game/Blueprints/Inventory/BP_Inventory.SwitchGrip` Inventory (`self.HeldItemIndex`) false (`self.BoxNumber`) Remove)
  (return 0))

(fn `UserConstructionScript`
  (`parent.UserConstructionScript`))