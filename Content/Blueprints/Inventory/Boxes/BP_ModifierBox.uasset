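; BP_ModifierBox is an inventory box that changes modifiers through the Inventory passed to its interactions.
; Both interactions call ChangeModifiers with the box's HeldItemIndex and BoxNumber.
; The main interaction steps to the right, while the sub interaction leaves the direction at its default and forwards the Remove flag for item removal.
; Construction only runs the parent's script.
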(fn `InteractMain`
  (params (Inventory :type "/Game/Blueprints/Inventory/BP_Inventory Object Reference") (ItemNumIn :type Integer))
  (returns (ItemNumberOut :type Integer))
  (`/Game/Blueprints/Inventory/BP_Inventory.ChangeModifiers` Inventory (`self.HeldItemIndex`) true (`self.BoxNumber`) false)
  (return 0))

(fn `InteractSub`
  (params (Inventory :type "/Game/Blueprints/Inventory/BP_Inventory Object Reference") (Remove :type Boolean))
  (returns (ItemNumber :type Integer))
  (`/Game/Blueprints/Inventory/BP_Inventory.ChangeModifiers` Inventory (`self.HeldItemIndex`) false (`self.BoxNumber`) Remove)
  (return 0))

(fn `UserConstructionScript`
  (`parent.UserConstructionScript`))