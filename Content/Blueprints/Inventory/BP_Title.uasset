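; Title screen actor that shows a Start Game and Exit Game menu and takes over the global camera.
; BeginPlay spawns both buttons at arrow markers and cross-links them as neighbours, which GetNextBox uses for directional selection and ConfirmSelected activates.
; FadeOut pops buttons and title with Niagara effects, then Tick widens a plane material radius with accelerating interpolation before destroying the actor.
; A separate Secret function opens a hidden level.
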(event `self.ReceiveBeginPlay`
  (bind _startgamebutton (`self.StartGameButton`))
  (`self.SetCameraFollow`)
  (bind _returnvalue (`|SpawnActorFromClass` "/Game/Blueprints/Inventory/Boxes/MenuPieces/BP_MenuItem_StartGame.BP_MenuItem_StartGame_C" (`SceneComponent.K2_GetComponentToWorld` (`self.StartGameArrow`)) "Undefined" "OverrideRootScale" self (struct) null))
  (set `self.StartGameButton` _returnvalue)
  (bind _returnvalue_2 (`|SpawnActorFromClass` "/Game/Blueprints/Inventory/Boxes/MenuPieces/BP_MenuItem_ExitGame.BP_MenuItem_ExitGame_C" (`SceneComponent.K2_GetComponentToWorld` (`self.ExitGameArrow`)) "Undefined" "OverrideRootScale" self (struct) null))
  (bind _output_get (set `self.ExitGameButton` _returnvalue_2))
  (set `/Game/Blueprints/Inventory/Boxes/BP_MenuItem_Base.AdjacentButtons` (make `/Game/Blueprints/Inventory/S_SurroundingButtons` _startgamebutton _startgamebutton null null) _output_get)
  (set `/Game/Blueprints/Inventory/Boxes/BP_MenuItem_Base.AdjacentButtons` (make `/Game/Blueprints/Inventory/S_SurroundingButtons` _output_get _output_get null null) _startgamebutton)
  (`/Game/Blueprints/Inventory/Boxes/BP_MenuItem_Base.SetSelected` _startgamebutton true)
  (set `self.CurrentSelection` _startgamebutton))

(event `self.ReceiveTick`
  (params (DeltaSeconds :type "Float (single-precision)"))
  (bind _returnvalue (`KismetMathLibrary.FInterpTo` (`self.RadiusDefaultValue`) 10000.0 (`GameplayStatics.GetWorldDeltaSeconds`) (`self.Interp Speed`)))
  (if (`self.FadeOut`)
    (bind _output_get (set `self.RadiusDefaultValue` _returnvalue))
    (`MeshComponent.SetScalarParameterValueOnMaterials` (`self.Plane`) "OuterRadius" _returnvalue)
    (set `self.Interp Speed` (+ (`self.Interp Speed`) 0.01))
    (if (>= _output_get 4500.0)
      (`self.K2_DestroyActor`))))

(event `Fade Out`
  (bind _title (`self.Title`))
  (bind _startgamebutton (`self.StartGameButton`))
  (bind _exitgamebutton (`self.ExitGameButton`))
  (bind (_returnvalue_location _returnvalue_rotation _returnvalue_scale) (`KismetMathLibrary.BreakTransform` (`self.GetTransform` _exitgamebutton)))
  (bind (_returnvalue_location_2 _returnvalue_rotation_2 _returnvalue_scale_2) (`KismetMathLibrary.BreakTransform` (`SceneComponent.K2_GetComponentToWorld` _title)))
  (bind (_returnvalue_location_3 _returnvalue_rotation_3 _returnvalue_scale_3) (`KismetMathLibrary.BreakTransform` (`self.GetTransform` _startgamebutton)))
  (set `self.FadeOut` true)
  (`NiagaraFunctionLibrary.SpawnSystemAtLocation` "/Game/Assets/Particles/NS_TitleScreenPop.NS_TitleScreenPop" _returnvalue_location _returnvalue_rotation _returnvalue_scale)
  (`self.K2_DestroyActor` _exitgamebutton)
  (`NiagaraFunctionLibrary.SpawnSystemAtLocation` "/Game/Assets/Particles/NS_TitleScreenPop.NS_TitleScreenPop" _returnvalue_location_3 _returnvalue_rotation_3 _returnvalue_scale_3)
  (`self.K2_DestroyActor` _startgamebutton)
  (`NiagaraFunctionLibrary.SpawnSystemAtLocation` "/Game/Assets/Particles/NS_TitleScreenPop.NS_TitleScreenPop" _returnvalue_location_2 _returnvalue_rotation_2 _returnvalue_scale_2)
  (`ActorComponent.K2_DestroyComponent` _title))

(fn `ConfirmSelected`
  (`/Game/Blueprints/Inventory/Boxes/BP_MenuItem_Base.InteractMain` (`self.CurrentSelection`) null 0))

(fn `GetNextBox`
  (params (Dir :type "Vector Structure"))
  (bind (_adjacentbuttons_up _adjacentbuttons_down) (break `/Game/Blueprints/Inventory/S_SurroundingButtons` (`/Game/Blueprints/Inventory/Boxes/BP_MenuItem_Base.AdjacentButtons` (`self.CurrentSelection`))))
  (bind (_adjacentbuttons_up_2 _adjacentbuttons_down_2 _adjacentbuttons_left _adjacentbuttons_right) (break `/Game/Blueprints/Inventory/S_SurroundingButtons` (`/Game/Blueprints/Inventory/Boxes/BP_MenuItem_Base.AdjacentButtons` (`self.CurrentSelection`))))
  (bind _returnvalue (select `int` (+ (`KismetMathLibrary.Round` (`KismetMathLibrary.SignOfFloat` Dir_Y)) 1) :`0` _adjacentbuttons_down :`1` null :`2` _adjacentbuttons_up))
  (bind _returnvalue_2 (select `int` (+ (`KismetMathLibrary.Round` (`KismetMathLibrary.SignOfFloat` Dir_X)) 1) :`0` _adjacentbuttons_left :`1` null :`2` _adjacentbuttons_right))
  (`/Engine/EditorBlueprintResources/StandardMacros.IsValid` _returnvalue_2
    (:`Is Valid`
      (`/Game/Blueprints/Inventory/Boxes/BP_MenuItem_Base.SetSelected` _returnvalue_2 true)
      (`/Game/Blueprints/Inventory/Boxes/BP_MenuItem_Base.SetSelected` (`self.CurrentSelection`) false)
      (set `self.CurrentSelection` _returnvalue_2))
    (:`Is Not Valid`
      _))
  (`/Engine/EditorBlueprintResources/StandardMacros.IsValid` _returnvalue
    (:`Is Valid`
      (`/Game/Blueprints/Inventory/Boxes/BP_MenuItem_Base.SetSelected` _returnvalue true)
      (`/Game/Blueprints/Inventory/Boxes/BP_MenuItem_Base.SetSelected` (`self.CurrentSelection`) false)
      (set `self.CurrentSelection` _returnvalue))))

(fn `Secret`
  (`GameplayStatics.OpenLevelBySoftObjectPtr` "/Game/Levels/Secret.Secret"))

(fn `SetButtonLocations`
  (`self.K2_SetActorLocation` (`self.StartGameButton`) (`SceneComponent.K2_GetComponentLocation` (`self.StartGameArrow`)) false true)
  (`self.K2_SetActorLocation` (`self.ExitGameButton`) (`SceneComponent.K2_GetComponentLocation` (`self.ExitGameArrow`)) false true))

(fn `SetCameraFollow`
  (bind _returnvalue (`GameplayStatics.GetActorOfClass` "/Game/Blueprints/World/BP_GlobalCamera.BP_GlobalCamera_C"))
  (set `/Game/Blueprints/World/BP_GlobalCamera.CurrentFollowTarget` self _returnvalue)
  (set `/Game/Blueprints/World/BP_GlobalCamera.CurrentFollowDistance` (0.0 0.0 1000.0) _returnvalue)
  (`PlayerController.SetViewTargetWithBlend` (`GameplayStatics.GetPlayerController` 0) _returnvalue 3.0 "VTBlend_Linear" 0.0 false))

(fn `UserConstructionScript`)