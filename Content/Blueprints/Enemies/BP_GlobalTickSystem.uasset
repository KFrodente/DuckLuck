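; BP_GlobalTickSystem is a shared, timer-driven substitute for Tick in the Enemies folder, built to stagger work across numbered slots.
; A looping timer at TimeBetweenTicks fires FakeTick, which broadcasts the TickCall dispatcher with the current slot number, then advances it, wrapping after MaxTickNumber.
; GetTickNumber hands out slot numbers round-robin over the same range, so callers can be spread across different fake ticks.
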(event `self.ReceiveBeginPlay`
  (`KismetSystemLibrary.K2_SetTimerDelegate` (delegate `FakeTick`) (`self.TimeBetweenTicks`) true))

(event `FakeTick`
  (bind _calledtick (`self.CalledTick`))
  (`self.TickCall` _calledtick)
  (`/Engine/EditorBlueprintResources/StandardMacros.IncrementInt` _calledtick
    (:`  `
      (if (> _calledtick (`self.MaxTickNumber`))
        (set `self.CalledTick` 0)))))

(fn `GetTickNumber`
  (returns (TickNumber :type Integer))
  (`/Engine/EditorBlueprintResources/StandardMacros.IncrementInt` (`self.NextTickNumber`)
    (:`  `
      (if (> (`self.NextTickNumber`) (`self.MaxTickNumber`))
        (set `self.NextTickNumber` 0))
      (return (`self.NextTickNumber`)))))

(fn `UserConstructionScript`)