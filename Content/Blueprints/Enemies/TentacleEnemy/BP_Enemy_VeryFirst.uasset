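; BP_Enemy_VeryFirst is a sprite-based enemy whose corpse becomes food and grants the basic gun trigger part.
; TakeDamage lowers health and calls Death at zero, though KilledEnemy always returns false.
; Death greys the sprite, switches collision to Food, increases friction and enables pickup.
; Interact unlocks the part once; Absorb also unlocks it, signals a world-trigger save, and returns remaining food with a destroy flag.
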(event `/Game/Blueprints/Interfaces_Enums/I_Damagable.Death`
  (bind _charactermovement (`self.CharacterMovement`))
  (bind _sprite (`self.Sprite`))
  (`PrimitiveComponent.SetCollisionProfileName` _sprite "Food" true)
  (`PaperFlipbookComponent.SetSpriteColor` _sprite (struct :`R` 0.267708 :`G` 0.267708 :`B` 0.267708 :`A` 1.0))
  (set `CharacterMovementComponent.BrakingFrictionFactor` 2.0 _charactermovement)
  (set `CharacterMovementComponent.BrakingFriction` 500.0 _charactermovement)
  (set `CharacterMovementComponent.GravityScale` 1.0 _charactermovement)
  (set `CharacterMovementComponent.GroundFriction` 500.0 _charactermovement)
  (`PrimitiveComponent.SetCollisionProfileName` (`self.CapsuleComponent`) "Food" true)
  (set `/Game/Blueprints/World/FoodSource.ActiveFoodSource` true (`self.FoodSource`))
  (set `self.Active` false)
  (set `self.Collectable` true)
  (set `self.CanBePickedUp` true))

(event `/Game/Blueprints/Interfaces_Enums/Interactable.interact`
  (params (PlayerWithHat :type "/Game/Blueprints/Player/BP_PlayerWithHat Object Reference") (Inventory :type "/Game/Blueprints/Inventory/BP_Inventory Object Reference") (HatPowered :type Boolean))
  (if (`self.Collectable`)
    (if (not (`self.Collected`))
      (`/Game/Blueprints/Inventory/BP_Inventory.UnlockGunPart` Inventory "/Game/Blueprints/Weapons/Gun/Triggers/BP_GunTrigger_Basic.BP_GunTrigger_Basic_C" null 2 false)
      (`GameplayStatics.PlaySound2D` "/Game/Assets/Audio/Player/snd_littleplatformer_collectpower_Cue.snd_littleplatformer_collectpower_Cue" 1.0 1.0 0.0 null null)
      (set `self.Collected` true))))

(fn `Absorb`
  (params (Inventory :type "/Game/Blueprints/Inventory/BP_Inventory Object Reference"))
  (returns (Health :type Integer) (Destroy :type Boolean))
  (`/Game/Blueprints/Inventory/BP_Inventory.UnlockGunPart` Inventory "/Game/Blueprints/Weapons/Gun/Triggers/BP_GunTrigger_Basic.BP_GunTrigger_Basic_C" null 2 false)
  (`GameplayStatics.PlaySound2D` "/Game/Assets/Audio/Player/snd_littleplatformer_collectpower_Cue.snd_littleplatformer_collectpower_Cue" 1.0 1.0 0.0 null null)
  (set `self.Collected` true)
  (message `/Game/Blueprints/SaveGame/BPI_SaveGame.SaveWorldTriggers` (`GameplayStatics.GetGameInstance`) true)
  (return (`KismetMathLibrary.FCeil` (`/Game/Blueprints/World/FoodSource.FoodRemaining` (`self.FoodSource`))) true))

(fn `InteractMain`
  (params (Inventory :type "/Game/Blueprints/Inventory/BP_Inventory Object Reference") (ItemNumIn :type Integer))
  (returns (ItemNumberOut :type Integer))
  (return 0))

(fn `InteractSub`
  (params (Inventory :type "/Game/Blueprints/Inventory/BP_Inventory Object Reference") (Remove :type Boolean))
  (returns (ItemNumber :type Integer))
  (return 0))

(fn `Take Damage`
  (params (Damage :type Integer) (DamageDealer :type "Actor Object Reference"))
  (returns (DamageDealt :type Integer) (KilledEnemy :type Boolean) (Dominance :type Integer))
  (bind _bpc_health (`self.BPC_Health`))
  (bind _output_get (set `/Game/Blueprints/Components/BPC_Health.CurrentHealth` (- (`/Game/Blueprints/Components/BPC_Health.CurrentHealth` _bpc_health) Damage) _bpc_health))
  (if (<= _output_get 0)
    (`self.Death`)
    (return (`local.Damage`) false 1)
    (else
      (return (`local.Damage`) false 0))))

(fn `UserConstructionScript`
  (`parent.UserConstructionScript`))