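; Tentacle enemy that launches overlapping Paper characters away and fires age-scaled bullets with recoil, extending a parent enemy class.
; A looping timer traces four side-view directions, braking the enemy near static geometry or freezing it if dead.
; Eating can make it dormant, heavy and able to be picked up, while hunger or damage wakes it weightless.
; Personality traits decide fight or flee, and death turns it into a food source.
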(event `self.ReceiveActorBeginOverlap`
  (params (OtherActor :type "Actor Object Reference"))
  (bind _aspaper_character (cast `PaperCharacter` OtherActor))
  (`self.LaunchCharacter` _aspaper_character (* (`KismetMathLibrary.Normal` (- (`self.K2_GetActorLocation` OtherActor) (`self.K2_GetActorLocation`))) (`self.LaunchStrength`)) true true))

(event `self.ReceiveBeginPlay`
  (`parent.ReceiveBeginPlay`)
  (set `self.MoveTimer` (`self.MoveCooldownTimer`))
  (`KismetSystemLibrary.K2_SetTimerDelegate` (delegate `FakeTick`) 0.1 true)
  (set `self.OHungerDeprecation` (`self.HungerDeprecationSpeed`)))

(event `FakeTick`
  (bind _returnvalue (`self.K2_GetActorLocation`))
  (bind _returnvalue_2 (`self.K2_GetActorLocation`))
  (bind _returnvalue_3 (`self.K2_GetActorLocation`))
  (bind _returnvalue_4 (`self.K2_GetActorLocation`))
  (bind _charactermovement (`self.CharacterMovement`))
  (bind (_outhit _returnvalue_5) (`KismetSystemLibrary.LineTraceSingleForObjects` _returnvalue_2 (+ _returnvalue_2 (`KismetMathLibrary.MakeVector` (+ (`CapsuleComponent.CapsuleRadius` (`self.CapsuleComponent`)) 2.5))) (`self.StaticCheck`)))
  (if _returnvalue_5
    (if (`/Game/Blueprints/Components/BPC_Health.isDead` (`self.BPC_Health`)) :!label _label
      (set `MovementComponent.Velocity` (0.0 0.0 0.0) _charactermovement)
      (set `CharacterMovementComponent.GravityScale` 0.0 (`self.CharacterMovement`))
      (else
        (set `MovementComponent.Velocity` (* (`MovementComponent.Velocity` _charactermovement) 0.75) _charactermovement)))
    (else
      (bind (_outhit_2 _returnvalue_6) (`KismetSystemLibrary.LineTraceSingleForObjects` _returnvalue_3 (+ _returnvalue_3 (`KismetMathLibrary.MakeVector` 0.0 0.0 (+ (`CapsuleComponent.CapsuleRadius` (`self.CapsuleComponent`)) 2.5))) (`self.StaticCheck`)))
      (if _returnvalue_6
        (goto _label)
        (else
          (bind (_outhit_3 _returnvalue_7) (`KismetSystemLibrary.LineTraceSingleForObjects` _returnvalue_4 (- _returnvalue_4 (`KismetMathLibrary.MakeVector` (+ (`CapsuleComponent.CapsuleRadius` (`self.CapsuleComponent`)) 2.5))) (`self.StaticCheck`)))
          (if _returnvalue_7
            (goto _label)
            (else
              (bind (_outhit_4 _returnvalue_8) (`KismetSystemLibrary.LineTraceSingleForObjects` _returnvalue (- _returnvalue (`KismetMathLibrary.MakeVector` 0.0 0.0 (+ (`CapsuleComponent.CapsuleRadius` (`self.CapsuleComponent`)) 2.5))) (`self.StaticCheck`)))
              (if _returnvalue_8
                (goto _label)))))))))

(event `/Game/Blueprints/Interfaces_Enums/I_Damagable.Death`
  (bind _bpc_health (`self.BPC_Health`))
  (bind _charactermovement (`self.CharacterMovement`))
  (bind _sprite (`self.Sprite`))
  (`PrimitiveComponent.SetCollisionProfileName` _sprite "Food" true)
  (`PaperFlipbookComponent.SetSpriteColor` _sprite (struct :`R` 0.267708 :`G` 0.267708 :`B` 0.267708 :`A` 1.0))
  (set `CharacterMovementComponent.BrakingFrictionFactor` 2.0 _charactermovement)
  (set `CharacterMovementComponent.BrakingFriction` 500.0 _charactermovement)
  (set `CharacterMovementComponent.GravityScale` 3.0 _charactermovement)
  (set `CharacterMovementComponent.GroundFriction` 500.0 _charactermovement)
  (`PrimitiveComponent.SetCollisionProfileName` (`self.CapsuleComponent`) "Food" true)
  (set `/Game/Blueprints/World/FoodSource.ActiveFoodSource` true (`self.FoodSource`))
  (set `self.Active` false)
  (`KismetSystemLibrary.K2_ClearAndInvalidateTimerHandle` (`self.AgeTimer`))
  (set `/Game/Blueprints/Components/BPC_Health.isDead` true _bpc_health)
  (set `/Game/Blueprints/Components/BPC_Health.CurrentHealth` 0 _bpc_health)
  (set `self.AIControllerClass` null)
  (set `self.CanBePickedUp` true)
  (`ActorComponent.K2_DestroyComponent` (`self.Beam`))
  (`ActorComponent.K2_DestroyComponent` (`self.GrapplePiece`)))

(fn `Absorb`
  (params (Inventory :type "/Game/Blueprints/Inventory/BP_Inventory Object Reference"))
  (returns (Health :type Integer) (Destroy :type Boolean))
  (bind (_health _destroy) (`parent.Absorb` Inventory))
  (return _health _destroy))

(fn `Attack`
  (params (ThingToAttack :type "Actor Object Reference") (WhereToAttack :type "Vector Structure") (BurstAmount :type Integer) (SpreadAmount :type Integer) (SpreadAngle :type "Float (double-precision)") (FoodUsage :type "Float (double-precision)") (WillReconsider :type Boolean))
  (returns (FireAgain :type Boolean) (Reconsidered :type Boolean))
  (bind _returnvalue (`self.K2_GetActorLocation`))
  (bind (_fireagain _reconsidered) (`parent.Attack` null (0.0 0.0 0.0) 0 0 0.0 FoodUsage WillReconsider))
  (if _reconsidered
    (return false true)
    (elif _fireagain
      (bind _ratio (`self.GetAgeRatio`))
      (bind _fireagain_2 (`/Game/Blueprints/Bullets/BP_BulletManager.SpawnBullet` (`self.BulletManager`) (`KismetMathLibrary.MakeTransform` (+ _returnvalue (* (`KismetMathLibrary.Normal` (- WhereToAttack _returnvalue)) 100.0)) (`KismetMathLibrary.FindLookAtRotation` _returnvalue WhereToAttack)) 450.0 (* 10.0 _ratio (`self.DamageMod`)) (`local.BurstAmount`) (`local.SpreadAmount`) 0.0 (`local.SpreadAngle`) 0.0 0.0 0.0 0 false 0 self "/Game/Blueprints/Bullets/BP_Bullet_Enemy.BP_Bullet_Enemy_C" null 0.0 0.0 0.0 0.0 0.0 0.0 0.0 true))
      (`self.LaunchCharacter` (* (`KismetMathLibrary.Normal` (- _returnvalue (`local.WhereToAttack`))) 100 SpreadAmount))
      (return _fireagain_2 false))))

(fn `CheckHunger`
  (params (FromWorldTick :type Boolean))
  (`parent.CheckHunger` FromWorldTick)
  (if (and (<= (`self.Hunger`) 0.1) (`self.Dormant`))
    (set `self.Dormant` false)
    (set `CharacterMovementComponent.GravityScale` 0.0 (`self.CharacterMovement`))
    (set `self.HungerDeprecationSpeed` (`self.OHungerDeprecation`))))

(fn `DisableCollision`
  (`parent.DisableCollision`)
  (`PrimitiveComponent.SetCollisionEnabled` (`self.Sphere`) "NoCollision")
  (`PrimitiveComponent.SetCollisionEnabled` (`self.CapsuleComponent`) "NoCollision"))

(fn `DoReactionCheck`
  (params (Type :type "/Game/Blueprints/Interfaces_Enums/E_EnemyType Enum" :default "NewEnumerator3"))
  (returns (Flee :type Boolean) (Fight :type Boolean))
  (bind _bpc_health (`self.BPC_Health`))
  (bind _returnvalue (>= (* (/ (* (`self.Intelligence`) (/ (/ (`/Game/Blueprints/Components/BPC_Health.MaxHealth` _bpc_health) (`/Game/Blueprints/Components/BPC_Health.CurrentHealth` _bpc_health)) (- 1.0 (`self.SelfPreservation`)))) (- 1.0 (`self.Aggressive`))) (- 1.0 (`self.Fear`))) (/ (* (- 1.0 (`self.Territorial`)) 4.0) (`BlueprintMapLibrary.Map_Find` (`/Game/Blueprints/Enemies/Components/BPC_Brain.Aggressors` (`self.Brain`)) (`local.Type`)))))
  (return (not _returnvalue) _returnvalue))

(fn `Eat Food`
  (params (Amount :type "Float (double-precision)"))
  (`parent.Eat Food` Amount)
  (if (>= (`self.Hunger`) 0.5)
    (set `self.Dormant` true)
    (set `self.CanBePickedUp` true)
    (set `CharacterMovementComponent.GravityScale` 5.0 (`self.CharacterMovement`))
    (set `self.PresetHungerDeprecation` true)
    (set `self.HungerDeprecationSpeed` (* (`self.OHungerDeprecation`) 0.8))))

(fn `EnableCollision`
  (`parent.EnableCollision`)
  (`PrimitiveComponent.SetCollisionEnabled` (`self.Sphere`) "QueryAndPhysics")
  (`PrimitiveComponent.SetCollisionEnabled` (`self.CapsuleComponent`) "QueryAndPhysics")
  (set `CharacterMovementComponent.GravityScale` 3.0 (`self.CharacterMovement`)))

(fn `GetAgeRatio`
  (returns (Ratio :type "Float (double-precision)"))
  (bind _age (`self.Age`))
  (bind _goldenage (`self.GoldenAge`))
  (return (select `bool` (<= _age _goldenage) :`false` 1.0 :`true` (/ _age _goldenage))))

(fn `Take Damage`
  (params (Damage :type Integer) (DamageDealer :type "Actor Object Reference") (AgeDamage :type Boolean))
  (returns (DamageDealt :type Integer) (KilledEnemy :type Boolean) (Dominance :type Integer))
  (locals (DamageFromPlayer :type Boolean))
  (bind (_damagedealt _killedenemy) (`parent.Take Damage` Damage DamageDealer AgeDamage))
  (if (not _killedenemy)
    (set `self.Dormant` false)
    (set `self.PresetHungerDeprecation` true)
    (set `self.HungerDeprecationSpeed` (`self.OHungerDeprecation`))
    (set `self.CanBePickedUp` false)
    (set `CharacterMovementComponent.GravityScale` 0.0 (`self.CharacterMovement`))))

(fn `UserConstructionScript`
  (`parent.UserConstructionScript`))