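; BP_Trait_Base is the base Blueprint for enemy traits that modify creatures.
; It declares an empty ApplyTrait hook that takes a Creature, alongside shared helper functions.
; RaiseToZero and LowerToOne clamp a by-ref value to a floor of zero or a ceiling of one and also return it.
; ChangeEvolutionChance adds an amount to the creature's ChanceToEvolve without clamping it.
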(fn `ApplyTrait`
  (params (Creature :type "/Game/Blueprints/Enemies/BP_Enemy_Base Object Reference")))

(fn `ChangeEvolutionChance`
  (params (Creature :type "/Game/Blueprints/Enemies/BP_Enemy_Base Object Reference") (Amount :type "Float (double-precision)"))
  (set `/Game/Blueprints/Enemies/BP_Enemy_Base.ChanceToEvolve` (+ (`/Game/Blueprints/Enemies/BP_Enemy_Base.ChanceToEvolve` Creature) Amount) Creature))

(fn `LowerToOne`
  (params (A :type "Float (double-precision) (by ref)"))
  (returns (Val :type "Float (double-precision)"))
  (bind _returnvalue (`KismetMathLibrary.FMin` A 1.0))
  (`|VariableSetRef` A _returnvalue)
  (return _returnvalue))

(fn `RaiseToZero`
  (params (A :type "Float (double-precision) (by ref)"))
  (returns (Val :type "Float (double-precision)"))
  (bind _returnvalue (`KismetMathLibrary.FMax` A))
  (`|VariableSetRef` A _returnvalue)
  (return _returnvalue))