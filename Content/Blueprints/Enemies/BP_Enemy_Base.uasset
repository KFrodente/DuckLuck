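; Base enemy character for creatures with randomized personality traits and a hunger drive, which become food sources when they die.
; Construction rolls each non-preset trait within its range and takes a tick slot from BP_GlobalTickSystem.
; On its slot, hunger drains until starvation deals lethal damage through TakeDamage.
; Each enemy spawns its own grid and bullet manager; Attack and CheckHunger are empty stubs here.
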(event `self.ReceiveBeginPlay`
  (add `/Game/Blueprints/Enemies/BP_GlobalTickSystem.TickCall` (`self.TickSystem`) (`|CreateDelegate` :!event `TickCall`))
  (bind _returnvalue (`|SpawnActorFromClass` "/Game/Blueprints/Grid/BP_Grid.BP_Grid_C" (`self.GetTransform`) "Undefined" "MultiplyWithRoot" null null))
  (set `self.Grid` _returnvalue)
  (bind _returnvalue_2 (`|SpawnActorFromClass` "/Game/Blueprints/Bullets/BP_BulletManager.BP_BulletManager_C" (`self.GetTransform`) "Undefined" "MultiplyWithRoot" null null))
  (set `self.BulletManager` _returnvalue_2))

(event `TickCall`
  (params (CalledTick :type Integer))
  (if (and (== CalledTick (`self.Tick`)) (`self.Active`))
    (bind _output_get (set `self.Hunger` (- (`self.Hunger`) (`self.HungerDeprecationSpeed`))))
    (if (<= _output_get -1.0)
      (`self.Take Damage` (* (`/Game/Blueprints/Components/BPC_Health.MaxHealth` (`self.BPC_Health`)) 5)))))

(event `/Game/Blueprints/Interfaces_Enums/I_Damagable.Death`
  (set `CharacterMovementComponent.GravityScale` 1.0 (`self.CharacterMovement`))
  (`PrimitiveComponent.SetCollisionObjectType` (`self.CapsuleComponent`) "ECC_GameTraceChannel4")
  (set `/Game/Blueprints/World/FoodSource.ActiveFoodSource` true (`self.FoodSource`))
  (set `self.Active` false))

(fn `AddDominance`
  (params (Amount :type Integer))
  (set `self.Dominance` (`KismetMathLibrary.Min` (`self.MaxDominance`) (+ Amount (`self.Dominance`)))))

(fn `Attack`
  (params (ThingToAttack :type "Actor Object Reference") (WhereToAttack :type "Vector Structure") (BurstAmount :type Integer) (SpreadAmount :type Integer) (SpreadAngle :type "Float (double-precision)"))
  (returns (FireAgain :type Boolean))
  (return false))

(fn `CheckHunger`
  (params (FromWorldTick :type Boolean)))

(fn `Eat Food`
  (params (Amount :type "Float (double-precision)"))
  (set `self.Hunger` (+ (`self.Hunger`) Amount)))

(fn `Take Damage`
  (params (Damage :type Integer))
  (returns (DamageDealt :type Integer) (KilledEnemy :type Boolean) (Dominance :type Integer))
  (bind _bpc_health (`self.BPC_Health`))
  (bind _output_get (set `/Game/Blueprints/Components/BPC_Health.CurrentHealth` (- (`/Game/Blueprints/Components/BPC_Health.CurrentHealth` _bpc_health) Damage) _bpc_health))
  (if (<= _output_get 0)
    (`self.Death`)
    (return Damage true 0)
    (else
      (return Damage false 0))))

(fn `UserConstructionScript`
  (bind (_fearminmax_x _fearminmax_y) (`KismetMathLibrary.BreakVector2D` (`self.FearMinMax`)))
  (bind (_intelligenceminmax_x _intelligenceminmax_y) (`KismetMathLibrary.BreakVector2D` (`self.IntelligenceMinMax`)))
  (bind (_territorialminmax_x _territorialminmax_y) (`KismetMathLibrary.BreakVector2D` (`self.TerritorialMinMax`)))
  (bind (_selfpreservationminmax_x _selfpreservationminmax_y) (`KismetMathLibrary.BreakVector2D` (`self.SelfPreservationMinMax`)))
  (bind (_hungerminmax_x _hungerminmax_y) (`KismetMathLibrary.BreakVector2D` (`self.HungerMinMax`)))
  (bind (_hungerdeprecationminmax_x _hungerdeprecationminmax_y) (`KismetMathLibrary.BreakVector2D` (`self.HungerDeprecationMinMax`)))
  (bind (_dominanceminmax_x _dominanceminmax_y) (`KismetMathLibrary.BreakVector2D` (`self.DominanceMinMax`)))
  (bind (_aggressiveminmax_x _aggressiveminmax_y) (`KismetMathLibrary.BreakVector2D` (`self.AggressiveMinMax`)))
  (bind _returnvalue (`GameplayStatics.GetActorOfClass` "/Game/Blueprints/Enemies/BP_GlobalTickSystem.BP_GlobalTickSystem_C"))
  (`/Engine/EditorBlueprintResources/StandardMacros.IsValid` _returnvalue
    (:`Is Valid`
      (bind _ticknumber (`/Game/Blueprints/Enemies/BP_GlobalTickSystem.GetTickNumber` _returnvalue))
      (set `self.Tick` _ticknumber)
      (set `self.TickSystem` _returnvalue)
      (`|ExecutionSequence`
        (:`then_0`
          (if (not (`self.PresetAggressive`))
            (set `self.Aggressive` (`KismetMathLibrary.RandomFloatInRange` _aggressiveminmax_x _aggressiveminmax_y))))
        (:`then_1`
          (if (not (`self.PresetFear`))
            (set `self.Fear` (`KismetMathLibrary.RandomFloatInRange` _fearminmax_x _fearminmax_y))))
        (:`then_2`
          (if (not (`self.PresetDominance`))
            (set `self.Dominance` (`KismetMathLibrary.RandomIntegerInRange` (`KismetMathLibrary.FTrunc` _dominanceminmax_x) (`KismetMathLibrary.FTrunc` _dominanceminmax_y)))))
        (:`then_3`
          (if (not (`self.PresetIntelligence`))
            (set `self.Intelligence` (`KismetMathLibrary.RandomFloatInRange` _intelligenceminmax_x _intelligenceminmax_y))))
        (:`then_4`
          (if (not (`self.PresetTerritorial`))
            (set `self.Territorial` (`KismetMathLibrary.RandomFloatInRange` _territorialminmax_x _territorialminmax_y))))
        (:`then_5`
          (if (not (`self.PresetSelfPreservation`))
            (set `self.SelfPreservation` (`KismetMathLibrary.RandomFloatInRange` _selfpreservationminmax_x _selfpreservationminmax_y))))
        (:`then_6`
          (if (not (`self.PresetHunger`))
            (set `self.Hunger` (`KismetMathLibrary.RandomFloatInRange` _hungerminmax_x _hungerminmax_y))))
        (:`then_7`
          (if (not (`self.PresetHungerDeprecation`))
            (set `self.HungerDeprecationSpeed` (`KismetMathLibrary.RandomFloatInRange` _hungerdeprecationminmax_x _hungerdeprecationminmax_y))))))))