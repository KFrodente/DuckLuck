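; Behavior tree task that sets an enemy's wait time from its fear and self-preservation traits.
; It reads both values from the BP_Enemy_Base pawn and multiplies their inverses into a scaled delay above a fixed minimum, so higher values in the zero-to-one range shorten the wait.
; The result goes to the WaitTime blackboard key and the task finishes successfully, but a failed cast never finishes it.
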(event `self.ReceiveExecuteAI`
  (params (OwnerController :type "AIController Object Reference") (ControlledPawn :type "Pawn Object Reference"))
  (bind _asbp_enemy_base (cast `/Game/Blueprints/Enemies/BP_Enemy_Base` ControlledPawn))
  (`BTFunctionLibrary.SetBlackboardValueAsFloat` (`self.WaitTime`) (+ (* (* 2.0 (- 1.0 (`/Game/Blueprints/Enemies/BP_Enemy_Base.Fear` _asbp_enemy_base))) (- 1.0 (`/Game/Blueprints/Enemies/BP_Enemy_Base.SelfPreservation` _asbp_enemy_base))) 0.5))
  (`self.FinishExecute` true))