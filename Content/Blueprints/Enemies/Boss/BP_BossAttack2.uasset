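; A boss attack actor that grows a sphere, then fires repeating twin bullet fans that sweep back and forth.
; On BeginPlay it caches its owning BP_Boss, spawns a BP_BulletManager and scales the sphere up on a looping timer for one second.
; A repeating shot timer then pulls two offset spreads from the boss's basic bullet pool, using a time-based sine to oscillate their angle.
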(event `self.ReceiveBeginPlay`
  (bind _asbp_boss (cast `/Game/Blueprints/Enemies/Boss/BP_Boss` (`self.GetOwner`)))
  (set `self.BossRef` _asbp_boss)
  (bind _returnvalue (`KismetSystemLibrary.K2_SetTimerDelegate` (delegate `Grow`) 0.1 true))
  (set `self.GrowTimer` _returnvalue)
  (bind _returnvalue_2 (`|SpawnActorFromClass` "/Game/Blueprints/Bullets/BP_BulletManager.BP_BulletManager_C" (`self.GetTransform`) "Undefined" "MultiplyWithRoot" null null))
  (set `self.BulletManager` _returnvalue_2)
  (`KismetSystemLibrary.K2_SetTimerDelegate` (delegate `StopGrow`) 1.0))

(event `StopGrow`
  (`KismetSystemLibrary.K2_ClearAndInvalidateTimerHandle` (`self.GrowTimer`))
  (`KismetSystemLibrary.K2_SetTimerDelegate` (delegate `ShootBullets`) (`self.TimeBetweenShots`) true))

(event `Grow`
  (bind _sphere (`self.Sphere`))
  (`SceneComponent.SetWorldScale3D` _sphere (+ (`SceneComponent.RelativeScale3D` _sphere) 0.1)))

(event `ShootBullets`
  (bind _returnvalue (`self.GetOwner`))
  (bind _returnvalue_2 (`self.GetTransform`))
  (bind _bulletmanager (`self.BulletManager`))
  (bind _anglechange (`self.AngleChange`))
  (bind _basicbulletobjectpool (`/Game/Blueprints/Enemies/Boss/BP_Boss.BasicBulletObjectPool` (`self.BossRef`)))
  (set `self.AngleChange` (+ (`self.AngleMod`) (* (`KismetMathLibrary.Sin` (* (`GameplayStatics.GetRealTimeSeconds`) 2.0)) 25.0)))
  (`/Game/Blueprints/Bullets/BP_BulletManager.SpawnBulletFromPool` _bulletmanager _returnvalue_2 1000.0 5.0 0 15 (- _anglechange 35.0) 45.0 -0.25 0.0 0.0 0 false 0 _returnvalue null 0.0 0.0 0.0 0.0 0.0 0.0 0.0 _basicbulletobjectpool)
  (`/Game/Blueprints/Bullets/BP_BulletManager.SpawnBulletFromPool` _bulletmanager _returnvalue_2 1000.0 5.0 0 15 (+ _anglechange 35.0) 45.0 -0.25 0.0 0.0 0 false 0 _returnvalue null 0.0 0.0 0.0 0.0 0.0 0.0 0.0 _basicbulletobjectpool))

(fn `UserConstructionScript`)