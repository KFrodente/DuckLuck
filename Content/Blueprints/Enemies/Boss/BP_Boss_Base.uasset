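; Base Blueprint for boss enemies, providing an on-screen health bar, a looping attack timer and three health-driven phases.
; BeginPlay creates the bar, tops up health and caches the global camera, while Death removes the bar, clears timers and blocks attacks.
; The TakeDamage override calls the parent, then CheckPhase enters phases 2 and 3 once each at health thresholds.
; AttackFromPhase and CanAttack are empty here, and the delayed attack re-enable logic is unwired.
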(event `self.ReceiveBeginPlay`
  (bind _bpc_health (`self.BPC_Health`))
  (bind _returnvalue (`|CreateWidget` "/Game/Blueprints/UI/UW_BossHealthbar.UW_BossHealthbar_C"))
  (set `self.HealthBar` _returnvalue)
  (set `/Game/Blueprints/UI/UW_BossHealthbar.BossRef` self _returnvalue)
  (`UserWidget.AddToViewport` _returnvalue 0)
  (set `/Game/Blueprints/Components/BPC_Health.MaxHealth` (`/Game/Blueprints/Components/BPC_Health.TotalMaxHealth` _bpc_health) _bpc_health)
  (`/Game/Blueprints/Components/BPC_Health.GainHealth` _bpc_health 100000)
  (bind _returnvalue_2 (`GameplayStatics.GetActorOfClass` "/Game/Blueprints/World/BP_GlobalCamera.BP_GlobalCamera_C"))
  (set `self.CameraRef` _returnvalue_2)
  (bind _returnvalue_3 (`KismetSystemLibrary.K2_SetTimerDelegate` (`|CreateDelegate` :!event `AttackFromPhase`) 1.0 true))
  (set `self.AttackTimer` _returnvalue_3))

(event `self.Death`
  (`Widget.RemoveFromParent` (`self.HealthBar`))
  (`KismetSystemLibrary.K2_ClearAndInvalidateTimerHandle` (`self.AttackTimer`))
  (`KismetSystemLibrary.K2_ClearAndInvalidateTimerHandle` (`self.AllowAttackTimer`))
  (set `self.IsAbleToAttack` false))

(event `EnterPhase1`
  (set `self.CurrentPhase` 1))

(event `AttackFromPhase`)

(event `EnterPhase2`
  (if (not (`self.Phase2Entered`))
    (set `self.Phase2Entered` true)
    (set `self.CurrentPhase` 2)))

(event `EnterPhase3`
  (if (not (`self.Phase3Entered`))
    (set `self.Phase3Entered` true)
    (set `self.CurrentPhase` 3)))

(event `CanAttack`)

(event `AllowAttacking`
  (set `self.IsAbleToAttack` true :!label _label))

(event `ResetAttackAllowance`
  (goto _label))

(fn `CheckPhase`
  (if (<= (`/Game/Blueprints/Components/BPC_Health.CurrentHealth` (`self.BPC_Health`)) (`self.Phase2Change`))
    (`self.EnterPhase2`)
    (if (<= (`/Game/Blueprints/Components/BPC_Health.CurrentHealth` (`self.BPC_Health`)) (`self.Phase3Change`))
      (`self.EnterPhase3`))))

(fn `Take Damage`
  (params (Damage :type Integer) (DamageDealer :type "Actor Object Reference") (AgeDamage :type Boolean))
  (returns (DamageDealt :type Integer) (KilledEnemy :type Boolean) (Dominance :type Integer))
  (bind (_damagedealt _killedenemy _dominance) (`parent.Take Damage` Damage DamageDealer AgeDamage))
  (`self.CheckPhase`)
  (return _damagedealt _killedenemy _dominance))

(fn `UserConstructionScript`)