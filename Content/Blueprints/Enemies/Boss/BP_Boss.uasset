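; Boss enemy that shakes the camera on BeginPlay, then enters phase 1 after a delay.
; AttackfromPhase, gated by IsAbleToAttack, draws four attacks in random order without repeats, refilling when empty.
; Attacks spawn tracked actors at arrow markers; Attack4 chains timed follow-ups.
; Phase 2 spawns a player-teleport portal and destroys active attacks, but has no attack selection here; Attack6 is uncalled.
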(event `self.ReceiveTick`
  (params (DeltaSeconds :type "Float (single-precision)"))
  (`KismetSystemLibrary.PrintString` (`KismetStringLibrary.Conv_BoolToString` (`self.IsAbleToAttack`)) true true (struct :`G` 0.66 :`B` 1.0 :`A` 1.0) 0.01))

(event `self.ReceiveBeginPlay`
  (`parent.ReceiveBeginPlay`)
  (`/Game/Blueprints/World/BP_GlobalCamera.ScreenShake` (`self.CameraRef`) 300.0 300.0 0.02 1.0)
  (`KismetSystemLibrary.Delay` 3.0)
  (`self.EnterPhase1`))

(event `self.EnterPhase1`
  (`parent.EnterPhase1`)
  (set `self.IsAbleToAttack` true))

(event `self.EnterPhase2`
  (bind _attackobjects (`self.AttackObjects`))
  (`parent.EnterPhase2`)
  (`/Engine/EditorBlueprintResources/StandardMacros.DoOnce` false
    (:`Completed`
      (`self.TeleportPlayer`)
      (`self.K2_DestroyActor` _attackobjects)
      (`KismetArrayLibrary.Array_Clear` _attackobjects))))

(event `self.AttackFromPhase`
  (if (`self.IsAbleToAttack`)
    (set `self.IsAbleToAttack` false)
    (switch `int` (`self.CurrentPhase`)
      (:`1`
        (if (== (`KismetArrayLibrary.Array_Length` (`self.PhaseAttackOrder`)) 0)
          (for _index (range 4)
            (`KismetArrayLibrary.Array_Add` (`self.PhaseAttackOrder`) _index)))
        (switch `int` (`KismetArrayLibrary.Array_Random` (`self.PhaseAttackOrder`))
          (:`0`
            (`self.Attack1`)
            (`KismetArrayLibrary.Array_RemoveItem` (`self.PhaseAttackOrder`)))
          (:`1`
            (`self.Attack2`)
            (`KismetArrayLibrary.Array_RemoveItem` (`self.PhaseAttackOrder`) 1))
          (:`2`
            (`self.Attack3`)
            (`KismetArrayLibrary.Array_RemoveItem` (`self.PhaseAttackOrder`) 2))
          (:`3`
            (`self.Attack4`)
            (`KismetArrayLibrary.Array_RemoveItem` (`self.PhaseAttackOrder`) 3)))))))

(event `/Game/Blueprints/Interfaces_Enums/I_Damagable.Death`
  (`parent.Death`))

(fn `Attack1`
  (bind _returnvalue (`|SpawnActorFromClass` "/Game/Blueprints/Enemies/Boss/BP_BossAttack1.BP_BossAttack1_C" (`SceneComponent.K2_GetComponentToWorld` (`self.Arrow1_0`)) "AlwaysSpawn" "OverrideRootScale" self 0.2 self self))
  (`KismetArrayLibrary.Array_Add` (`self.AttackObjects`) _returnvalue)
  (bind _returnvalue_2 (`|SpawnActorFromClass` "/Game/Blueprints/Enemies/Boss/BP_BossAttack1.BP_BossAttack1_C" (`SceneComponent.K2_GetComponentToWorld` (`self.Arrow2_0`)) "AlwaysSpawn" "OverrideRootScale" self 0.2 self self))
  (`KismetArrayLibrary.Array_Add` (`self.AttackObjects`) _returnvalue_2)
  (set `self.IsAbleToAttack` false))

(fn `Attack2`
  (bind _returnvalue (`|SpawnActorFromClass` "/Game/Blueprints/Enemies/Boss/BP_BossAttack2.BP_BossAttack2_C" (`SceneComponent.K2_GetComponentToWorld` (`self.Arrow3_0`)) "AlwaysSpawn" "OverrideRootScale" self 25.0 3.0 0.2 self self))
  (set `self.IsAbleToAttack` false)
  (`KismetArrayLibrary.Array_Add` (`self.AttackObjects`) _returnvalue))

(fn `Attack3`
  (bind _returnvalue (`|SpawnActorFromClass` "/Game/Blueprints/Enemies/Boss/BP_BossAttack3.BP_BossAttack3_C" (`SceneComponent.K2_GetComponentToWorld` (select `bool` (`KismetMathLibrary.RandomBool`) :`false` (`self.Arrow5_0`) :`true` (`self.Arrow4_0`) :!type "SceneComponent Object Reference")) "AlwaysSpawn" "OverrideRootScale" self 1.0 self self))
  (set `self.IsAbleToAttack` false)
  (`KismetArrayLibrary.Array_Add` (`self.AttackObjects`) _returnvalue))

(fn `Attack4`
  (bind _output_get (set `self.GoingRight` (`KismetMathLibrary.RandomBool`)))
  (bind _returnvalue (`|SpawnActorFromClass` "/Game/Blueprints/Enemies/Boss/BP_BossAttack4.BP_BossAttack4_C" (`SceneComponent.K2_GetComponentToWorld` (select `bool` _output_get :`false` (`self.Arrow6_0`) :`true` (`self.Arrow7_0`) :!type "SceneComponent Object Reference")) "AlwaysSpawn" "OverrideRootScale" self (select `bool` _output_get :`false` -100.0 :`true` 100.0) 0.05 self self))
  (`KismetSystemLibrary.K2_SetTimer` null "Attack4P2" 1.0)
  (set `self.IsAbleToAttack` false)
  (`KismetArrayLibrary.Array_Add` (`self.AttackObjects`) _returnvalue))

(fn `Attack4P2`
  (bind _output_get (set `self.GoingRight` (not (`self.GoingRight`))))
  (bind _returnvalue (`|SpawnActorFromClass` "/Game/Blueprints/Enemies/Boss/BP_BossAttack4.BP_BossAttack4_C" (`SceneComponent.K2_GetComponentToWorld` (select `bool` _output_get :`false` (`self.Arrow6_0`) :`true` (`self.Arrow7_0`) :!type "SceneComponent Object Reference")) "AlwaysSpawn" "OverrideRootScale" self (select `bool` _output_get :`false` -100.0 :`true` 100.0) 0.05 self self))
  (`KismetArrayLibrary.Array_Add` (`self.AttackObjects`) _returnvalue)
  (if (!= (`self.CurrentPhase`) 1)
    (`KismetSystemLibrary.K2_SetTimer` null "Attack4P3" 2.0)))

(fn `Attack4P3`
  (bind _returnvalue (`|SpawnActorFromClass` "/Game/Blueprints/Enemies/Boss/BP_BossAttack4_2.BP_BossAttack4_2_C" (`SceneComponent.K2_GetComponentToWorld` (select `bool` (`KismetMathLibrary.RandomBool`) :`false` (`self.Arrow9`) :`true` (`self.Arrow8`) :!type "SceneComponent Object Reference")) "AlwaysSpawn" "OverrideRootScale" self 0.0 0.2 self self))
  (`KismetArrayLibrary.Array_Add` (`self.AttackObjects`) _returnvalue))

(fn `Attack6`
  (bind _returnvalue (`|SpawnActorFromClass` "/Game/Blueprints/Enemies/Boss/BP_BossAttack6.BP_BossAttack6_C" (`SceneComponent.K2_GetComponentToWorld` (select `bool` (`KismetMathLibrary.RandomBool`) :`false` (`self.Arrow11`) :`true` (`self.Arrow10`) :!type "SceneComponent Object Reference")) "Undefined" "OverrideRootScale" self 0.2 self self))
  (set `self.IsAbleToAttack` false)
  (`KismetArrayLibrary.Array_Add` (`self.AttackObjects`) _returnvalue))

(fn `RemoveAttackFromList`
  (params (Attack :type "/Game/Blueprints/Enemies/Boss/BP_BossAttack_Base Object Reference"))
  (`KismetArrayLibrary.Array_RemoveItem` (`self.AttackObjects`) Attack))

(fn `Take Damage`
  (params (Damage :type Integer) (DamageDealer :type "Actor Object Reference") (AgeDamage :type Boolean))
  (returns (DamageDealt :type Integer) (KilledEnemy :type Boolean) (Dominance :type Integer))
  (bind (_damagedealt _killedenemy _dominance) (`parent.Take Damage` Damage DamageDealer AgeDamage))
  (return _damagedealt _killedenemy _dominance))

(fn `TeleportPlayer`
  (`|SpawnActorFromClass` "/Game/Blueprints/Enemies/Boss/BP_Boss_Portal.BP_Boss_Portal_C" (`SceneComponent.K2_GetComponentToWorld` (`self.Arrow3_0`)) "Undefined" "MultiplyWithRoot" null self self)
  (set `self.IsAbleToAttack` false))

(fn `UserConstructionScript`)