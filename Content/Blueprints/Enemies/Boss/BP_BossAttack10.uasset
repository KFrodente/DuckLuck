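; BP_BossAttack10 is a boss attack actor that charges up as a growing sprite, then fires a spinning, long-lasting laser.
; A looping timer scales the sprite up for one second, then StopGrow spawns the laser at the Arrow using the attack's width, warning delay and remaining lifespan.
; A second timer rotates the sprite and snaps the laser to the Arrow's transform.
; It also spawns a BulletManager on BeginPlay but never uses it.
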(event `self.ReceiveBeginPlay`
  (`parent.ReceiveBeginPlay`)
  (bind _returnvalue (`KismetSystemLibrary.K2_SetTimerDelegate` (delegate `Grow`) 0.1 true))
  (set `self.GrowTimer` _returnvalue)
  (bind _returnvalue_2 (`|SpawnActorFromClass` "/Game/Blueprints/Bullets/BP_BulletManager.BP_BulletManager_C" (`self.GetTransform`) "Undefined" "MultiplyWithRoot" null null))
  (set `self.BulletManager` _returnvalue_2)
  (`KismetSystemLibrary.K2_SetTimerDelegate` (delegate `StopGrow`) 1.0))

(event `StopGrow`
  (`KismetSystemLibrary.K2_ClearAndInvalidateTimerHandle` (`self.GrowTimer`))
  (bind _returnvalue (`|SpawnActorFromClass` "/Game/Blueprints/Bullets/Boss/BP_Bullet_LaserLasting_Boss.BP_Bullet_LaserLasting_Boss_C" (`SceneComponent.K2_GetComponentToWorld` (`self.Arrow`)) "Undefined" "OverrideRootScale" (`self.GetOwner`) (`self.Width`) (`self.Warning Delay`) (- (`self.Lifespan`) 1.0) 10.0 0.0 null 0.0 0.0 0.0 0.0 false false false false false false false 0.0 0.0 0.0 false false null))
  (set `self.SpawnedLaser` _returnvalue)
  (`KismetSystemLibrary.K2_SetTimerDelegate` (delegate `Rotate`) 0.05 true))

(event `Grow`
  (`SceneComponent.SetWorldScale3D` (`self.Sprite`) (+ (`SceneComponent.RelativeScale3D` (`self.Sprite`)) 0.02)))

(event `Rotate`
  (`SceneComponent.K2_AddRelativeRotation` (`self.Sprite`) (struct :`Pitch` 10.0) false false)
  (`self.K2_SetActorTransform` (`self.SpawnedLaser`) (`SceneComponent.K2_GetComponentToWorld` (`self.Arrow`)) false true))

(fn `UserConstructionScript`)