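; BP_BossAttack9 is a boss attack that grows a sphere, then repeatedly fires full-circle bullet spreads.
; On BeginPlay it spawns its own BP_BulletManager and scales the sphere up on a looping timer for two seconds.
; It then starts a looping shot timer, pulling bullets from the boss's basic object pool through the manager.
; Each volley passes an angle offset, updates a shot counter and runs angle arithmetic.
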(event `self.ReceiveBeginPlay`
  (`parent.ReceiveBeginPlay`)
  (bind _returnvalue (`KismetSystemLibrary.K2_SetTimerDelegate` (delegate `Grow`) 0.1 true))
  (set `self.GrowTimer` _returnvalue)
  (bind _returnvalue_2 (`|SpawnActorFromClass` "/Game/Blueprints/Bullets/BP_BulletManager.BP_BulletManager_C" (`self.GetTransform`) "Undefined" "MultiplyWithRoot" null null))
  (set `self.BulletManager` _returnvalue_2)
  (`KismetSystemLibrary.K2_SetTimerDelegate` (delegate `StopGrow`) 2.0))

(event `StopGrow`
  (`KismetSystemLibrary.K2_ClearAndInvalidateTimerHandle` (`self.GrowTimer`))
  (`KismetSystemLibrary.K2_SetTimerDelegate` (delegate `ShootBullets`) (`self.TimeBetweenShots`) true))

(event `Grow`
  (bind _sphere (`self.Sphere`))
  (`SceneComponent.SetWorldScale3D` _sphere (+ (`SceneComponent.RelativeScale3D` _sphere) 0.05)))

(event `ShootBullets`
  (bind _bossref (`self.BossRef`))
  (`/Game/Blueprints/Bullets/BP_BulletManager.SpawnBulletFromPool` (`self.BulletManager`) (`self.GetTransform`) 400.0 5.0 0 30 (`self.AngleChange`) 360.0 -0.5 0.0 0.0 0 false 0 _bossref null 0.0 0.0 0.0 0.0 0.0 0.0 0.0 (`/Game/Blueprints/Enemies/Boss/BP_Boss_Base.BasicBulletObjectPool` _bossref))
  (bind _val (`/Game/BasicFunctions.+= (float)` (`self.AngleChange`) 5.0))
  (`/Engine/EditorBlueprintResources/StandardMacros.IncrementInt` (`self.TimesChanged`)
    (:`  `
      (`/Game/BasicFunctions.+= (float)` (`self.TotalAngleChange`) _val))))

(fn `UserConstructionScript`)