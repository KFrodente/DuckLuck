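; Boss attack actor that swells a sphere for about a second, then repeatedly fires bullet spreads until destroyed.
; BeginPlay spawns a BulletManager and runs a looping grow timer, which StopGrow clears before starting the looping shot timer.
; Each shot requests three spreads 120 degrees apart from the boss's basic bullet pool, offset by AngleChange, which appears intended to advance per shot for a rotating pattern.
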(event `self.ReceiveBeginPlay`
  (bind _returnvalue (`KismetSystemLibrary.K2_SetTimerDelegate` (delegate `Grow`) 0.1 true))
  (set `self.GrowTimer` _returnvalue)
  (bind _returnvalue_2 (`|SpawnActorFromClass` "/Game/Blueprints/Bullets/BP_BulletManager.BP_BulletManager_C" (`self.GetTransform`) "Undefined" "MultiplyWithRoot" null null))
  (set `self.BulletManager` _returnvalue_2)
  (`KismetSystemLibrary.K2_SetTimerDelegate` (delegate `StopGrow`) 1.0))

(event `StopGrow`
  (`KismetSystemLibrary.K2_ClearAndInvalidateTimerHandle` (`self.GrowTimer`))
  (`KismetSystemLibrary.K2_SetTimerDelegate` (delegate `ShootBullets`) (`self.TimeBetweenShots`) true))

(event `Grow`
  (bind _sphere (`self.Sphere`))
  (`SceneComponent.SetWorldScale3D` _sphere (+ (`SceneComponent.RelativeScale3D` _sphere) 0.1)))

(event `ShootBullets`
  (bind _returnvalue (`self.GetOwner`))
  (bind _returnvalue_2 (`self.GetTransform`))
  (bind _anglechange (`self.AngleChange`))
  (bind _bulletmanager (`self.BulletManager`))
  (bind _returnvalue_3 (+ _anglechange 120.0))
  (bind _basicbulletobjectpool (`/Game/Blueprints/Enemies/Boss/BP_Boss_Base.BasicBulletObjectPool` (`self.BossRef`)))
  (`/Game/Blueprints/Bullets/BP_BulletManager.SpawnBulletFromPool` _bulletmanager _returnvalue_2 1000.0 5.0 0 10 _anglechange 15.0 -0.25 0.0 0.0 0 false 0 _returnvalue null 0.0 0.0 0.0 0.0 0.0 0.0 0.0 _basicbulletobjectpool)
  (`/Game/Blueprints/Bullets/BP_BulletManager.SpawnBulletFromPool` _bulletmanager _returnvalue_2 1000.0 5.0 0 10 _returnvalue_3 15.0 -0.25 0.0 0.0 0 false 0 _returnvalue null 0.0 0.0 0.0 0.0 0.0 0.0 0.0 _basicbulletobjectpool)
  (`/Game/Blueprints/Bullets/BP_BulletManager.SpawnBulletFromPool` _bulletmanager _returnvalue_2 1000.0 5.0 0 10 (+ _returnvalue_3 120.0) 15.0 -0.25 0.0 0.0 0 false 0 _returnvalue null 0.0 0.0 0.0 0.0 0.0 0.0 0.0 _basicbulletobjectpool)
  (`/Game/BasicFunctions.+= (float)` (`self.AngleChange`) 10.0))

(event `self.ReceiveDestroyed`
  (`parent.ReceiveDestroyed`))

(fn `UserConstructionScript`)