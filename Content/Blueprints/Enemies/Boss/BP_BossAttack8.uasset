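; Boss attack actor that combines telegraphed lasers with a steady bullet stream.
; On spawn it creates its own bullet manager and scales up its sphere on a timer for a second before starting two looping fire timers.
; One spawns two lingering warning-delayed lasers, each at a random arrow from its pair.
; The faster one fires small bullets from two other arrows, drawn from the boss's object pool.
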(event `self.ReceiveBeginPlay`
  (`parent.ReceiveBeginPlay`)
  (bind _returnvalue (`KismetSystemLibrary.K2_SetTimerDelegate` (delegate `Grow`) 0.1 true))
  (set `self.GrowTimer` _returnvalue)
  (bind _returnvalue_2 (`|SpawnActorFromClass` "/Game/Blueprints/Bullets/BP_BulletManager.BP_BulletManager_C" (`self.GetTransform`) "Undefined" "MultiplyWithRoot" null null))
  (set `self.BulletManager` _returnvalue_2)
  (`KismetSystemLibrary.K2_SetTimerDelegate` (delegate `StopGrow`) 1.0))

(event `StopGrow`
  (`KismetSystemLibrary.K2_ClearAndInvalidateTimerHandle` (`self.GrowTimer`))
  (`KismetSystemLibrary.K2_SetTimerDelegate` (delegate `ShootBullets`) (`self.TimeBetweenShots`) true)
  (`KismetSystemLibrary.K2_SetTimerDelegate` (delegate `FireDownSides`) 0.1 true))

(event `Grow`
  (bind _sphere (`self.Sphere`))
  (`SceneComponent.SetWorldScale3D` _sphere (+ (`SceneComponent.RelativeScale3D` _sphere) 0.1)))

(event `FireDownSides`
  (bind _bulletmanager (`self.BulletManager`))
  (bind _basicbulletobjectpool (`/Game/Blueprints/Enemies/Boss/BP_Boss_Base.BasicBulletObjectPool` (`self.BossRef`)))
  (`/Game/Blueprints/Bullets/BP_BulletManager.SpawnBulletFromPool` _bulletmanager (`SceneComponent.K2_GetComponentToWorld` (`self.Arrow`)) 1000.0 5.0 0 2 0.0 1.0 -0.25 0.0 0.0 0 false 0 null null 0.0 0.0 0.0 0.0 0.0 0.0 0.0 _basicbulletobjectpool)
  (`/Game/Blueprints/Bullets/BP_BulletManager.SpawnBulletFromPool` _bulletmanager (`SceneComponent.K2_GetComponentToWorld` (`self.Arrow1`)) 1000.0 5.0 0 2 0.0 0.0 -0.25 0.0 0.0 0 false 0 null null 0.0 0.0 0.0 0.0 0.0 0.0 0.0 _basicbulletobjectpool)
  (`GameplayStatics.PlaySound2D` "/Game/Assets/Audio/Boss/BossNormalShoot.BossNormalShoot" 0.8 (`KismetMathLibrary.RandomFloatInRange` 1.2 1.4) 0.0 null null))

(event `ShootBullets`
  (`|SpawnActorFromClass` "/Game/Blueprints/Bullets/Boss/BP_Bullet_LaserLasting_Boss.BP_Bullet_LaserLasting_Boss_C" (`SceneComponent.K2_GetComponentToWorld` (select `bool` (`KismetMathLibrary.RandomBool`) :`false` (`self.Arrow3`) :`true` (`self.Arrow2`))) "Undefined" "MultiplyWithRoot" (`self.GetOwner`) 300.0 0.8 1.2 5.0 0.0 null 0.0 0.0 0.0 0.0 0.0 0.0 0.0 false false null)
  (`|SpawnActorFromClass` "/Game/Blueprints/Bullets/Boss/BP_Bullet_LaserLasting_Boss.BP_Bullet_LaserLasting_Boss_C" (`SceneComponent.K2_GetComponentToWorld` (select `bool` (`KismetMathLibrary.RandomBool`) :`false` (`self.Arrow4`) :`true` (`self.Arrow5`))) "Undefined" "MultiplyWithRoot" (`self.GetOwner`) 300.0 0.8 1.2 5.0 0.0 null 0.0 0.0 0.0 0.0 0.0 0.0 0.0 false false null)
  (`GameplayStatics.PlaySound2D` "/Game/Assets/Audio/Boss/BossLaser.BossLaser" 0.8 (`KismetMathLibrary.RandomFloatInRange` 0.9 1.1) 0.0 null null))

(fn `UserConstructionScript`)