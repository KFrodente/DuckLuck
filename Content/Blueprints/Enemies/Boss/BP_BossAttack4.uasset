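; BP_BossAttack4 is a boss attack actor that fires a sweep of laser bullets.
; On spawn it creates its own BP_BulletManager and scales up its sprite on a short looping timer.
; A second timer then starts repeated shots through the manager, teleporting the actor along X after each.
; After a fixed shot count it destroys itself, and its Destroyed event calls CanAttack on the boss.
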(event `self.ReceiveBeginPlay`
  (bind _returnvalue (`KismetSystemLibrary.K2_SetTimerDelegate` (delegate `Grow`) 0.1 true))
  (set `self.GrowTimer` _returnvalue)
  (bind _returnvalue_2 (`|SpawnActorFromClass` "/Game/Blueprints/Bullets/BP_BulletManager.BP_BulletManager_C" (`self.GetTransform`) "Undefined" "MultiplyWithRoot" null null))
  (set `self.BulletManager` _returnvalue_2)
  (`KismetSystemLibrary.K2_SetTimerDelegate` (delegate `StopGrow`) 1.0))

(event `StopGrow`
  (`KismetSystemLibrary.K2_ClearAndInvalidateTimerHandle` (`self.GrowTimer`))
  (`KismetSystemLibrary.K2_SetTimerDelegate` (delegate `ShootBullets`) (`self.TimeBetweenShots`) true))

(event `Grow`
  (`SceneComponent.SetWorldScale3D` (`self.Sprite`) (+ (`SceneComponent.RelativeScale3D` (`self.Sprite`)) 0.1)))

(event `ShootBullets`
  (bind (_returnvalue_x _returnvalue_y _returnvalue_z) (`KismetMathLibrary.BreakVector` (`self.K2_GetActorLocation`)))
  (if (< (`self.LasersShot`) 28)
    (`/Game/Blueprints/Bullets/BP_BulletManager.SpawnBullet` (`self.BulletManager`) (`self.GetTransform`) 0.0 10.0 0 1 0.0 0.0 2.0 0.0 0.0 0 false 0 (`self.GetOwner`) "/Game/Blueprints/Bullets/BP_Bullet_Laser_Boss.BP_Bullet_Laser_Boss_C" null 0.0 0.0 0.0 0.0 0.0 0.0 0.0)
    (`self.K2_SetActorLocation` (`KismetMathLibrary.MakeVector` (+ _returnvalue_x (`self.PositionChange`)) 0.0 _returnvalue_z) false true)
    (`/Engine/EditorBlueprintResources/StandardMacros.IncrementInt` (`self.LasersShot`))
    (else
      (`self.K2_DestroyActor`))))

(event `self.ReceiveDestroyed`
  (`/Game/Blueprints/Enemies/Boss/BP_Boss_Base.CanAttack` (`self.BossRef`)))

(fn `UserConstructionScript`)