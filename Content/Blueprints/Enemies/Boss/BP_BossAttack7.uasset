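; BP_BossAttack7 is a boss attack actor that grows a sphere, then fires twin fans of bullets in a sweeping pattern.
; On BeginPlay it spawns a bullet manager and scales the sphere up on a looping timer for one second.
; A repeating timer then fires two spreads, offset either side of a sine-driven angle over real time, drawing from the boss's basic bullet pool.
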(event `self.ReceiveBeginPlay`
  (`parent.ReceiveBeginPlay`)
  (bind _returnvalue (`KismetSystemLibrary.K2_SetTimerDelegate` (delegate `Grow`) 0.1 true))
  (set `self.GrowTimer` _returnvalue)
  (bind _returnvalue_2 (`|SpawnActorFromClass` "/Game/Blueprints/Bullets/BP_BulletManager.BP_BulletManager_C" (`self.GetTransform`) "Undefined" "MultiplyWithRoot" null null))
  (set `self.BulletManager` _returnvalue_2)
  (`KismetSystemLibrary.K2_SetTimerDelegate` (delegate `StopGrow`) 1.0))

(event `StopGrow`
  (`KismetSystemLibrary.K2_ClearAndInvalidateTimerHandle` (`self.GrowTimer`))
  (`KismetSystemLibrary.K2_SetTimerDelegate` (delegate `ShootBullets`) (`self.TimeBetweenShots`) true))

(event `Grow`
  (bind _sphere (`self.Sphere`))
  (`SceneComponent.SetWorldScale3D` _sphere (+ (`SceneComponent.RelativeScale3D` _sphere) 0.1)))

(event `ShootBullets`
  (bind _returnvalue (`self.GetOwner`))
  (bind _returnvalue_2 (`self.GetTransform`))
  (bind _anglebetweensides (`self.AngleBetweenSides`))
  (bind _bulletmanager (`self.BulletManager`))
  (bind _anglechange (`self.AngleChange`))
  (bind _basicbulletobjectpool (`/Game/Blueprints/Enemies/Boss/BP_Boss_Base.BasicBulletObjectPool` (`self.BossRef`)))
  (set `self.AngleChange` (+ (`self.AngleMod`) (* (`KismetMathLibrary.Sin` (* (`GameplayStatics.GetRealTimeSeconds`) (`self.Speed`))) (`self.Amplitude`))))
  (`/Game/Blueprints/Bullets/BP_BulletManager.SpawnBulletFromPool` _bulletmanager _returnvalue_2 1000.0 5.0 0 5 (- _anglechange _anglebetweensides) 45.0 -0.25 0.0 0.0 0 false 0 _returnvalue null 0.0 0.0 0.0 0.0 0.0 0.0 0.0 _basicbulletobjectpool)
  (`/Game/Blueprints/Bullets/BP_BulletManager.SpawnBulletFromPool` _bulletmanager _returnvalue_2 1000.0 5.0 0 5 (+ _anglechange _anglebetweensides) 45.0 -0.25 0.0 0.0 0 false 0 _returnvalue null 0.0 0.0 0.0 0.0 0.0 0.0 0.0 _basicbulletobjectpool))

(fn `UserConstructionScript`)