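; BP_BossAttack3 is a boss attack actor that grows a sphere, then repeatedly fires radial spreads of boss laser bullets.
; On BeginPlay it spawns a BP_BulletManager and scales the sphere up on a looping timer for one second.
; It then switches to a looping shot timer that has the manager spawn full-circle spreads, using AngleChange as the angle offset.
; When destroyed, it calls CanAttack on the boss reference.
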(event `self.ReceiveBeginPlay`
  (bind _returnvalue (`KismetSystemLibrary.K2_SetTimerDelegate` (delegate `Grow`) 0.1 true))
  (set `self.GrowTimer` _returnvalue)
  (bind _returnvalue_2 (`|SpawnActorFromClass` "/Game/Blueprints/Bullets/BP_BulletManager.BP_BulletManager_C" (`self.GetTransform`) "Undefined" "MultiplyWithRoot" null null))
  (set `self.BulletManager` _returnvalue_2)
  (`KismetSystemLibrary.K2_SetTimerDelegate` (delegate `StopGrow`) 1.0))

(event `StopGrow`
  (`KismetSystemLibrary.K2_ClearAndInvalidateTimerHandle` (`self.GrowTimer`))
  (`KismetSystemLibrary.K2_SetTimerDelegate` (delegate `ShootBullets`) (`self.TimeBetweenShots`) true))

(event `Grow`
  (bind _sphere (`self.Sphere`))
  (`SceneComponent.SetWorldScale3D` _sphere (+ (`SceneComponent.RelativeScale3D` _sphere) 0.1)))

(event `ShootBullets`
  (`/Game/Blueprints/Bullets/BP_BulletManager.SpawnBullet` (`self.BulletManager`) (`self.GetTransform`) 0.0 10.0 0 20 (`self.AngleChange`) 360.0 4.0 0.0 0.0 0 false 0 (`self.GetOwner`) "/Game/Blueprints/Bullets/BP_Bullet_Laser_Boss.BP_Bullet_Laser_Boss_C" null 0.0 0.0 0.0 0.0 0.0 0.0 0.0)
  (`/Game/BasicFunctions.+= (float)` (`self.AngleChange`) 45.0))

(event `self.ReceiveDestroyed`
  (`/Game/Blueprints/Enemies/Boss/BP_Boss_Base.CanAttack` (`self.BossRef`)))

(fn `UserConstructionScript`)