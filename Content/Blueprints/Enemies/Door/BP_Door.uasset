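; BP_Door is a breakable door built as an enemy, which only a BP_PlayerWithHat can knock down.
; Any hit from that player zeroes its health and calls Death, which hides the cube, disables collision and starts a one-shot timer, likely for respawning.
; ReviveDoor, also called on BeginPlay, restores health, visibility and collision.
; TickCall and CheckHunger are empty, and damage reports no damage, kill or dominance.
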(event `self.ReceiveBeginPlay`
  (set `/Game/Blueprints/Components/BPC_Health.CurrentHealth` 1 (`self.BPC_Health`))
  (`self.ReviveDoor`))

(event `self.TickCall`
  (params (CalledTick :type Integer)))

(event `/Game/Blueprints/Interfaces_Enums/I_Damagable.Death`
  (bind _cube (`self.Cube`))
  (bind _capsulecomponent (`self.CapsuleComponent`))
  (set `self.Active` false)
  (`ActorComponent.SetActive` _cube false false)
  (`SceneComponent.SetVisibility` _cube false false)
  (`PrimitiveComponent.SetCollisionEnabled` _cube "NoCollision")
  (`ActorComponent.SetActive` _capsulecomponent false false)
  (`PrimitiveComponent.SetCollisionEnabled` _capsulecomponent "NoCollision"))

(fn `CheckHunger`
  (params (FromWorldTick :type Boolean)))

(fn `ReviveDoor`
  (bind _cube (`self.Cube`))
  (bind _capsulecomponent (`self.CapsuleComponent`))
  (set `/Game/Blueprints/Components/BPC_Health.CurrentHealth` 1 (`self.BPC_Health`))
  (`PrimitiveComponent.SetCollisionEnabled` _capsulecomponent "QueryAndPhysics")
  (`ActorComponent.SetActive` _capsulecomponent true false)
  (set `self.Active` true)
  (`ActorComponent.SetActive` _cube true false)
  (`PrimitiveComponent.SetCollisionEnabled` _cube "QueryAndPhysics")
  (`SceneComponent.SetVisibility` _cube true false))

(fn `Take Damage`
  (params (Damage :type Integer) (DamageDealer :type "Actor Object Reference"))
  (returns (DamageDealt :type Integer) (KilledEnemy :type Boolean) (Dominance :type Integer))
  (cast `/Game/Blueprints/Player/BP_PlayerWithHat` DamageDealer)
  (set `/Game/Blueprints/Components/BPC_Health.CurrentHealth` 0 (`self.BPC_Health`))
  (`/Game/Blueprints/Interfaces_Enums/I_Damagable.Death`)
  (`ActorComponent.SetActive` (`self.CapsuleComponent`) false false)
  (`KismetSystemLibrary.K2_SetTimerDelegate` (`|CreateDelegate` :!event `ReviveDoor`) 5.0)
  (return 0 false 0))

(fn `UserConstructionScript`)