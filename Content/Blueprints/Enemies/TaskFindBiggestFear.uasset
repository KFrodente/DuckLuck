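; Behavior tree task where an enemy decides whether to fight or flee the most dominant visible actor nearby.
; A sphere overlap and wall line traces select the highest-Dominance enemy or player as BiggestFear.
; The stronger trait, Fear or Aggressive, is tested first, scaled by Dominance difference, with fleeing only when outranked.
; FindFood makes reactions probabilistic; results set the Flee, Fight and WantedActor blackboard keys.
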(event `self.ReceiveExecuteAI`
  (params (OwnerController :type "AIController Object Reference") (ControlledPawn :type "Pawn Object Reference"))
  (bind _wantedactor (`self.WantedActor`))
  (bind _returnvalue (`BTFunctionLibrary.GetBlackboardValueAsBool` (`self.FindFood`)))
  (bind _returnvalue_2 (`BTFunctionLibrary.GetBlackboardValueAsBool` (`self.FindFood`)))
  (set `self.CheckedFear` false)
  (set `self.CheckedAggression` false)
  (set `self.SeenEnemies` 0)
  (set `self.BiggestFear` null)
  (set `self.HighestDominance` 0)
  (bind (_outactors _returnvalue_3) (`KismetSystemLibrary.SphereOverlapActors` (`Actor.K2_GetActorLocation` ControlledPawn) 1000.0 (`self.EnemySearch`)))
  (if (and _returnvalue_3 (> (`KismetArrayLibrary.Array_Length` _outactors) 1))
    (for _array_element _outactors
      (if (!= _array_element ControlledPawn)
        (bind (_outhit _returnvalue_4) (`KismetSystemLibrary.LineTraceSingleForObjects` :`Start` (`Actor.K2_GetActorLocation` ControlledPawn) :`End` (`Actor.K2_GetActorLocation` _array_element) :`ObjectTypes` (`self.WorldSearch`) :`TraceColor` (struct :`R` 0.309498 :`G` 0.347551 :`B` 1.0 :`A` 1.0) :`TraceHitColor` (struct :`R` 0.949116 :`G` 0.064575 :`B` 1.0 :`A` 1.0)))
        (if (not _returnvalue_4)
          (bind _asbp_enemy_base (cast `/Game/Blueprints/Enemies/BP_Enemy_Base` _array_element)
            (:`then`
              (bind _dominance (`/Game/Blueprints/Enemies/BP_Enemy_Base.Dominance` _asbp_enemy_base))
              (if (> _dominance (`self.HighestDominance`))
                (set `self.BiggestFear` _asbp_enemy_base)
                (set `self.HighestDominance` _dominance)
                (`/Engine/EditorBlueprintResources/StandardMacros.IncrementInt` (`self.SeenEnemies`) :!label _label)))
            (:`CastFailed`
              (bind _asbp_player_with_hat (cast `/Game/Blueprints/Player/BP_PlayerWithHat` _array_element)
                (:`then`
                  (bind _dominance_2 (`/Game/Blueprints/Player/BP_PlayerWithHat.Dominance` _asbp_player_with_hat))
                  (if (> _dominance_2 (`self.HighestDominance`))
                    (set `self.BiggestFear` _asbp_player_with_hat)
                    (set `self.HighestDominance` _dominance_2)
                    (goto _label)))
                (:`CastFailed`
                  (bind _asbp_player_no_hat (cast `/Game/Blueprints/Player/BP_PlayerNoHat` _array_element))
                  (if (> 0 (`self.HighestDominance`))
                    (set `self.BiggestFear` _asbp_player_no_hat)
                    (set `self.HighestDominance` 0)
                    (goto _label)))))))))
    (bind _asbp_enemy_base_2 (cast `/Game/Blueprints/Enemies/BP_Enemy_Base` ControlledPawn)
      (:`then`
        (if (> (`self.SeenEnemies`) 0)
          (if (>= (`/Game/Blueprints/Enemies/BP_Enemy_Base.Fear` _asbp_enemy_base_2) (`/Game/Blueprints/Enemies/BP_Enemy_Base.Aggressive` _asbp_enemy_base_2))
            (`/Engine/EditorBlueprintResources/StandardMacros.IsValid` (`self.BiggestFear`) :!label _label_2
              (:`Is Valid`
                (bind _returnvalue_5 (- (`/Game/Blueprints/Enemies/BP_Enemy_Base.Dominance` _asbp_enemy_base_2) (`self.HighestDominance`)))
                (if (>= _returnvalue_5 0)
                  (set `self.CheckedFear` true)
                  (if (`self.CheckedFear`) :!label _label_3
                    (if (`self.CheckedAggression`)
                      (`BTFunctionLibrary.SetBlackboardValueAsBool` (`self.Flee`) :!label _label_4)
                      (`BTFunctionLibrary.SetBlackboardValueAsBool` (`self.Fight`))
                      (`BTFunctionLibrary.SetBlackboardValueAsObject` _wantedactor ControlledPawn)
                      (`self.FinishExecute` false)
                      (else
                        (`/Engine/EditorBlueprintResources/StandardMacros.IsValid` (`self.BiggestFear`) :!label _label_5
                          (:`Is Valid`
                            (bind _aggressive (`/Game/Blueprints/Enemies/BP_Enemy_Base.Aggressive` _asbp_enemy_base_2))
                            (if (> (* _aggressive (`KismetMathLibrary.Abs_Int` (- (`/Game/Blueprints/Enemies/BP_Enemy_Base.Dominance` _asbp_enemy_base_2) (`self.HighestDominance`)))) 0.8)
                              (if (or (and _returnvalue_2 (`KismetMathLibrary.RandomBoolWithWeight` _aggressive)) (not _returnvalue_2))
                                (`BTFunctionLibrary.SetBlackboardValueAsBool` (`self.Flee`))
                                (`BTFunctionLibrary.SetBlackboardValueAsBool` (`self.Fight`) true)
                                (`BTFunctionLibrary.SetBlackboardValueAsObject` (`self.WantedActor`) (`self.BiggestFear`))
                                (`self.FinishExecute` true)
                                (else
                                  (set `self.CheckedAggression` true)
                                  (goto _label_3)))
                              (else
                                (set `self.CheckedAggression` true)
                                (goto _label_3))))
                          (:`Is Not Valid`
                            (goto _label_4)))))
                    (else
                      (goto _label_2)))
                  (else
                    (bind _fear (`/Game/Blueprints/Enemies/BP_Enemy_Base.Fear` _asbp_enemy_base_2))
                    (if (> (* _fear (`KismetMathLibrary.Abs_Int` _returnvalue_5)) 0.8)
                      (if (or (and _returnvalue (`KismetMathLibrary.RandomBoolWithWeight` _fear)) (not _returnvalue))
                        (`BTFunctionLibrary.SetBlackboardValueAsBool` (`self.Flee`) true)
                        (`BTFunctionLibrary.SetBlackboardValueAsBool` (`self.Fight`))
                        (`BTFunctionLibrary.SetBlackboardValueAsObject` _wantedactor (`self.BiggestFear`))
                        (`self.FinishExecute` true)
                        (else
                          (set `self.CheckedFear` true)
                          (goto _label_3)))
                      (else
                        (set `self.CheckedFear` true)
                        (goto _label_3))))))
              (:`Is Not Valid`
                (goto _label_4)))
            (else
              (goto _label_5)))
          (else
            (goto _label_3))))
      (:`CastFailed`
        (goto _label_3)))
    (else
      (`BTFunctionLibrary.SetBlackboardValueAsBool` (`self.Flee`))
      (`self.FinishExecute` false))))