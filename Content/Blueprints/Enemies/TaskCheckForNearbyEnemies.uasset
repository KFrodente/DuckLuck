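; Behavior tree node for enemy AI that checks for nearby actors and flags when the enemy should change priority.
; Each tick it sphere-overlaps around the controlled BP_Enemy_Base pawn and continues if more than one actor is found.
; If not already fighting, a randomly boosted Aggressive trait over a threshold sets the ChangePriority blackboard key.
; Failing that, Fear gets the same roll unless already fleeing.
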(event `self.ReceiveTickAI`
  (params (OwnerController :type "AIController Object Reference") (ControlledPawn :type "Pawn Object Reference") (DeltaSeconds :type "Float (single-precision)"))
  (bind _asbp_enemy_base (cast `/Game/Blueprints/Enemies/BP_Enemy_Base` ControlledPawn))
  (bind _outactors (`KismetSystemLibrary.SphereOverlapActors` (`Actor.K2_GetActorLocation` ControlledPawn) (`self.CheckRadius`) (`self.EnemyTypes`)))
  (if (> (`KismetArrayLibrary.Array_Length` _outactors) 1)
    (bind _aggressive (`/Game/Blueprints/Enemies/BP_Enemy_Base.Aggressive` _asbp_enemy_base))
    (if (and (not (`BTFunctionLibrary.GetBlackboardValueAsBool` (`self.Fight`))) (> (+ _aggressive (`KismetMathLibrary.RandomFloatInRange` 0.0 _aggressive)) 0.8))
      (`BTFunctionLibrary.SetBlackboardValueAsBool` (`self.ChangePriority`) true :!label _label)
      (else
        (bind _fear (`/Game/Blueprints/Enemies/BP_Enemy_Base.Fear` _asbp_enemy_base))
        (if (and (not (`BTFunctionLibrary.GetBlackboardValueAsBool` (`self.Flee`))) (> (+ _fear (`KismetMathLibrary.RandomFloatInRange` 0.0 _fear)) 0.8))
          (goto _label))))))