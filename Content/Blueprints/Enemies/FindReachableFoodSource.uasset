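; Behavior tree task that picks a reachable food source for a BP_Enemy_Base to go after.
; With a valid WantedActor it re-searches only if an Intelligence-weighted random roll passes, otherwise succeeding with the current target.
; A sphere overlap finds active FoodSource components matching the preferred or wildcard type, ranked by the enemy Grid's heuristic path distance.
; The cheapest reachable one sets the blackboard actor and position; finding none fails the task.
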(event `self.ReceiveExecuteAI`
  (params (OwnerController :type "AIController Object Reference") (ControlledPawn :type "Pawn Object Reference"))
  (bind _returnvalue (`BTFunctionLibrary.GetBlackboardValueAsActor` (`self.WantedActor`)))
  (bind _asbp_enemy_base (cast `/Game/Blueprints/Enemies/BP_Enemy_Base` ControlledPawn))
  (set `self.FoundFood` false)
  (set `self.LowestHeuristic` 100000)
  (if (`KismetSystemLibrary.IsValid` _returnvalue)
    (if (> (+ (`/Game/Blueprints/Enemies/BP_Enemy_Base.Intelligence` _asbp_enemy_base) (`KismetMathLibrary.RandomFloat`)) 0.8)
      (bind (_outactors _returnvalue_2) (`KismetSystemLibrary.SphereOverlapActors` (`Actor.K2_GetActorLocation` ControlledPawn) (`self.SearchRange`) (`self.Object Types`) :!label _label))
      (if _returnvalue_2
        (for _array_element _outactors
          (bind _returnvalue_3 (`Actor.GetComponentByClass` _array_element "/Game/Blueprints/World/FoodSource.FoodSource_C"))
          (`/Engine/EditorBlueprintResources/StandardMacros.IsValid` _returnvalue_3
            (:`Is Valid`
              (bind _foodtype (`/Game/Blueprints/World/FoodSource.FoodType` _returnvalue_3))
              (if (and (or (`|EnumEquality` (`/Game/Blueprints/Enemies/BP_Enemy_Base.PreferredFood` _asbp_enemy_base) _foodtype) (`|EnumEquality` _foodtype "NewEnumerator2")) (`/Game/Blueprints/World/FoodSource.ActiveFoodSource` _returnvalue_3) (!= _returnvalue_3 _returnvalue))
                ;[1 1 1] if it cant find something have it wander
                (bind (_totalheuristic _lowestheuristic _foundpath) (`/Game/Blueprints/Grid/BP_Grid.Get Heuristical Distance` (`/Game/Blueprints/Enemies/BP_Enemy_Base.Grid` _asbp_enemy_base) (`Actor.K2_GetActorLocation` ControlledPawn) (`Actor.K2_GetActorLocation` _array_element) (`self.FoodCheckDistance`) (0.0 0.0 1.0)))
                (if (and (< _totalheuristic (`self.LowestHeuristic`)) _foundpath)
                  (set `self.LowestHeuristic` _totalheuristic)
                  (`BTFunctionLibrary.SetBlackboardValueAsObject` (`self.WantedActor`) _array_element)
                  (`BTFunctionLibrary.SetBlackboardValueAsVector` (`self.WatedPosition`) (`Actor.K2_GetActorLocation` _array_element))
                  (set `self.FoundFood` true))))))
        (`self.FinishExecute` (`self.FoundFood`))
        (else
          (`self.FinishExecute` false)))
      (else
        (`self.FinishExecute` true)))
    (else
      (goto _label))))