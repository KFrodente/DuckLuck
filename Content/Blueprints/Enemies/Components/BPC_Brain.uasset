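; Enemy brain component that gives its owner personality traits and tracks aggression and fear toward others.
; Shortly after BeginPlay it constructs preset or random trait objects, with random picks recursing by weighted chance, then applies them to the BP_Enemy_Base owner.
; AddToEnemyMaps updates aggression and fear maps per enemy type and per named creature.
; Per-creature threshold tiers add randomly worded first-person memories, gated by component-wide one-shot flags.
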(event `self.ReceiveBeginPlay`
  (`KismetSystemLibrary.K2_SetTimerDelegate` (delegate `GetTraits`) 0.5))

(event `GetTraits`
  (if (not (`self.AlreadyGainedTraits`))
    (`self.DoTraitTasks`)))

(fn `AddToEnemyMaps`
  (params (EnemyType :type "/Game/Blueprints/Interfaces_Enums/E_EnemyType Enum" :default "NewEnumerator3") (AggAmount :type "Float (double-precision)") (FearAmount :type "Float (double-precision)") (OtherName :type String))
  (bind _val (`/Game/BasicFunctions.+= (float)` (`BlueprintMapLibrary.Map_Find` (`self.Aggressors`) EnemyType) (`local.AggAmount`)))
  (bind _val_2 (`/Game/BasicFunctions.RaiseToZero (float)` _val))
  (`BlueprintMapLibrary.Map_Add` (`self.Aggressors`) (`local.EnemyType`) _val_2)
  (bind _val_3 (`/Game/BasicFunctions.+= (float)` (`BlueprintMapLibrary.Map_Find` (`self.Fears`) (`local.EnemyType`)) (`local.FearAmount`)))
  (bind _val_4 (`/Game/BasicFunctions.RaiseToZero (float)` _val_3))
  (`BlueprintMapLibrary.Map_Add` (`self.Fears`) (`local.EnemyType`) _val_4)
  (`self.AddToSpecificCreatures` (`local.AggAmount`) (`local.FearAmount`) (`local.OtherName`)))

(fn `AddToSpecificCreatures`
  (params (AggAmount :type "Float (double-precision)") (FearAmount :type "Float (double-precision)") (CreatureName :type String))
  (locals (OAggression :type "Float (double-precision)") (OFear :type "Float (double-precision)"))
  (bind _creaturename (`local.CreatureName`))
  (bind _creaturename_2 (`local.CreatureName`))
  (bind _creaturename_3 (`local.CreatureName`))
  (bind _creaturename_4 (`local.CreatureName`))
  (bind _creaturename_5 (`local.CreatureName`))
  (bind _creaturename_6 (`local.CreatureName`))
  (bind _value (`BlueprintMapLibrary.Map_Find` (`self.SpecificFear`) (`local.CreatureName`)))
  (bind _value_2 (`BlueprintMapLibrary.Map_Find` (`self.SpecificAggression`) CreatureName))
  (set `local.OAggression` _value_2)
  (bind _val (`/Game/BasicFunctions.+= (float)` _value_2 (`local.AggAmount`)))
  (`BlueprintMapLibrary.Map_Add` (`self.SpecificAggression`) (`local.CreatureName`) _val)
  (if (>= _val 1.0)
    (if (>= _val 2.0)
      (if (>= _val 3.0)
        (if (not (>= _val 4.0))
          (if (not (`self.DoneAggro_3`))
            (`KismetArrayLibrary.Array_Add` (`self.Memories`) (`KismetTextLibrary.Conv_TextToString` (select `int` (`KismetMathLibrary.RandomIntegerInRange` 0 2) :`0` (`|FormatText` "I am starting to get annoyed by {otherName}" _creaturename_4) :`1` (`|FormatText` "I am easily angered by {otherName}" _creaturename_4) :`2` (`|FormatText` "I was irritated by {otherName}" _creaturename_4))))
            (set `self.DoneAggro_3` true))
          (set `local.OFear` _value :!label _label)
          (bind _val_2 (`/Game/BasicFunctions.+= (float)` _value (`local.FearAmount`)))
          (`BlueprintMapLibrary.Map_Add` (`self.SpecificFear`) (`local.CreatureName`) _val_2)
          (if (>= _val_2 1.0)
            (if (>= _val_2 2.0)
              (if (>= _val_2 3.0)
                (if (>= _val_2 4.0)
                  _
                  (elif (not (`self.DoneFear_3`))
                    (`KismetArrayLibrary.Array_Add` (`self.Memories`) (`KismetTextLibrary.Conv_TextToString` (select `int` (`KismetMathLibrary.RandomIntegerInRange` 0 2) :`0` (`|FormatText` "{otherName} terrifies me" _creaturename) :`1` (`|FormatText` "I can't get away from {otherName} " _creaturename) :`2` (`|FormatText` "{otherName} please let me leave I'm begging you" _creaturename))))
                    (set `self.DoneFear_3` true)))
                (elif (not (`self.DoneFear_2`))
                  (`KismetArrayLibrary.Array_Add` (`self.Memories`) (`KismetTextLibrary.Conv_TextToString` (select `int` (`KismetMathLibrary.RandomIntegerInRange` 0 2) :`0` (`|FormatText` "{otherName} really scares me" _creaturename_5) :`1` (`|FormatText` "Why wont {otherName} chase someone else" _creaturename_5) :`2` (`|FormatText` "{otherName} please leave me alone" _creaturename_5))))
                  (set `self.DoneFear_2` true)))
              (elif (not (`self.DoneFear_1`))
                (`KismetArrayLibrary.Array_Add` (`self.Memories`) (`KismetTextLibrary.Conv_TextToString` (select `int` (`KismetMathLibrary.RandomIntegerInRange` 0 2) :`0` (`|FormatText` "{otherName} is a little scary" _creaturename_2) :`1` (`|FormatText` "{otherName} keeps following me" _creaturename_2) :`2` (`|FormatText` "{otherName} wont leave me alone" _creaturename_2))))
                (set `self.DoneFear_1` true)))))
        (elif (`self.DoneAggro_2`)
          (goto _label)
          (else
            (`KismetArrayLibrary.Array_Add` (`self.Memories`) (`KismetTextLibrary.Conv_TextToString` (select `int` (`KismetMathLibrary.RandomIntegerInRange` 0 2) :`0` (`|FormatText` "I am starting to get annoyed by {otherName}" _creaturename_6) :`1` (`|FormatText` "I am easily angered by {otherName}" _creaturename_6) :`2` (`|FormatText` "I was irritated by {otherName}" _creaturename_6))))
            (set `self.DoneAggro_2` true)
            (goto _label))))
      (elif (`self.DoneAggro_1`)
        (goto _label)
        (else
          (`KismetArrayLibrary.Array_Add` (`self.Memories`) (`KismetTextLibrary.Conv_TextToString` (select `int` (`KismetMathLibrary.RandomIntegerInRange` 0 2) :`0` (`|FormatText` "{otherName} annoyed me" _creaturename_3) :`1` (`|FormatText` "I am easily angered by {otherName}" _creaturename_3) :`2` (`|FormatText` "I was irritated by {otherName}" _creaturename_3))))
          (set `self.DoneAggro_1` true)
          (goto _label))))
    (else
      (goto _label))))

(fn `DoTraitTasks`
  (`KismetArrayLibrary.Array_Clear` (`self.Traits`))
  (`|ExecutionSequence`
    (:`then_0`
      (if (`self.PresetTraits`)
        (for _array_element (`self.TraitClasses`)
          (`self.GainTraits` false _array_element))
        (else
          (`self.GainTraits` true))))
    (:`then_1`
      (set `self.AlreadyGainedTraits` true)
      (bind _asbp_enemy_base (cast `/Game/Blueprints/Enemies/BP_Enemy_Base` (`self.GetOwner`)))
      (for _array_element_2 (`self.Traits`)
        (`/Game/Blueprints/Enemies/Traits/BP_Trait_Base.ApplyTrait` _array_element_2 _asbp_enemy_base)))))

(fn `GainTraits`
  (params (Random :type Boolean) (WantedTrait :type "/Game/Blueprints/Enemies/Traits/BP_Trait_Base Class Reference"))
  (bind _unusedtraits (`self.UnusedTraits`))
  (bind _unusedtraits_2 (`self.UnusedTraits`))
  (if Random
    (bind (_trait _pickedtype) (`/Game/BasicFunctions.GetTrait` _unusedtraits))
    (`KismetArrayLibrary.Array_Remove` _unusedtraits (`KismetArrayLibrary.Array_Find` _unusedtraits _pickedtype))
    (`KismetArrayLibrary.Array_Add` (`self.TraitClasses`) _trait)
    (bind _returnvalue (`|GenericCreateObject` (`self.GetOwner`) _trait))
    (`KismetArrayLibrary.Array_Add` (`self.Traits`) _returnvalue)
    (if (`KismetMathLibrary.RandomBoolWithWeight` (`self.AdditionalTraitChance`))
      (`/Game/BasicFunctions.*= (float)` (`self.AdditionalTraitChance`) 0.5)
      (`self.GainTraits` true))
    (else
      (bind _returnvalue_2 (`|GenericCreateObject` (`self.GetOwner`) WantedTrait))
      (`KismetArrayLibrary.Array_Add` (`self.Traits`) _returnvalue_2)
      (`KismetArrayLibrary.Array_Remove` _unusedtraits_2 (`KismetArrayLibrary.Array_Find` _unusedtraits_2 (`/Game/Blueprints/Enemies/Traits/BP_Trait_Base.TraitType` _returnvalue_2))))))