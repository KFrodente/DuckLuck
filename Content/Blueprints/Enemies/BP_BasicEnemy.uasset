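; BP_BasicEnemy is a basic enemy actor that takes damage and is destroyed when its health runs out.
; AnyDamage truncates incoming damage to an integer and forwards it to TakeDamage, which subtracts it from the BPCHealth component's CurrentHealth and prints the result.
; At zero or below, TakeDamage calls the Death event, which destroys the actor.
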(event `/Game/Blueprints/Interfaces_Enums/I_PlayerDamagable.Take Damage`
  (params (Damage :type Integer))
  (bind _bpc_health (`self.BPC_Health`))
  (bind _output_get (set `/Game/Blueprints/Components/BPC_Health.CurrentHealth` (- (`/Game/Blueprints/Components/BPC_Health.CurrentHealth` _bpc_health) Damage) _bpc_health))
  (`KismetSystemLibrary.PrintText` (`KismetTextLibrary.Conv_IntToText` _output_get))
  (if (<= _output_get 0)
    (`/Game/Blueprints/Interfaces_Enums/I_PlayerDamagable.Death`)))

(event `/Game/Blueprints/Interfaces_Enums/I_PlayerDamagable.Death`
  (`self.K2_DestroyActor`))

(event `self.ReceiveAnyDamage`
  (params (Damage :type "Float (single-precision)") (DamageType :type "DamageType Object Reference") (InstigatedBy :type "Controller Object Reference") (DamageCauser :type "Actor Object Reference"))
  (`/Game/Blueprints/Interfaces_Enums/I_PlayerDamagable.Take Damage` (`KismetMathLibrary.FTrunc` Damage)))

(fn `UserConstructionScript`
  (`parent.UserConstructionScript`))