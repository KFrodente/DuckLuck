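; Grid pathfinding helper that searches 64-unit cells on the XZ plane toward a goal.
; Capped greedy searches expand four neighbors, skip blocked or used cells, favor low Manhattan distance, and return total and lowest heuristic plus path success.
; The jump variant flags cells without ground below as airborne, scans checked cells backward for jump start/end points, and draws debug boxes.
; GetStartHeuristic returns just the starting cell's estimate.
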(fn `Get Heuristical Distance`
  (params (P1 :type "Vector Structure") (Goal :type "Vector Structure") (MaxCheckDistance :type Integer) (PointNormal :type "Vector Structure"))
  (returns (TotalHeuristic :type Integer) (LowestHeuristic :type Integer) (FoundPath :type Boolean))
  (bind _x (.x Goal))
  (bind _z (.z Goal))
  (bind _x_2 (.x P1))
  (bind _z_2 (.z P1))
  (bind _lowestheuristic (`self.LowestHeuristic`))
  (bind _currentgrid (`self.CurrentGrid`))
  (bind _lowestheuristic_2 (`self.LowestHeuristic`))
  (bind (_position _heuristicvalue _cost) (break `/Game/Blueprints/Grid/S_Grid` _currentgrid))
  (bind _returnvalue (mod _x_2 64.0))
  (bind _returnvalue_2 (mod _z_2 64.0))
  (bind _returnvalue_3 (+ _cost 1))
  (set `self.R` (`KismetMathLibrary.RandomFloat`))
  (set `self.G` (`KismetMathLibrary.RandomFloat`))
  (set `self.B` (`KismetMathLibrary.RandomFloat`))
  (`KismetArrayLibrary.Array_Clear` (`self.UsedPositions`))
  (set `self.CheckDistance` 0)
  (set `self.TotalHeuristic` 0)
  (set `self.LowestHeuristic` -1)
  (set `self.FoundPath` false)
  (bind _output_get (set `self.Start` (`KismetMathLibrary.MakeVector` (+ _x_2 (+ (* PointNormal_X (* _returnvalue 2.0)) _returnvalue)) 0.0 (+ _z_2 (+ (* (* _returnvalue_2 2.0) (* PointNormal_Z -1.0)) _returnvalue_2)))))
  (set `self.Goal` (`KismetMathLibrary.MakeVector` (+ _x (mod _x 64.0)) 0.0 (+ _z (mod _z 64.0))))
  (`self.MakeNewPosition` _output_get _output_get)
  (if (== (`KismetArrayLibrary.Array_Length` (`self.CheckList`)) 0)
    (return -1 -1 false)
    (else
      (while (< (`self.CheckDistance`) MaxCheckDistance)
        (bind _output_get_2 (set `self.CurrentGrid` (`|GetArrayItem` (`self.CheckList`))))
        (bind (_position_2 _heuristicvalue_2) (break `/Game/Blueprints/Grid/S_Grid` _output_get_2))
        (set `self.TotalHeuristic` (+ (`self.TotalHeuristic`) _heuristicvalue_2))
        (if (or (< _heuristicvalue_2 _lowestheuristic_2) (< _lowestheuristic_2 0))
          (set `self.LowestHeuristic` _heuristicvalue_2))
        (if (== _position_2 (`self.Goal`) :`ErrorTolerance` 64.0)
          (set `self.FoundPath` true)
          (`KismetArrayLibrary.Array_Clear` (`self.BeenCheckedList`) :!label _label)
          (`KismetArrayLibrary.Array_Clear` (`self.CheckList`))
          (return (`self.TotalHeuristic`) (`self.LowestHeuristic`) (`self.FoundPath`))
          (else
            (`KismetArrayLibrary.Array_Add` (`self.BeenCheckedList`) _currentgrid)
            (`KismetArrayLibrary.Array_Remove` (`self.CheckList`))
            (`self.MakeNewPosition` (+ _position (64.0 0.0 0.0)) _position _returnvalue_3)
            (`self.MakeNewPosition` (+ _position (-64.0 0.0 0.0)) _position _returnvalue_3)
            (`self.MakeNewPosition` (+ _position (0.0 0.0 64.0)) _position _returnvalue_3)
            (`self.MakeNewPosition` (+ _position (0.0 0.0 -64.0)) _position _returnvalue_3)
            (`/Engine/EditorBlueprintResources/StandardMacros.IncrementInt` (`self.CheckDistance`)))))
      (while (> (`KismetArrayLibrary.Array_Length` (`self.CheckList`)) 0)
        (bind _output_get_3 (set `self.CurrentGrid` (`|GetArrayItem` (`self.CheckList`))))
        (bind (_position_3 _heuristicvalue_3) (break `/Game/Blueprints/Grid/S_Grid` _output_get_3))
        (set `self.TotalHeuristic` (+ (`self.TotalHeuristic`) _heuristicvalue_3))
        (if (or (< _heuristicvalue_3 _lowestheuristic) (< _lowestheuristic 0))
          (set `self.LowestHeuristic` _heuristicvalue_3))
        (if (== _position_3 (`self.Goal`) :`ErrorTolerance` 64.0)
          (set `self.FoundPath` true)
          (goto _label)
          (else
            (`KismetArrayLibrary.Array_Add` (`self.BeenCheckedList`))
            (`KismetArrayLibrary.Array_Remove` (`self.CheckList`)))))
      (goto _label))))

(fn `Get HeuristicalDistanceWithJump`
  (params (P1 :type "Vector Structure") (Goal :type "Vector Structure") (MaxCheckDistance :type Integer) (PointNormal :type "Vector Structure"))
  (returns (TotalHeuristic :type Integer) (LowestHeuristic :type Integer) (FoundPath :type Boolean) (JumpStartLocations :type "Array of Vector Structure") (JumpEndLocations :type "Array of Vector Structure"))
  (bind _x (.x Goal))
  (bind _z (.z Goal))
  (bind _x_2 (.x P1))
  (bind _z_2 (.z P1))
  (bind _beencheckedlist (`self.BeenCheckedList`))
  (bind _lowestheuristic (`self.LowestHeuristic`))
  (bind _beencheckedlist_2 (`self.BeenCheckedList`))
  (bind _currentgrid (`self.CurrentGrid`))
  (bind _lowestheuristic_2 (`self.LowestHeuristic`))
  (bind (_position _heuristicvalue _cost) (break `/Game/Blueprints/Grid/S_Grid` _currentgrid))
  (bind _returnvalue (mod _x_2 64.0))
  (bind _returnvalue_2 (mod _z_2 64.0))
  (bind (_position_2 _heuristicvalue_2 _cost_2 _parentposition _inair) (break `/Game/Blueprints/Grid/S_Grid` (`|GetArrayItem` (`self.BeenCheckedList`) (`self.PrevIndex`))))
  (bind _returnvalue_3 (+ _cost 1))
  (set `self.R` (`KismetMathLibrary.RandomFloat`))
  (set `self.G` (`KismetMathLibrary.RandomFloat`))
  (set `self.B` (`KismetMathLibrary.RandomFloat`))
  (`KismetArrayLibrary.Array_Clear` (`self.UsedPositions`))
  (set `self.CheckDistance` 0)
  (set `self.TotalHeuristic` 0)
  (set `self.LowestHeuristic` -1)
  (set `self.FoundPath` false)
  (bind _output_get (set `self.Start` (`KismetMathLibrary.MakeVector` (+ _x_2 (+ (* PointNormal_X (* _returnvalue 2.0)) _returnvalue)) 0.0 (+ _z_2 (+ (* (* _returnvalue_2 2.0) (* PointNormal_Z -1.0)) _returnvalue_2)))))
  (set `self.Goal` (`KismetMathLibrary.MakeVector` (+ _x (mod _x 64.0)) 0.0 (+ _z (mod _z 64.0))))
  (`self.MakeNewPosition` _output_get _output_get)
  (if (== (`KismetArrayLibrary.Array_Length` (`self.CheckList`)) 0)
    (return -1 -1 false)
    (else
      (while (< (`self.CheckDistance`) MaxCheckDistance)
        (bind _output_get_2 (set `self.CurrentGrid` (`|GetArrayItem` (`self.CheckList`))))
        (bind (_position_3 _heuristicvalue_3) (break `/Game/Blueprints/Grid/S_Grid` _output_get_2))
        (set `self.TotalHeuristic` (+ (`self.TotalHeuristic`) _heuristicvalue_3))
        (if (or (< _heuristicvalue_3 _lowestheuristic_2) (< _lowestheuristic_2 0))
          (set `self.LowestHeuristic` _heuristicvalue_3))
        (if (== _position_3 (`self.Goal`) :`ErrorTolerance` 64.0)
          (set `self.FoundPath` true)
          (`|ExecutionSequence` :!label _label
            (:`then_0`
              (goto _label_2 :!via `Reset`))
            (:`then_1`
              (set `self.MadeFinalPath` false)
              (set `self.PrevIndex` (`KismetArrayLibrary.Array_LastIndex` _beencheckedlist))
              (`KismetArrayLibrary.Array_Clear` (`self.JumpEnd`))
              (`KismetArrayLibrary.Array_Clear` (`self.JumpStart`))
              (`/Engine/EditorBlueprintResources/StandardMacros.DoOnce` false :!label _label_2
                (:`Completed`
                  (bind (_arrayindex _arrayelement) (`/Engine/EditorBlueprintResources/StandardMacros.ReverseForEachLoop` _beencheckedlist)
                    (:`LoopBody`
                      (bind (_position_4 _heuristicvalue_4 _cost_3 _parentposition_2 _inair_2) (break `/Game/Blueprints/Grid/S_Grid` _arrayelement))
                      (if (== _position_4 _parentposition)
                        (if (and _inair_2 (not _inair))
                          (`KismetArrayLibrary.Array_Insert` (`self.JumpStart`) _position_2)
                          (elif (and (not _inair_2) _inair)
                            (`KismetArrayLibrary.Array_Insert` (`self.JumpEnd`) _position_4))))
                      (bind _output_get_3 (set `self.PrevIndex` _arrayindex))
                      (set `self.MadeFinalPath` (not (== _output_get_3 0))))
                    (:`Completed`
                      (for _array_element _beencheckedlist_2
                        (bind (_position_5 _heuristicvalue_5 _cost_4 _parentposition_3 _inair_3) (break `/Game/Blueprints/Grid/S_Grid` _array_element))
                        (`KismetSystemLibrary.DrawDebugBox` _position_5 (16.0 10.0 16.0) (select `bool` _inair_3 :`false` (struct :`R` 0.13305 :`G` 1.0 :`A` 1.0) :`true` (struct :`R` 1.0 :`B` 0.75 :`A` 1.0) :!type "LinearColor Structure") (struct) 5.0 5.0))
                      (`KismetArrayLibrary.Array_Clear` _beencheckedlist_2)
                      (`KismetArrayLibrary.Array_Clear` (`self.CheckList`))
                      (return (`self.TotalHeuristic`) (`self.LowestHeuristic`) (`self.FoundPath`) (`self.JumpStart`) (`self.JumpEnd`))))))))
          (else
            (`KismetArrayLibrary.Array_Add` (`self.BeenCheckedList`) _currentgrid)
            (`KismetArrayLibrary.Array_Remove` (`self.CheckList`))
            (`self.MakeNewPositionForJump` (+ _position (64.0 0.0 0.0)) _position _returnvalue_3)
            (`self.MakeNewPositionForJump` (+ _position (-64.0 0.0 0.0)) _position _returnvalue_3)
            (`self.MakeNewPositionForJump` (+ _position (0.0 0.0 64.0)) _position _returnvalue_3)
            (`self.MakeNewPositionForJump` (+ _position (0.0 0.0 -64.0)) _position _returnvalue_3)
            (`/Engine/EditorBlueprintResources/StandardMacros.IncrementInt` (`self.CheckDistance`)))))
      (while (> (`KismetArrayLibrary.Array_Length` (`self.CheckList`)) 0)
        (bind _output_get_4 (set `self.CurrentGrid` (`|GetArrayItem` (`self.CheckList`))))
        (bind (_position_6 _heuristicvalue_6) (break `/Game/Blueprints/Grid/S_Grid` _output_get_4))
        (set `self.TotalHeuristic` (+ (`self.TotalHeuristic`) _heuristicvalue_6))
        (if (or (< _heuristicvalue_6 _lowestheuristic) (< _lowestheuristic 0))
          (set `self.LowestHeuristic` _heuristicvalue_6))
        (if (== _position_6 (`self.Goal`) :`ErrorTolerance` 64.0)
          (set `self.FoundPath` true)
          (goto _label)
          (else
            (`KismetArrayLibrary.Array_Add` (`self.BeenCheckedList`))
            (`KismetArrayLibrary.Array_Remove` (`self.CheckList`)))))
      (goto _label))))

(fn `GetStartHeuristic`
  (params (FirstPos :type "Vector Structure") (Goal :type "Vector Structure") (Normal :type "Vector Structure"))
  (returns (Heuristic :type Integer))
  (bind _x (.x Goal))
  (bind _z (.z Goal))
  (bind _x_2 (.x FirstPos))
  (bind _z_2 (.z FirstPos))
  (bind _returnvalue (mod _x_2 64.0))
  (bind _returnvalue_2 (mod _z_2 64.0))
  (bind _output_get (set `self.Start` (`KismetMathLibrary.MakeVector` (+ _x_2 (+ (* Normal_X (* _returnvalue 2.0)) _returnvalue)) 0.0 (+ _z_2 (+ (* (* _returnvalue_2 2.0) (* Normal_Z -1.0)) _returnvalue_2)))))
  (bind _output_get_2 (set `self.Goal` (`KismetMathLibrary.MakeVector` (+ _x (mod _x 64.0)) 0.0 (+ _z (mod _z 64.0)))))
  (bind _gridstruct (`self.MakeGridStruct` _output_get _output_get_2 0 _output_get))
  (return (`.HeuristicValue_7_9B5350CA49265427590D25AA90D26CA7` (break `/Game/Blueprints/Grid/S_Grid` _gridstruct))))

(fn `MakeGridStruct`
  (params (Position :type "Vector Structure") (Goal :type "Vector Structure") (Cost :type Integer) (Parent :type "Vector Structure") (InAir :type Boolean))
  (returns (GridStruct :type "/Game/Blueprints/Grid/S_Grid Structure"))
  (return (make `/Game/Blueprints/Grid/S_Grid` (`KismetMathLibrary.MakeVector` (`KismetMathLibrary.Conv_IntToDouble` (`KismetMathLibrary.FTrunc` (.x Position))) 0.0 (`KismetMathLibrary.Conv_IntToDouble` (`KismetMathLibrary.FTrunc` (.z Position)))) (`KismetMathLibrary.FTrunc` (+ (`KismetMathLibrary.Abs` (- (/ (.x Position) 64.0) (/ (.x Goal) 64.0))) (`KismetMathLibrary.Abs` (- (/ (.z Position) 64.0) (/ (.z Goal) 64.0))))) Cost (`KismetMathLibrary.MakeVector` (`KismetMathLibrary.Conv_IntToDouble` (`KismetMathLibrary.FTrunc` (.x Parent))) 0.0 (`KismetMathLibrary.Conv_IntToDouble` (`KismetMathLibrary.FTrunc` (.z Parent)))) InAir)))

(fn `UserConstructionScript`)